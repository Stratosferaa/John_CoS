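; Spline path actor that binds characters to a movement spline, with a matching camera spline beside it.
; Trigger boxes, placed near both spline ends by the construction script, hand an overlapping character this actor and its nearest spline distance if it has no RefSpline.
; CreateCameraSpline rebuilds CameraSpline by sampling the path at fixed spacing, offset sideways and raised, optionally skipping points too close to the previous one.
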(event `self.BoxLeft.OnComponentBeginOverlap`
  (params (OverlappedComponent :type "PrimitiveComponent Object Reference") (OtherActor :type "Actor Object Reference") (OtherComp :type "PrimitiveComponent Object Reference") (OtherBodyIndex :type Integer) (bFromSweep :type Boolean) (SweepResult :type "HitResult Structure (by ref)"))
  (bind _reftochar (`self.RefToChar`))
  (bind _spline (`self.Spline`))
  (bind _ascharacter (cast `/Game/Main/Character` OtherActor))
  (set `self.RefToChar` _ascharacter)
  (`/Game/Main/Character.Ref-Spline` _reftochar :!label _label
    (:`then`)
    (:`else`
      (set `/Game/Main/Character.spline dist` (`SplineComponent.GetDistanceAlongSplineAtSplineInputKey` _spline (`SplineComponent.FindInputKeyClosestToWorldLocation` _spline (`self.K2_GetActorLocation` _reftochar))) _reftochar)
      (set `/Game/Main/Character.Ref-Spline` self _reftochar))))

(event `self.BoxRight.OnComponentBeginOverlap`
  (params (OverlappedComponent :type "PrimitiveComponent Object Reference") (OtherActor :type "Actor Object Reference") (OtherComp :type "PrimitiveComponent Object Reference") (OtherBodyIndex :type Integer) (bFromSweep :type Boolean) (SweepResult :type "HitResult Structure (by ref)"))
  (bind _ascharacter (cast `/Game/Main/Character` OtherActor))
  (set `self.RefToChar` _ascharacter)
  (goto _label))

(event `Create Camera Spline`
  (bind _spline_camera_poins_dist (`self.Spline_camera_poins dist`))
  (bind _coordinate_space (`self.Coordinate Space`))
  (bind _spline (`self.Spline`))
  (bind _returnvalue (`SplineComponent.GetSplineLength` (`self.Spline`)))
  ;[0.01879 0 1] Создание сплайна
  ;[1 1 1] Очищаем старый Сплайн
  (`SplineComponent.ClearSplinePoints` (`self.Camera Spline`) true)
  ;[0.505 1 1] Создание новых точек для сплайна
  (for _index (range (+ (`KismetMathLibrary.FTrunc` (/ _returnvalue _spline_camera_poins_dist)) 1))
    (if (`self.Corection-`)
      (bind _returnvalue_2 (* _index _spline_camera_poins_dist))
      (bind _returnvalue_3 (+ (`SplineComponent.GetLocationAtDistanceAlongSpline` _spline _returnvalue_2 _coordinate_space) (* (`KismetMathLibrary.GetRightVector` (`SplineComponent.GetRotationAtDistanceAlongSpline` _spline _returnvalue_2 _coordinate_space)) (`self.AutoCreateDist_camera`)) (0.0 0.0 130.0)))
      (if (not (== (`self.pos-`) _returnvalue_3 :`ErrorTolerance` (* 2 (`self.Spline_camera_poins dist`))))
        (`SplineComponent.AddSplinePoint` (`self.Camera Spline`) _returnvalue_3 (`self.Coordinate Space`) false :!label _label_2)
        (set `self.pos-` _returnvalue_3))
      (else
        (goto _label_2))))
  (`SplineComponent.AddSplinePoint` (`self.Camera Spline`) (+ (`SplineComponent.GetLocationAtDistanceAlongSpline` _spline _returnvalue _coordinate_space) (* (`KismetMathLibrary.GetRightVector` (`SplineComponent.GetRotationAtDistanceAlongSpline` _spline _returnvalue _coordinate_space)) (`self.AutoCreateDist_camera`)) (0.0 0.0 130.0)) (`self.Coordinate Space`) true))

(event `CustomEvent_0`
  (`SceneComponent.K2_SetRelativeLocation` (`self.BoxLeft`) (`SplineComponent.GetLocationAtDistanceAlongSpline` (`self.Spline`) 50.0 "Local") false false)
  (`SceneComponent.K2_SetRelativeLocation` (`self.BoxRight`) (`SplineComponent.GetLocationAtDistanceAlongSpline` (`self.Spline`) (- (`SplineComponent.GetSplineLength` (`self.Spline`)) 50.0) "Local") false false))

(fn `UserConstructionScript`
  (locals (NewLocalVar_0 :type "Float (double-precision)" :default 25.0))
  (`SceneComponent.K2_SetRelativeLocation` (`self.BoxLeft`) (`SplineComponent.GetLocationAtDistanceAlongSpline` (`self.Spline`) (`local.NewLocalVar_0`) "Local") false false)
  (`SceneComponent.K2_SetRelativeLocation` (`self.BoxRight`) (`SplineComponent.GetLocationAtDistanceAlongSpline` (`self.Spline`) (- (`SplineComponent.GetSplineLength` (`self.Spline`)) (`local.NewLocalVar_0`)) "Local") false false))