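; Play-mode player controller that handles mouse dragging of physics objects, menu input, level restart and a basic save slot.
; Grab events from Main_Character start a Tick loop that moves its PhysicsHandle along the cursor ray, stopped by a sphere trace, with a downward-traced decal marking the ground below.
; Escape skips cinematics and toggles the in-game menu; Tab fires a dispatcher.
; BeginPlay saves the level name, Load only prints it, and debug R deletes the save.
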(event `Key|Tab`
  (params (Key :type "Key Structure"))
  (:`Pressed`
    (`self.EDTab` true))
  (:`Released`
    (`self.EDTab` false)))

(event `Key|Escape`
  (params (Key :type "Key Structure"))
  (:`Pressed`
    (bind _foundwidgets (`WidgetBlueprintLibrary.GetAllWidgetsOfClass` "/Game/Shimaletik/Scip_sinematic.Scip_sinematic_C"))
    (if (`KismetArrayLibrary.Array_IsValidIndex` _foundwidgets)
      (`/Game/Shimaletik/Scip_sinematic.Esc scip` _foundwidgets))))

(event `self.ReceiveBeginPlay`
  (bind _reftochar (`self.RefToChar`))
  (`|ExecutionSequence`
    (:`then_0`
      (bind _returnvalue (`GameplayStatics.GetActorOfClass` "/Game/Shimaletik/ContoledItemMap.ContoledItemMap_C"))
      (`/Engine/EditorBlueprintResources/StandardMacros.IsValid` _returnvalue
        (:`Is Not Valid`
          (`|SpawnActorFromClass` "/Game/Shimaletik/ContoledItemMap.ContoledItemMap_C" (`KismetMathLibrary.MakeTransform` (0.0 0.0 0.0)) "AlwaysSpawn" "OverrideRootScale" null null))))
    (:`then_1`
      (set `self.bShowMouseCursor` true)
      (bind _asmain_character (cast `/Game/_Props_2/Core/Character/Main_Character` (`GameplayStatics.GetPlayerCharacter` 0)))
      (bind _output_get (set `self.RefToChar` _asmain_character))
      (add `/Game/_Props_2/Core/Character/Main_Character.SetPhysicsObject` _output_get (`|CreateDelegate` :!event `SetPhysicsObject`))
      (set `self.CameraScene` (`/Game/_Props_2/Core/Character/Main_Character.SideViewCameraComponent` _reftochar))
      (set `self.PhysicsHandle` (`/Game/_Props_2/Core/Character/Main_Character.PhysicsHandle` _reftochar)))
    (:`then_2`
      (`self.Save`))))

(event `Key|R`
  (params (Key :type "Key Structure"))
  ;[1 1 1] DEBUG HARD RESET SAVE / УДАЛЕНИЕ СЕЙВА
  (:`Pressed`
    (`GameplayStatics.DeleteGameInSlot` "0")
    (set `self.Save Game` null)))

(event `Key|Escape`
  (params (Key :type "Key Structure"))
  (:`Pressed`
    (`/Engine/EditorBlueprintResources/StandardMacros.FlipFlop` :!label _label
      (:`A`
        (bind _returnvalue (`|CreateWidget` "/Game/Shimaletik/Menu/W_InGameMenu.W_InGameMenu_C"))
        (`UserWidget.AddToViewport` _returnvalue 1)
        (set `self.OpenMenu` true))
      (:`B`
        (if (`Widget.IsVisible` _returnvalue)
          (`Widget.RemoveFromParent` _returnvalue)
          (set `self.OpenMenu` false)
          (else
            (goto _label)))))
    (bind _foundwidgets (`WidgetBlueprintLibrary.GetAllWidgetsOfClass` "/Game/Shimaletik/Cursors/A1W.A1W_C" false))
    (set `/Game/Shimaletik/Cursors/A1W.Default` (`self.OpenMenu`) (`|GetArrayItem` _foundwidgets))))

(event `SetPhysicsObject`
  (params (Take :type Boolean) (Component :type "PrimitiveComponent Object Reference") (GrabLocation :type "Vector Structure"))
  ;[1 1 1] Таскание и корект обекта
  (if Take
    (set `self.GrabbedComponent` Component)
    (bind _output_get (set `self.GrabbedLocation` GrabLocation))
    (set `self.Start_grab_dist` (`KismetMathLibrary.VSize` (- _output_get (`SceneComponent.K2_GetComponentLocation` (`/Game/_Props_2/Core/Character/Main_Character.SideViewCameraComponent` (`self.RefToChar`))))))
    (set `self.TimerHandlePhysics` (struct))
    (set `self.NewVar_0` true)
    (bind _returnvalue (`GameplayStatics.SpawnDecalAtLocation` "/Game/Shimaletik/Decal_material.Decal_material" (20.0 20.0 20.0)))
    (set `self.decal` _returnvalue)
    (else
      (`KismetSystemLibrary.K2_ClearAndInvalidateTimerHandle` (`self.TimerHandlePhysics`))
      (set `self.GrabbedComponent` null)
      (set `self.GrabbedLocation` (0.0 0.0 0.0))
      (set `self.LocationObjectY` 0.0)
      (set `self.NewVar_0` false)
      (bind _decal (`self.decal`)
        (:`then`
          (`ActorComponent.K2_DestroyComponent` _decal))
        (:`else`)))))

(event `Save`
  ;[1 1 1] СОХРАНЕНИЕ / SAVE
  (bind _returnvalue (`GameplayStatics.CreateSaveGameObject` "/Game/_Props/Arti/SaveGameArti.SaveGameArti_C"))
  (bind _output_get (set `self.Save Game` _returnvalue))
  (bind _returnvalue_2 (`GameplayStatics.GetCurrentLevelName` true))
  (`KismetSystemLibrary.PrintString` _returnvalue_2)
  (set `/Game/_Props/Arti/SaveGameArti.SavedWorldName` (`KismetStringLibrary.Conv_StringToName` _returnvalue_2) _output_get)
  (`GameplayStatics.SaveGameToSlot` _output_get "0"))

(event `self.ReceiveTick`
  (params (DeltaSeconds :type "Float (single-precision)"))
  (bind (_worldlocation _worlddirection) (`self.DeprojectMousePositionToWorld`))
  (bind _grabbedcomponent (`self.GrabbedComponent`))
  (bind _decal (`self.decal`))
  (bind _grabbedcomponent_2 (`self.GrabbedComponent`))
  (bind _returnvalue (`SceneComponent.K2_GetComponentLocation` _grabbedcomponent))
  (bind _returnvalue_2 (+ _worldlocation (* _worlddirection (- (`self.Start_grab_dist`) (`self.LocationObjectY`)))))
  ;[1 1 1] Таскание и корект обекта
  ;;[1 1 1] Корект обекта
  (if (`self.NewVar_0`)
    (`/Engine/EditorBlueprintResources/StandardMacros.IsValid` _grabbedcomponent_2
      (:`Is Valid`
        (bind (_outhit _returnvalue_3) (`KismetSystemLibrary.SphereTraceSingle` _worldlocation _returnvalue_2 20.0 "TraceTypeQuery1" false (`|MakeArray` (`ActorComponent.GetOwner` _grabbedcomponent_2))))
        (`PhysicsHandleComponent.SetTargetLocationAndRotation` :`self` (`self.PhysicsHandle`) :`NewLocation` (`KismetMathLibrary.SelectVector` (`.Location` (`GameplayStatics.BreakHitResult` _outhit)) _returnvalue_2 _returnvalue_3))
        (bind (_outhit_2 _returnvalue_4) (`KismetSystemLibrary.CapsuleTraceSingle` _returnvalue (- _returnvalue (0.0 0.0 1000.0)) 5.0 5.0 "TraceTypeQuery1" false (`|MakeArray` (`ActorComponent.GetOwner` _grabbedcomponent))))
        (if _returnvalue_4
          (`SceneComponent.K2_SetWorldLocation` _decal (`.Location` (`GameplayStatics.BreakHitResult` _outhit_2)) false false)
          (else
            (`SceneComponent.K2_SetWorldLocation` _decal (0.0 0.0 0.0) false false))))
      (:`Is Not Valid`
        (bind _decal_2 (`self.decal`)
          (:`then`
            (`ActorComponent.K2_DestroyComponent` _decal_2))
          (:`else`))))))

(event `Load`
  ;[1 1 1] ЗАГРУЗКА / LOAD
  (`GameplayStatics.SetGamePaused` true)
  (bind _returnvalue (`GameplayStatics.LoadGameFromSlot` "0"))
  (bind _assave_game_arti (cast `/Game/_Props/Arti/SaveGameArti` _returnvalue)
    (:`then`
      (`KismetSystemLibrary.PrintString` (`KismetStringLibrary.Conv_NameToString` (`/Game/_Props/Arti/SaveGameArti.SavedWorldName` _assave_game_arti))))
    (:`CastFailed`
      _))
  (`GameplayStatics.SetGamePaused` false))

(event `Restart`
  ;[1 1 1] Restart
  (bind _returnvalue (`GameplayStatics.GetCurrentLevelName` true))
  (`GameplayStatics.OpenLevel` (`KismetStringLibrary.Conv_StringToName` _returnvalue)))

(fn `UserConstructionScript`)