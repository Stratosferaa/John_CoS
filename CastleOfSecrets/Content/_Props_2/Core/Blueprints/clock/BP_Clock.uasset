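; Clock puzzle prop where placing the missing hour, minute and second hands releases a door key.
; Each add event destroys the pickup, reveals that hand and spins it on a timeline.
; With all three placed, timelines rotate two clock parts open, then the bird animates as the child-actor key moves out.
; The socket-attached key regains collision and gravity after a delay; interaction toggles Custom Depth highlighting.
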(event `AddArrowCloackMinut`
  (params (Target :type "Actor Object Reference"))
  (`self.K2_DestroyActor` Target)
  (`SceneComponent.SetVisibility` (`self.MinuteHand_B`) true false)
  (`self.RotateCloacl`))

(event `self.ReceiveBeginPlay`
  (bind _meshitem (`/Game/_Props_2/Core/Blueprints/Items/BP_BaseItem.MeshItem` (`self.As BP Key Door`)))
  (bind _asbp_key_door (cast `/Game/_Props_2/Core/Blueprints/Items/BP_KeyDoor` (`ChildActorComponent.ChildActor` (`self.ChildActor`)) :!pure true))
  (set `self.As BP Key Door` _asbp_key_door)
  (`SceneComponent.K2_AttachToComponent` (`/Game/_Props_2/Core/Blueprints/Items/BP_BaseItem.MeshItem` _asbp_key_door) (`self.BIRD_untitled_Cube_001`) "KeyPoint" "KeepWorld" "KeepWorld" "KeepWorld" true)
  (`PrimitiveComponent.SetEnableGravity` _meshitem false)
  (`PrimitiveComponent.SetSimulatePhysics` _meshitem false)
  (`PrimitiveComponent.SetCollisionEnabled` _meshitem "NoCollision"))

(event `AddArrowHaour`
  (params (Target :type "Actor Object Reference"))
  (`self.K2_DestroyActor` Target)
  (`SceneComponent.SetVisibility` (`self.HourHand_D`) true false)
  (`self.RotateCloackHour`))

(event `AddArrowSecond`
  (params (Target :type "Actor Object Reference"))
  (`self.K2_DestroyActor` Target)
  (`SceneComponent.SetVisibility` (`self.SecondHand_A`) true false)
  (`self.RotateCloackSecond`))

(event `/Game/_Props_2/Core/Blueprints/Interface/BP_Info.InfoInteraction`
  (params (Char :type "/Game/Main/Character Object Reference") (On :type Boolean) (HitComponent :type "PrimitiveComponent Object Reference"))
  (`PrimitiveComponent.SetRenderCustomDepth` (`self.Clockkk_Clocks123_clock_2_osnova`) On)
  (`PrimitiveComponent.SetRenderCustomDepth` (`self.untitled_Cube_006`) On)
  (`PrimitiveComponent.SetRenderCustomDepth` (`self.untitled_Cube_005`) On)
  (`PrimitiveComponent.SetRenderCustomDepth` (`self.untitled_Cube_004`) On)
  (`PrimitiveComponent.SetRenderCustomDepth` (`self.untitled_Cube_003`) On)
  (`PrimitiveComponent.SetRenderCustomDepth` (`self.untitled_Cube_002`) On))

(event `Bird`
  (if (and (`self.SecondVisibility`) (`self.HourVisibility`) (`self.MinutVisibility`))
    (`/Engine/EditorBlueprintResources/StandardMacros.DoOnce` false
      (:`Completed`
        (`|ExecutionSequence`
          (:`then_0`
            (bind (_direction _scale) (`Timeline|Timeline_5`)
              (:`Update`
                (`SceneComponent.K2_AddLocalOffset` (`Actor.RootComponent` (`self.As BP Key Door`)) (`KismetMathLibrary.MakeVector` 0.0 _scale) false false))
              (:`Finished`
                (`self.KeyEvent`))))
          (:`then_1`
            (`SkeletalMeshComponent.PlayAnimation` (`self.BIRD_untitled_Cube_012`) "/Game/_Props_2/Core/Blueprints/clock/IconCloak/BIRD_untitled_Cube_012_Anim.BIRD_untitled_Cube_012_Anim" false)))))))

(event `KeyEvent`
  (bind _meshitem (`/Game/_Props_2/Core/Blueprints/Items/BP_BaseItem.MeshItem` (`self.As BP Key Door`)))
  (`KismetSystemLibrary.Delay` 4.0)
  (`PrimitiveComponent.SetCollisionEnabled` _meshitem "QueryAndPhysics")
  (`PrimitiveComponent.SetEnableGravity` _meshitem true))

(event `self.ReceiveTick`
  (params (DeltaSeconds :type "Float (single-precision)")))

(event `OpenDoor`
  (if (and (`self.SecondVisibility`) (`self.HourVisibility`) (`self.MinutVisibility`))
    (`/Engine/EditorBlueprintResources/StandardMacros.DoOnce` false
      (:`Completed`
        (bind (_direction _cloack) (`Timeline|Timeline_3` :!via `PlayFromStart`)
          (:`Update`
            (`SceneComponent.K2_AddWorldRotation` (`self.untitled_Cube_006`) (`KismetMathLibrary.MakeRotator` 0.0 0.0 _cloack) false false)
            (bind (_direction_2 _cloack_2) (`Timeline|Timeline_4`)
              (:`Update`
                (`SceneComponent.K2_AddWorldRotation` (`self.untitled_Cube_005`) (`KismetMathLibrary.MakeRotator` 0.0 0.0 _cloack_2) false false))
              (:`Finished`
                (`self.Bird`)))))))))

(event `RotateCloacl`
  (bind (_rotatepositionlast_roll _rotatepositionlast_pitch _rotatepositionlast_yaw) (`KismetMathLibrary.BreakRotator` (`self.RotatePositionLast`)))
  (set `self.MinutVisibility` true)
  (bind (_direction _cloack) (`Timeline|Timeline_2` :!via `PlayFromStart`)
    (:`Update`
      (`SceneComponent.K2_AddWorldRotation` (`self.MinuteHand_B`) (`KismetMathLibrary.MakeRotator` _rotatepositionlast_roll _cloack _rotatepositionlast_yaw) false false)
      (set `self.RotatePositionLast` (`KismetMathLibrary.MakeRotator` _rotatepositionlast_roll 0.0 _rotatepositionlast_yaw)))
    (:`Finished`
      (`self.OpenDoor`))))

(event `RotateCloackHour`
  (bind (_rotatepositionlast_roll _rotatepositionlast_pitch _rotatepositionlast_yaw) (`KismetMathLibrary.BreakRotator` (`self.RotatePositionLast`)))
  (set `self.HourVisibility` true)
  (bind (_direction _cloack) (`Timeline|Timeline_0_0` :!via `PlayFromStart`)
    (:`Update`
      (`SceneComponent.K2_AddWorldRotation` (`self.HourHand_D`) (`KismetMathLibrary.MakeRotator` _rotatepositionlast_roll _cloack _rotatepositionlast_yaw) false false)
      (set `self.RotatePositionLast` (`KismetMathLibrary.MakeRotator` _rotatepositionlast_roll 0.0 _rotatepositionlast_yaw)))
    (:`Finished`
      (`self.OpenDoor`))))

(event `RotateCloackSecond`
  (bind (_rotatepositionlast_roll _rotatepositionlast_pitch _rotatepositionlast_yaw) (`KismetMathLibrary.BreakRotator` (`self.RotatePositionLast`)))
  (set `self.SecondVisibility` true)
  (bind (_direction _cloack) (`Timeline|Timeline_1_0` :!via `PlayFromStart`)
    (:`Update`
      (`SceneComponent.K2_AddWorldRotation` (`self.SecondHand_A`) (`KismetMathLibrary.MakeRotator` _rotatepositionlast_roll _cloack _rotatepositionlast_yaw) false false)
      (set `self.RotatePositionLast` (`KismetMathLibrary.MakeRotator` _rotatepositionlast_roll 0.0 _rotatepositionlast_yaw)))
    (:`Finished`
      (`self.OpenDoor`))))

(fn `UserConstructionScript`)