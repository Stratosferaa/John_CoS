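; BP_Chain is a chain prop that lowers and raises through MoveDown and MoveUp events and picks up a Knight it touches.
; Two timelines add their track value to the root's world Z each update.
; A Knight overlapping the box attaches to AttachPoint after a half-second delay, blocking further MoveDown calls.
; MoveUp starts only while the location's vector length is below that of the position saved at BeginPlay.
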(event `MoveDown`
  (bind _defaultsceneroot (`self.DefaultSceneRoot`))
  (bind (_returnvalue_x _returnvalue_y _returnvalue_z) (`KismetMathLibrary.BreakVector` (`SceneComponent.K2_GetComponentLocation` _defaultsceneroot)))
  ;[1 1 1] MoveChainDown
  (if (not (`self.IsAttach`))
    (bind (_direction _rotater) (`Timeline|TimeLineDown` :!via `PlayFromStart`)
      (:`Update`
        (`SceneComponent.K2_SetWorldLocation` _defaultsceneroot (`KismetMathLibrary.MakeVector` _returnvalue_x _returnvalue_y (+ _returnvalue_z _rotater)) false false)))))

(event `MoveUp`
  (bind _defaultsceneroot (`self.DefaultSceneRoot`))
  (bind (_returnvalue_x _returnvalue_y _returnvalue_z) (`KismetMathLibrary.BreakVector` (`SceneComponent.K2_GetComponentLocation` _defaultsceneroot)))
  ;[1 1 1] MoveChainUp
  (if (not (>= (`KismetMathLibrary.VSize` (`SceneComponent.K2_GetComponentLocation` (`self.DefaultSceneRoot`))) (`KismetMathLibrary.VSize` (`self.StartLocation`))))
    (bind (_direction _rotater) (`Timeline|TimeLineUp` :!via `PlayFromStart`)
      (:`Update`
        (`SceneComponent.K2_SetWorldLocation` _defaultsceneroot (`KismetMathLibrary.MakeVector` _returnvalue_x _returnvalue_y (+ _returnvalue_z _rotater)) false false)))))

(event `self.ReceiveBeginPlay`
  ;[1 1 1] StartPosition/BeginPlay
  (`/Engine/EditorBlueprintResources/StandardMacros.DoOnce` false
    (:`Completed`
      (set `self.StartLocation` (`SceneComponent.K2_GetComponentLocation` (`self.DefaultSceneRoot`))))))

(event `self.Box.OnComponentBeginOverlap`
  (params (OverlappedComponent :type "PrimitiveComponent Object Reference") (OtherActor :type "Actor Object Reference") (OtherComp :type "PrimitiveComponent Object Reference") (OtherBodyIndex :type Integer) (bFromSweep :type Boolean) (SweepResult :type "HitResult Structure (by ref)"))
  (bind _asknight (cast `/Game/_Props_2/Core/Blueprints/TorhRota/Knight` OtherActor))
  (`KismetSystemLibrary.Delay` 0.5)
  (`self.K2_AttachToComponent` _asknight (`self.AttachPoint`) "None" "KeepWorld" "KeepWorld" "KeepWorld" true)
  (set `self.IsAttach` true))

(fn `UserConstructionScript`)