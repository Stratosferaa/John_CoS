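; Interactable torch prop that rotates when used and then triggers a linked object to move down, like a lever.
; InfoInteraction toggles custom depth on the torch mesh, presumably for highlighting.
; Interact plays the Rotate timeline, adding world rotation each update from its value and the stored last rotation, then calls MoveDown on MoveLocationDown.
; An IsMove flag blocks re-triggering until a short delay after that call.
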(event `/Game/_Props_2/Core/Blueprints/Interface/BP_Info.InfoInteraction`
  (params (Char :type "/Game/Main/Character Object Reference") (On :type Boolean) (HitComponent :type "PrimitiveComponent Object Reference"))
  ;[1 1 1] RenderVisibility
  (`PrimitiveComponent.SetRenderCustomDepth` (`self.SM_Torch`) On))

(event `Interact_1_1`
  (bind (_rotatepositionlast_roll _rotatepositionlast_pitch _rotatepositionlast_yaw) (`KismetMathLibrary.BreakRotator` (`self.RotatePositionLast`)))
  ;[1 1 1] Rotation/MoveChain
  (if (not (`self.IsMove`))
    (set `self.IsMove` true)
    (bind (_direction _rotater) (`Timeline|Rotate` :!via `PlayFromStart`)
      (:`Update`
        (`SceneComponent.K2_AddWorldRotation` (`self.SM_Torch`) (`KismetMathLibrary.MakeRotator` _rotatepositionlast_roll _rotater _rotatepositionlast_yaw) false false)
        (set `self.RotatePositionLast` (`KismetMathLibrary.MakeRotator` _rotatepositionlast_roll _rotater _rotatepositionlast_yaw)))
      (:`Finished`
        (`/Game/_Props_2/Core/Blueprints/TorhRota/BP_Chain.MoveDown` (`self.MoveLocationDown`))
        (`KismetSystemLibrary.Delay` 0.2)
        (set `self.IsMove` false)))))

(fn `Interact`
  (returns (Valid :type Boolean))
  (return false))

(fn `UserConstructionScript`)