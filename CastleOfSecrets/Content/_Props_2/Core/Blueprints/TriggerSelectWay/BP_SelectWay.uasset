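; Junction trigger that lets the player switch between a left/right spline path and a forward/backward one.
; Box overlap by a Character shows arrow meshes for whichever spline references are valid, and hides all arrows on exit.
; Clicking an arrow selects its axis's spline; if it differs from the player's current one, the character finds the nearest point on it and updates its location.
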(event `/Game/_Props_2/Core/Blueprints/Interface/BP_Info.ClicedMouse`
  (params (PrimComp :type "PrimitiveComponent Object Reference"))
  (bind _asstatic_mesh_component (cast `StaticMeshComponent` PrimComp))
  (bind _ascharacter (cast `/Game/Main/Character` (`GameplayStatics.GetPlayerCharacter` 0)))
  (bind _returnvalue (select `bool` (>= (`KismetArrayLibrary.Array_Find` (`|MakeArray` (`self.ArrowLeft`) (`self.ArrowRight`) (`self.ArrowForward`) (`self.ArrowBackward`)) _asstatic_mesh_component) 2) :`false` (`self.RefSplineToLeft Right`) :`true` (`self.RefSplineToForward Backward`)))
  (if (not (== (`/Game/Main/Character.Ref-Spline` _ascharacter) _returnvalue))
    (`/Game/Main/Character.Find near spline` _ascharacter _returnvalue)
    (`/Game/Main/Character.UpdateLcoation` _ascharacter)))

(event `/Game/_Props_2/Core/Blueprints/Interface/BP_Info.InfoInteraction`
  (params (Char :type "/Game/Main/Character Object Reference") (On :type Boolean) (HitComponent :type "PrimitiveComponent Object Reference"))
  (set `self.Char_0` Char))

(event `self.Box_0.OnComponentBeginOverlap`
  (params (OverlappedComponent :type "PrimitiveComponent Object Reference") (OtherActor :type "Actor Object Reference") (OtherComp :type "PrimitiveComponent Object Reference") (OtherBodyIndex :type Integer) (bFromSweep :type Boolean) (SweepResult :type "HitResult Structure (by ref)"))
  (cast `/Game/Main/Character` OtherActor)
  (`self.SetRenderOpacityArrows` true))

(event `self.Box_0.OnComponentEndOverlap`
  (params (OverlappedComponent :type "PrimitiveComponent Object Reference") (OtherActor :type "Actor Object Reference") (OtherComp :type "PrimitiveComponent Object Reference") (OtherBodyIndex :type Integer))
  (cast `/Game/Main/Character` OtherActor)
  (`self.SetRenderOpacityArrows` false))

(fn `SetRenderOpacityArrows`
  (params (Render :type Boolean))
  (bind _refsplinetoforward_backward (`self.RefSplineToForward Backward`))
  (bind _refsplinetoleft_right (`self.RefSplineToLeft Right`))
  (if Render
    (`SceneComponent.SetVisibility` (`self.ArrowLeft`) (`KismetSystemLibrary.IsValid` _refsplinetoleft_right) false)
    (`SceneComponent.SetVisibility` (`self.ArrowRight`) (`KismetSystemLibrary.IsValid` _refsplinetoleft_right) false)
    (`SceneComponent.SetVisibility` (`self.ArrowBackward`) (`KismetSystemLibrary.IsValid` _refsplinetoforward_backward) false)
    (`SceneComponent.SetVisibility` (`self.ArrowForward`) (`KismetSystemLibrary.IsValid` _refsplinetoforward_backward) false)
    (else
      (`SceneComponent.SetVisibility` (`self.ArrowLeft`) false false)
      (`SceneComponent.SetVisibility` (`self.ArrowRight`) false false)
      (`SceneComponent.SetVisibility` (`self.ArrowForward`) false false)
      (`SceneComponent.SetVisibility` (`self.ArrowBackward`) false false))))

(fn `UserConstructionScript`)