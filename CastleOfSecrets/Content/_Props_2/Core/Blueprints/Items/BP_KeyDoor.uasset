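; BP_KeyDoor is an item Blueprint, apparently a door key, built on a parent class whose construction script it calls.
; Its only active logic is a Tick debug readout that prints the Visibility channel collision responses of MeshItem, AddColision and AutoCraft as one concatenated on-screen string.
; BeginPlay and ActorBeginOverlap are disabled stubs, and the file itself contains no door or key behavior.
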(event `self.ReceiveTick`
  (params (DeltaSeconds :type "Float (single-precision)"))
  (`KismetSystemLibrary.PrintString` (`KismetStringLibrary.Concat_StrStr` (`|GetEnumeratorNameAsString` (`PrimitiveComponent.GetCollisionResponseToChannel` (`self.MeshItem`) "ECC_Visibility")) "   " (`|GetEnumeratorNameAsString` (`PrimitiveComponent.GetCollisionResponseToChannel` (`self.AddColision`) "ECC_Visibility")) "   " (`|GetEnumeratorNameAsString` (`PrimitiveComponent.GetCollisionResponseToChannel` (`self.AutoCraft`) "ECC_Visibility"))) true true (struct :`G` 0.66 :`B` 1.0 :`A` 1.0) 0.0))

(fn `UserConstructionScript`
  (`parent.UserConstructionScript`))