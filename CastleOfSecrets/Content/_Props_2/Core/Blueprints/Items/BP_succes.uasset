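; Item Blueprint with a scripted knife move, triggered by an event that receives a picture reference.
; The Knife event turns off physics on the item mesh and snaps it to the picture's Scene component.
; Two chained timelines then animate the mesh, first along world Z and then along world X, writing their curve values as absolute coordinates rather than offsets.
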(event `Knife`
  (params (Picturce :type "/Game/_Props_2/Core/picture/Picturce_BP Object Reference"))
  (bind _meshitem (`self.MeshItem`))
  (`PrimitiveComponent.SetSimulatePhysics` _meshitem false)
  (`SceneComponent.K2_SetWorldLocation` _meshitem (`SceneComponent.K2_GetComponentLocation` (`/Game/_Props_2/Core/picture/Picturce_BP.Scene` Picturce)) false false)
  (`self.MoveKnife`))

(event `MoveKnife`
  (bind _meshitem (`self.MeshItem`))
  (bind (_returnvalue_x _returnvalue_y) (`KismetMathLibrary.BreakVector` (`SceneComponent.K2_GetComponentLocation` _meshitem)))
  (bind (_returnvalue_x_2 _returnvalue_y_2 _returnvalue_z) (`KismetMathLibrary.BreakVector` (`SceneComponent.K2_GetComponentLocation` (`self.MeshItem`))))
  (bind (_direction _worldloca) (`Timeline|Move Up` :!via `PlayFromStart`)
    (:`Update`
      (`SceneComponent.K2_SetWorldLocation` _meshitem (`KismetMathLibrary.MakeVector` _returnvalue_x _returnvalue_y _worldloca) false false))
    (:`Finished`
      (bind (_direction_2 _worldloca_2) (`Timeline|Timeline_0_0` :!via `PlayFromStart`)
        (:`Update`
          (`SceneComponent.K2_SetWorldLocation` (`self.MeshItem`) (`KismetMathLibrary.MakeVector` _worldloca_2 _returnvalue_y_2 _returnvalue_z) false false))))))

(fn `UserConstructionScript`
  (`parent.UserConstructionScript`))