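; Base Blueprint for interactive physics items, with hover outline and stat widget, sounds, and stub hooks for children.
; Overlapping a partner found in the Craftitem map reports to the quest object, optionally plays a cinematic, moves the result item into place and can destroy either ingredient.
; CDestroy shrinks the mesh by timeline, then destroys it or parks it high above, while Cspawn scales it back.
; UpdateRespawn saves its transform in ContoledItemMap.
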(event `Update qest stat item`
  (bind _returnvalue (`self.GetComponentByClass` "/Game/Shimaletik/Components/playChinematik_Cliced.playChinematik_Cliced_C"))
  (`/Engine/EditorBlueprintResources/StandardMacros.IsValid` _returnvalue
    (:`Is Valid`
      (set `/Game/Shimaletik/Components/playChinematik_Cliced.Qests` (`self.Qests`) _returnvalue))))

(event `self.ReceiveBeginPlay`
  (bind _meshitem (`self.MeshItem`))
  (bind _output (`|GetArrayItem` (`self.GetComponentsByTag` self "/Game/Shimaletik/Components/playChinematik_Cliced.playChinematik_Cliced_C" "КликСинематик")))
  (bind _output_2 (`|GetArrayItem` (`self.GetComponentsByTag` self "/Game/Shimaletik/Components/playChinematik_Cliced.playChinematik_Cliced_C" "УспешныйКрафт")))
  (`|ExecutionSequence`
    (:`then_0`
      (`|ExecutionSequence`
        (:`then_0`
          (`/Engine/EditorBlueprintResources/StandardMacros.IsValid` _output
            (:`Is Valid`
              (set `self.КликСинематик` _output))))
        (:`then_1`
          (`/Engine/EditorBlueprintResources/StandardMacros.IsValid` _output_2
            (:`Is Valid`
              (set `self.УспешныйКрафт` _output_2))))))
    (:`then_1`
      (`PrimitiveComponent.SetMassOverrideInKg` (`self.MeshItem`) "None" 1e-05 true)
      (`PrimitiveComponent.SetMassOverrideInKg` (`self.AddColision`) "None" 1e-05 true)
      (`PrimitiveComponent.SetMassOverrideInKg` (`self.BoxParticle`) "None" 1e-05 true)
      (`PrimitiveComponent.SetSimulatePhysics` _meshitem (`self.Simuleit phisic`))
      (set `self.TransfomScaleDefault` (`SceneComponent.K2_GetComponentScale` _meshitem))
      (`KismetSystemLibrary.Delay` 1.0)
      (`PrimitiveComponent.SetCollisionResponseToChannel` (`self.MeshItem`) "ECC_WorldDynamic" "ECR_Block")
      (bind _ascharacter (cast `/Game/Main/Character` (`GameplayStatics.GetPlayerCharacter` 0)))
      (set `self.As Main Character` _ascharacter))))

(event `/Game/_Props_2/Core/Blueprints/Interface/BP_WidghetBackLight.Backlight`
  (params (Backlight :type Boolean))
  (`SceneComponent.SetVisibility` (`self.Widget`) Backlight false))

(event `obvodca`
  (params (on :type Boolean)))

(event `/Game/_Props_2/Core/Blueprints/Interface/BP_Info.InfoInteraction`
  (params (Char :type "/Game/Main/Character Object Reference") (On :type Boolean) (HitComponent :type "PrimitiveComponent Object Reference"))
  (bind (_icon _description) (break `/Game/_Props_2/Core/Blueprints/Struct/ST_SlotItem` (`self.ParamItem`)))
  (`self.obvodca` On)
  (`PrimitiveComponent.SetRenderCustomDepth` (`self.MeshItem`) (select `bool` (`self.Подсветка`) :`true` On))
  (`|ExecutionSequence`
    (:`then_0`
      (if On
        (`self.NewVar_0`
          (:`then`)
          (:`else`
            (bind _returnvalue (`|CreateWidget` "/Game/Shimaletik/inv/ui/Stat_item.Stat_item_C" null _description _icon))
            (`UserWidget.AddToViewport` _returnvalue 0)
            (set `self.NewVar_0` _returnvalue)))
        (else
          (bind _foundwidgets (`WidgetBlueprintLibrary.GetAllWidgetsOfClass` "/Game/Shimaletik/inv/ui/Stat_item.Stat_item_C" false))
          (if (`KismetArrayLibrary.Array_IsValidIndex` _foundwidgets)
            (`Widget.RemoveFromParent` _foundwidgets))
          (set `self.NewVar_0` null))))
    (:`then_1`
      (if (`self.Simuleit phisic`)
        _))))

(event `self.ReceiveTick`
  (params (DeltaSeconds :type "Float (single-precision)")))

(event `CustomEvent_0`
  (`KismetSystemLibrary.Delay` 0.0)
  (`self.UpdateRespawn`))

(event `/Game/_Props_2/Core/Blueprints/Interface/BP_Interaction.Grabed`
  (params (Yes :type Boolean) (`BP-BaseItem` :type "/Game/_Props_2/Core/Blueprints/Items/BP_BaseItem Object Reference"))
  ;[0.01879 0 1] Схвачен или отпущен предмет
  (set `self.Bp Baseitem` `BP-BaseItem`))

(event `self.AutoCraft.OnComponentBeginOverlap`
  (params (OverlappedComponent :type "PrimitiveComponent Object Reference") (OtherActor :type "Actor Object Reference") (OtherComp :type "PrimitiveComponent Object Reference") (OtherBodyIndex :type Integer) (bFromSweep :type Boolean) (SweepResult :type "HitResult Structure (by ref)"))
  (bind _craftitem (`self.Craftitem`))
  (bind _bp_baseitem (`self.Bp Baseitem`))
  (bind _returnvalue (`self.GetComponentByClass` _bp_baseitem "/Game/Shimaletik/Components/playChinematik_Cliced.playChinematik_Cliced_C"))
  (bind _asbp_base_item (cast `/Game/_Props_2/Core/Blueprints/Items/BP_BaseItem` OtherActor))
  (set `self.Bp Baseitem` _asbp_base_item)
  (bind _keys (`BlueprintMapLibrary.Map_Keys` _craftitem))
  (bind _returnvalue_2 (`KismetArrayLibrary.Array_Find` _keys _bp_baseitem))
  (if (not (== _returnvalue_2 -1))
    (bind _values (`BlueprintMapLibrary.Map_Values` _craftitem))
    (`self.FQest` (`|GetArrayItem` _keys _returnvalue_2) "NewEnumerator1")
    (`self.FQest` "NewEnumerator0")
    (bind (`_уничтожитьсебя` `_уничтожитьскемскрафтился` `_запуститьускемскрафтилсяанимацию` `_ктопоявитсяприкрафте` `_уникальнаяточкапоявления`) (break `/Game/_Props_2/Core/Blueprints/Items/Craftitem` (`|GetArrayItem` _values _returnvalue_2)))
    (if `_запуститьускемскрафтилсяанимацию`
      (`/Engine/EditorBlueprintResources/StandardMacros.IsValid` _returnvalue
        (:`Is Valid`
          (if (not (`MovieSceneSequencePlayer.IsPlaying` (`/Game/Shimaletik/Components/playChinematik_Cliced.level Sequence` _returnvalue)))
            (`/Game/Shimaletik/Components/playChinematik_Cliced.Start_anim` _returnvalue self)
            (`/Engine/EditorBlueprintResources/StandardMacros.IsValid` `_ктопоявитсяприкрафте` :!label _label
              (:`Is Valid`
                (`self.K2_SetActorLocation` `_ктопоявитсяприкрафте` (`KismetMathLibrary.SelectVector` (`self.K2_GetActorLocation` `_уникальнаяточкапоявления`) (`self.K2_GetActorLocation` _bp_baseitem) (`KismetSystemLibrary.IsValid` `_уникальнаяточкапоявления`)) false true)
                (`self.CustomEvent_0` `_ктопоявитсяприкрафте`))
              (:`Is Not Valid`
                _))
            (if `_уничтожитьсебя`
              (if (not (`/Game/_Props_2/Core/Blueprints/Items/BP_BaseItem.Used?` _bp_baseitem))
                (`self.CDestroy` true)
                (if (`/Game/_Props_2/Core/Blueprints/Items/BP_BaseItem.Used?` _bp_baseitem) :!label _label_2
                  _
                  (elif `_уничтожитьскемскрафтился`
                    (`self.CDestroy` _bp_baseitem true))))
              (else
                (goto _label_2)))
            (`self.Crafting Event` _bp_baseitem (stale `/Game/_Props_2/Core/Blueprints/Interface/BP_Interaction.Grabed` Yes) self)
            (`GameplayStatics.PlaySound2D` (`self.ЗвукКогда Скрафтился`) 1.0 1.0 0.0 null null)
            (bind `_успешныйкрафт` (`/Game/_Props_2/Core/Blueprints/Items/BP_BaseItem.УспешныйКрафт` (`self.Bp Baseitem`))
              (:`then`
                _)
              (:`else`
                _))
            (bind _foundwidgets (`WidgetBlueprintLibrary.GetAllWidgetsOfClass` "/Game/Shimaletik/Cursors/A1W.A1W_C" false))
            (bind _output (`|GetArrayItem` _foundwidgets))
            (`/Engine/EditorBlueprintResources/StandardMacros.IsValid` _output
              (:`Is Valid`
                (set `/Game/Shimaletik/Cursors/A1W.tupsCursor` "NewEnumerator0" _output)))))
        (:`Is Not Valid`
          (`KismetSystemLibrary.PrintString` "Error Bp_baseItem not valid playChinematik_Cliced")
          (goto _label)))
      (else
        (goto _label)))))

(event `Crafting Event`
  (params (Condition :type Boolean) (Bp_baseitem :type "/Game/_Props_2/Core/Blueprints/Items/BP_BaseItem Object Reference"))
  ;[1 1 1] Исользовать в чаилдах для испелнения кода карфта
)

(event `/Game/_Props_2/Core/Blueprints/Interface/BP_Info.ClicedMouse`
  (params (PrimComp :type "PrimitiveComponent Object Reference"))
  (`GameplayStatics.PlaySound2D` (`self.ЗвукКогда Кликаеш`) 1.0 1.0 0.0 null null))

(event `CDestroy`
  (params (Destroy :type Boolean))
  (bind _meshitem (`self.MeshItem`))
  (bind _qests (`self.Qests`))
  (bind _returnvalue (`SceneComponent.K2_GetComponentScale` _meshitem))
  (`|ExecutionSequence`
    (:`then_0`
      (if (not Destroy)
        (`/Engine/EditorBlueprintResources/StandardMacros.IsValid` _qests
          (:`Is Valid`
            (`/Game/Shimaletik/Blueprints/Qests/quests.Qest update stat` _qests self "NewEnumerator0")))))
    (:`then_1`
      (`self.SetActorEnableCollision` false)
      (if (not (== _returnvalue (0.0 0.0 0.0)))
        (`/Engine/EditorBlueprintResources/StandardMacros.DoOnce` false :!label _label_3
          (:`Completed`
            (set `self.Self scale` _returnvalue)
            (set `self.FinishedScale` false)
            (`PrimitiveComponent.SetSimulatePhysics` _meshitem false)
            (bind (_direction _newtrack_0) (`Timeline|Timeline_0` :!via `PlayFromStart`)
              (:`Update`
                (`SceneComponent.SetWorldScale3D` (`self.MeshItem`) (`KismetMathLibrary.VLerp` (0.0 0.0 0.0) (`self.Self scale`) _newtrack_0)))
              (:`Finished`
                (if Destroy
                  (`self.K2_DestroyActor`)
                  (else
                    (`self.K2_AddActorWorldOffset` (0.0 0.0 50000.0))
                    (set `self.FinishedScale` true)
                    (goto _label_3 :!via `Reset`)))))))))))

(event `Cspawn`
  (bind (_direction _newtrack_2) (`Timeline|Timeline_1` :!via `PlayFromStart`)
    (:`Update`
      (`SceneComponent.SetWorldScale3D` (`self.MeshItem`) (`KismetMathLibrary.VLerp` (0.0 0.0 0.0) (`self.Self scale`) _newtrack_2)))))

(fn `CraftOrUseItem`
  (params (Item :type "/Game/_Props_2/Core/Blueprints/Items/BP_BaseItem Object Reference")))

(fn `FQest`
  (params (Enum_QestTupe :type "/Game/Shimaletik/Blueprints/Qests/Enum_QestTupe Enum" :default "NewEnumerator0"))
  (bind _qests (`self.Qests`))
  (`/Engine/EditorBlueprintResources/StandardMacros.IsValid` _qests
    (:`Is Valid`
      (`/Game/Shimaletik/Blueprints/Qests/quests.Qest update stat` _qests self Enum_QestTupe))))

(fn `Interact`
  (returns (Valid :type Boolean))
  (return false))

(fn `PlaySoundUseItem`
  (`GameplayStatics.PlaySoundAtLocation` (`self.Sound`) (`self.K2_GetActorLocation`) (struct) 1.0 1.0 0.0 null null null))

(fn `UpdateRespawn`
  (locals (NewLocalVar_0 :type Integer :default 0))
  (bind _returnvalue (`GameplayStatics.GetActorOfClass` "/Game/Shimaletik/ContoledItemMap.ContoledItemMap_C"))
  (`/Engine/EditorBlueprintResources/StandardMacros.IsValid` _returnvalue
    (:`Is Valid`
      (bind _out_actors (`/Game/Shimaletik/ContoledItemMap.Out Actors` _returnvalue))
      (for (_array_element _array_index) _out_actors
        (if (== (`.Item_5_BAB1941C41DB1BBB561E648D00D5BC36` (break `/Game/Shimaletik/ReturnItemLcoation` _array_element)) self)
          (`|ExecutionSequence`
            (:`then_0`
              (`KismetArrayLibrary.Array_Set` _out_actors _array_index (make `/Game/Shimaletik/ReturnItemLcoation` self (`self.GetTransform`))))
            (:`then_1`
              (break))))))))

(fn `UseItem`
  (params (Item :type "Actor Object Reference"))
  (`self.PlaySoundUseItem`)
  (return))

(fn `UserConstructionScript`)