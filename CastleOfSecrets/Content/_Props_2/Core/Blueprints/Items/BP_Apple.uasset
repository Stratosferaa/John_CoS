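; BP_Apple is an apple item Blueprint with very little logic of its own.
; CraftingEvent nudges the actor up along its local Z axis without sweeping.
; Tick prints the mobility of MeshItem and AddColision every frame as on-screen debug output.
; The construction script only calls the parent's, and the BeginPlay and overlap events are disabled stubs.
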(event `self.ReceiveTick`
  (params (DeltaSeconds :type "Float (single-precision)"))
  (`KismetSystemLibrary.PrintString` (`|GetEnumeratorNameAsString` (`SceneComponent.Mobility` (`self.MeshItem`))) true true (struct :`G` 0.155926 :`B` 0.127438 :`A` 1.0) 0.0)
  (`KismetSystemLibrary.PrintString` (`|GetEnumeratorNameAsString` (`SceneComponent.Mobility` (`self.AddColision`))) true true (struct :`R` 0.06445 :`G` 0.155926 :`B` 0.000933 :`A` 1.0) 0.0))

(event `self.Crafting Event`
  (params (Condition :type Boolean) (Bp_baseitem :type "/Game/_Props_2/Core/Blueprints/Items/BP_BaseItem Object Reference"))
  (`self.K2_AddActorLocalOffset` (0.0 0.0 50.0)))

(fn `UserConstructionScript`
  (`parent.UserConstructionScript`))