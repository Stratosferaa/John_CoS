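; BP_PastLocation is a trigger zone that moves a BP_Lest prop into a hard-coded world position and rotation when it enters.
; On Box overlap it clears the player character's HitActor and switches the prop's mesh to WorldStatic collision.
; The MoveLocation timeline then disables physics and drives the root toward the target, lerping from the current mesh location and root rotation each update rather than cached start values.
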(event `self.ReceiveBeginPlay`
  (bind _asmain_character (cast `/Game/_Props_2/Core/Character/Main_Character` (`GameplayStatics.GetPlayerCharacter` 0)))
  (set `self.As Main Character` _asmain_character))

(event `self.Box.OnComponentBeginOverlap`
  (params (OverlappedComponent :type "PrimitiveComponent Object Reference") (OtherActor :type "Actor Object Reference") (OtherComp :type "PrimitiveComponent Object Reference") (OtherBodyIndex :type Integer) (bFromSweep :type Boolean) (SweepResult :type "HitResult Structure (by ref)"))
  (bind _asbp_lest (cast `/Game/_Props_2/Core/Blueprints/Items/BP_Lest` OtherActor :!pure true))
  (bind _rootcomponent (`Actor.RootComponent` _asbp_lest))
  (bind _meshitem (`/Game/_Props_2/Core/Blueprints/Items/BP_Lest.MeshItem` _asbp_lest))
  (`/Engine/EditorBlueprintResources/StandardMacros.IsValid` _asbp_lest
    (:`Is Valid`
      (set `/Game/_Props_2/Core/Character/Main_Character.HitActor` null (`self.As Main Character`))
      (`PrimitiveComponent.SetCollisionObjectType` _meshitem "ECC_WorldStatic")
      (bind (_direction _time) (`Timeline|MoveLocation`)
        (:`Update`
          (`PrimitiveComponent.SetSimulatePhysics` _meshitem false)
          (`SceneComponent.K2_SetWorldLocation` _rootcomponent (`KismetMathLibrary.VLerp` (`SceneComponent.K2_GetComponentLocation` _meshitem) (4042.680908 -3222.171387 6536.623535) _time) false false)
          (`SceneComponent.K2_SetWorldRotation` _rootcomponent (`KismetMathLibrary.RLerp` (`SceneComponent.K2_GetComponentRotation` _rootcomponent) (struct :`Pitch` -1.70224 :`Yaw` 91.92749 :`Roll` -86.996582) _time) false false))))))

(fn `UserConstructionScript`)