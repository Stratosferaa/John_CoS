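; BP_ZoneItemBack is a trigger zone that returns any BP_BaseItem entering it to the player.
; On BeginPlay it caches the player character.
; When an item overlaps its Box, it spawns a fresh actor of the same class at the player's Sprite location, keeping the mesh scale, then destroys the original, so instance state is not copied.
; Its Interact function simply returns false.
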(event `self.ReceiveBeginPlay`
  (bind _ascharacter (cast `/Game/Main/Character` (`GameplayStatics.GetPlayerCharacter` 0)))
  (set `self.As Main Character` _ascharacter))

(event `self.Box.OnComponentBeginOverlap`
  (params (OverlappedComponent :type "PrimitiveComponent Object Reference") (OtherActor :type "Actor Object Reference") (OtherComp :type "PrimitiveComponent Object Reference") (OtherBodyIndex :type Integer) (bFromSweep :type Boolean) (SweepResult :type "HitResult Structure (by ref)"))
  (bind _asbp_base_item (cast `/Game/_Props_2/Core/Blueprints/Items/BP_BaseItem` OtherActor))
  (`/Engine/EditorBlueprintResources/StandardMacros.IsValid` _asbp_base_item
    (:`Is Valid`
      (`|SpawnActorFromClass` (`GameplayStatics.GetObjectClass` _asbp_base_item) (`KismetMathLibrary.MakeTransform` (`SceneComponent.K2_GetComponentLocation` (`PaperCharacter.Sprite` (`self.As Main Character`))) (struct) (`SceneComponent.K2_GetComponentScale` (`/Game/_Props_2/Core/Blueprints/Items/BP_BaseItem.MeshItem` _asbp_base_item))) "Undefined" "OverrideRootScale" null true null)
      (`self.K2_DestroyActor` _asbp_base_item))))

(fn `Interact`
  (returns (Valid :type Boolean))
  (return false))

(fn `UserConstructionScript`)