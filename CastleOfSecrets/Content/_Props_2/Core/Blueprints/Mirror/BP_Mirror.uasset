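; BP_Mirror is an interactive mirror prop that accepts a placed stone and can be tilted up or down.
; InfoInteraction toggles custom-depth highlighting, while RotateUp and RotateDown step the mirror mesh's roll.
; StonePut destroys the passed actor, reveals the built-in stone and slides a scene component by timeline.
; It then plays a level sequence with player input disabled while a second timeline rotates the mirror, and a timer restores input.
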(event `/Game/_Props_2/Core/Blueprints/Interface/BP_Info.InfoInteraction`
  (params (Char :type "/Game/Main/Character Object Reference") (On :type Boolean) (HitComponent :type "PrimitiveComponent Object Reference"))
  (`PrimitiveComponent.SetRenderCustomDepth` (`self.ZERKALO_Plane`) On)
  (`PrimitiveComponent.SetRenderCustomDepth` (`self.StaticMesh1`) On))

(event `self.ReceiveBeginPlay`
  ;[1 1 1] BeginPlay
  (bind _ascharacter (cast `/Game/Main/Character` (`self.GetOwner`)))
  (set `self.CharacterRef` _ascharacter))

(event `StonePut`
  (params (Target :type "Actor Object Reference"))
  (bind _cutscene (`self.CutScene`))
  ;[1 1 1] MoveStone
  (`self.K2_DestroyActor` Target)
  (`SceneComponent.SetVisibility` (`self.StoneMesh`) true false)
  (bind (_direction _move) (`Timeline|Timeline_0` :!via `PlayFromStart`)
    (:`Update`
      (`SceneComponent.K2_AddLocalOffset` (`self.Scene`) (`KismetMathLibrary.MakeVector` _move) false false))
    (:`Finished`
      (`|ExecutionSequence`
        (:`then_0`
          (bind (_outactor _returnvalue) (`LevelSequencePlayer.CreateLevelSequencePlayer` (`self.Player`)))
          (set `self.CutScene` _returnvalue))
        (:`then_1`
          (`self.DisableInput` (`GameplayStatics.GetPlayerController` 0))
          (`MovieSceneSequencePlayer.Play` _cutscene)
          (`KismetSystemLibrary.K2_SetTimerDelegate` (delegate `EndPlay`) (`TimeManagementBlueprintLibrary.Conv_QualifiedFrameTimeToSeconds` (`MovieSceneSequencePlayer.GetEndTime` _cutscene)))
          (bind (_direction_2 _move_2) (`Timeline|Timeline_1` :!via `PlayFromStart`)
            (:`Update`
              (`SceneComponent.K2_AddLocalRotation` (`self.StaticMesh1`) (`KismetMathLibrary.MakeRotator` _move_2) false false))))))))

(event `RotateUp`
  ;[1 1 1] RotateMirror
  (bind _result (`/Engine/EditorBlueprintResources/StandardMacros.IncrementFloat` (`self.UPRotate`))
    (:`  `
      (`SceneComponent.K2_AddLocalRotation` (`self.StaticMesh1`) (`KismetMathLibrary.MakeRotator` _result) false false)
      (set `self.UPRotate` 6.0))))

(event `RotateDown`
  ;[1 1 1] RotateMirror
  (bind _result (`/Engine/EditorBlueprintResources/StandardMacros.DecrementFloat` (`self.DownRotate`))
    (:`  `
      (`SceneComponent.K2_AddLocalRotation` (`self.StaticMesh1`) (`KismetMathLibrary.MakeRotator` _result) false false)
      (set `self.DownRotate` -6.0))))

(event `EndPlay`
  (`self.EnableInput` (`GameplayStatics.GetPlayerController` 0))
  (`MovieSceneSequencePlayer.Stop` (`self.CutScene`)))

(fn `UserConstructionScript`)