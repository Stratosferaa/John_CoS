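; HUD_Play is the play HUD Blueprint that sets up cursor and input mode for the main controller on BeginPlay.
; It caches player 0 as Main-Controller, then calls CreateGamePlayWidget and SetShowMouseCursor.
; The cursor helper switches between Game And UI input focused on WGamePlay and Game Only.
; CreateGamePlayWidget only branches on its flag, as its UI_HUD creation and viewport nodes are disconnected, so it creates no widget.
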(event `self.ReceiveBeginPlay`
  (bind _asmain__controller (cast `/Game/Main/Main-Controller` (`GameplayStatics.GetPlayerController` 0)))
  (set `self.RefToPC` _asmain__controller)
  (`self.CreateGamePlayWidget` true)
  (`self.Set Show Mouse Cursor` true (`self.W_GamePlay`)))

(fn `CreateGamePlayWidget`
  (params (Create :type Boolean))
  (if Create
    _))

(fn `Set Show Mouse Cursor`
  (params (Show :type Boolean) (InWidgetToFocus :type "Widget Object Reference"))
  (bind _reftopc (`self.RefToPC`))
  (bind _reftopc_2 (`self.RefToPC`))
  (if Show
    (set `PlayerController.bShowMouseCursor` true _reftopc_2)
    (`WidgetBlueprintLibrary.SetInputMode_GameAndUIEx` _reftopc InWidgetToFocus "DoNotLock" false)
    (else
      (set `PlayerController.bShowMouseCursor` false _reftopc_2)
      (`WidgetBlueprintLibrary.SetInputMode_GameOnly` _reftopc))))

(fn `UserConstructionScript`)