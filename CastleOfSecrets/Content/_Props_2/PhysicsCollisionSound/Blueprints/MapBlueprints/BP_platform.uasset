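; BP_platform is a moving platform that shuttles back and forth along its relative Y axis.
; On BeginPlay it stores the start location and an end with Y set to 1000, waits briefly, then starts a timeline that lerps the Platform component between them.
; A FlipFlop on the timeline's finish alternates reverse and forward playback after a short pause, looping the motion without Tick or sweep collision.
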(event `self.ReceiveBeginPlay`
  (bind _relativelocation (`SceneComponent.RelativeLocation` (`self.platform`)))
  (set `self.pos1` 1000.0)
  (set `self.Start_Loc` _relativelocation)
  (set `self.End_Loc` (`KismetMathLibrary.MakeVector` (.x _relativelocation) (`self.pos1`) (.z _relativelocation)))
  (`KismetSystemLibrary.Delay` 3.0)
  (bind (_direction _newtrack_0) (`Timeline|Timeline_0` :!label _label)
    (:`Update`
      (`SceneComponent.K2_SetRelativeLocation` (`self.platform`) (`KismetMathLibrary.VLerp` (`self.Start_Loc`) (`self.End_Loc`) _newtrack_0) false false))
    (:`Finished`
      (`/Engine/EditorBlueprintResources/StandardMacros.FlipFlop`
        (:`A`
          (`KismetSystemLibrary.Delay` 0.3)
          (goto _label :!via `ReverseFromEnd`))
        (:`B`
          (`KismetSystemLibrary.Delay` 0.3)
          (goto _label :!via `PlayFromStart`))))))

(event `self.ReceiveTick`
  (params (DeltaSeconds :type "Float (single-precision)")))

(fn `UserConstructionScript`)