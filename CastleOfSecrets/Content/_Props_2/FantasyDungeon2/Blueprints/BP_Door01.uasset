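; Dungeon door prop that either slides or swings open, automatically on overlap or once via the E key.
; Collision overlaps set open/close flags for auto doors, or show a prompt widget and open a Gate for E input on manual doors, which never close.
; Tick steps position or yaw by a fixed amount per frame to clamped limits, so speed is frame-rate dependent.
; Construction script picks the entrance mesh and shows arrows matching the motion type.
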(event `self.Collision.OnComponentEndOverlap`
  (params (OverlappedComponent :type "PrimitiveComponent Object Reference") (OtherActor :type "Actor Object Reference") (OtherComp :type "PrimitiveComponent Object Reference") (OtherBodyIndex :type Integer))
  ;[1 1 1] Overlap collision
  (set `self.Auto Close` true)
  (set `self.Auto Open` false)
  (`WidgetLayoutLibrary.RemoveAllWidgets`))

(event `Key|E`
  (params (Key :type "Key Structure"))
  ;[1 1 1] Press key E
  (:`Pressed`
    (`/Engine/EditorBlueprintResources/StandardMacros.Gate` true :!label _label
      (:`Exit`
        (set `self.Opened` true)
        (`WidgetLayoutLibrary.RemoveAllWidgets`)
        (set `self.Door Open` true)))))

(event `self.Collision.OnComponentBeginOverlap`
  (params (OverlappedComponent :type "PrimitiveComponent Object Reference") (OtherActor :type "Actor Object Reference") (OtherComp :type "PrimitiveComponent Object Reference") (OtherBodyIndex :type Integer) (bFromSweep :type Boolean) (SweepResult :type "HitResult Structure (by ref)"))
  ;[1 1 1] Overlap collision
  (set `self.Auto Close` false)
  (set `self.Auto Open` true)
  ;[1 1 1] Press key E
  (if (`self.AutoDoor`)
    _
    (elif (not (`self.Door Open`))
      (bind _returnvalue (`|CreateWidget` "/Game/_Props_2/FantasyDungeon2/Blueprints/BP_PressE_Widget.BP_PressE_Widget_C"))
      (`UserWidget.AddToViewport` _returnvalue 0)
      (`self.EnableInput` (`GameplayStatics.GetPlayerController` 0))
      (goto _label :!via `Open`))))

(event `self.ReceiveTick`
  (params (DeltaSeconds :type "Float (single-precision)"))
  (bind _doorposition (`self.DoorPosition`))
  (bind _doorrotation (`self.DoorRotation`))
  (bind _door (`self.Door`))
  (bind _doorposition_2 (`self.DoorPosition`))
  (bind _doorrotation_2 (`self.DoorRotation`))
  (if (`self.AutoDoor`)
    ;[1 1 1] Door open
    (if (`self.Auto Open`)
      (if (`self.Door move/rotation`) :!label _label_2
        ;;[1 1 1] Move
        (`/Engine/EditorBlueprintResources/StandardMacros.CompareFloat` _doorposition 54.0
          (:`>`
            (set `self.DoorPosition` 54.0 :!label _label_3)
            (set `self.Auto Open` false)
            (set `self.Opened` false))
          (:`==`
            (goto _label_3))
          (:`<`
            (set `self.DoorPosition` (+ _doorposition 1.0))
            (`SceneComponent.K2_SetRelativeLocation` _door (`KismetMathLibrary.MakeVector` 0.0 (`self.DoorPosition`)) false false :!label _label_4)))
        (else
          ;;[1 1 1] Rotation
          (`/Engine/EditorBlueprintResources/StandardMacros.CompareFloat` _doorrotation 90.0
            (:`>`
              (set `self.DoorRotation` 90.0 :!label _label_5)
              (set `self.Auto Open` false)
              (set `self.Opened` false))
            (:`==`
              (goto _label_5))
            (:`<`
              (set `self.DoorRotation` (+ _doorrotation 1.0))
              (`SceneComponent.K2_SetRelativeRotation` _door (`KismetMathLibrary.MakeRotator` 0.0 0.0 (`self.DoorRotation`)) false false :!label _label_6)))))
      (else
        ;[1 1 1] Door close
        (if (`self.Auto Close`)
          (if (`self.Door move/rotation`)
            ;;[1 1 1] Move
            (`/Engine/EditorBlueprintResources/StandardMacros.CompareFloat` _doorposition_2 -56.950001
              (:`>`
                (set `self.DoorPosition` (- _doorposition_2 1.0))
                (goto _label_4))
              (:`==`
                _)
              (:`<`
                _))
            (set `self.DoorPosition` -56.950001)
            (set `self.Auto Close` false)
            (else
              ;;[1 1 1] Rotation
              (`/Engine/EditorBlueprintResources/StandardMacros.CompareFloat` _doorrotation_2
                (:`>`
                  (set `self.DoorRotation` (- _doorrotation_2 1.0))
                  (goto _label_6))
                (:`==`
                  _)
                (:`<`
                  _))
              (set `self.DoorRotation` 0.0)
              (set `self.Auto Close` false))))))
    (elif (`self.Opened`)
      (goto _label_2))))

(fn `UserConstructionScript`
  (bind _entrance (`self.Entrance`))
  (switch `int` (`self.EntranceVar`)
    (:`Default`
      (`StaticMeshComponent.SetStaticMesh` _entrance "/Game/_Props_2/FantasyDungeon2/Meshes/Door/SM_Entrance01.SM_Entrance01" :!label _label))
    (:`0`
      (goto _label))
    (:`1`
      (`StaticMeshComponent.SetStaticMesh` _entrance "/Game/_Props_2/FantasyDungeon2/Meshes/Door/SM_Entrance02.SM_Entrance02")))
  (if (`self.Door move/rotation`)
    (`SceneComponent.SetVisibility` (`self.Arrow1`) true false)
    (`SceneComponent.SetVisibility` (`self.Arrow`) true false)
    (`SceneComponent.SetVisibility` (`self.Arrow3`) false false)
    (`SceneComponent.SetVisibility` (`self.Arrow7`) false false)
    (`SceneComponent.SetVisibility` (`self.Arrow6`) false false)
    (`SceneComponent.SetVisibility` (`self.Arrow5`) false false)
    (`SceneComponent.SetVisibility` (`self.Arrow4`) false false)
    (`SceneComponent.SetVisibility` (`self.Arrow2`) false false)
    (else
      (`SceneComponent.SetVisibility` (`self.Arrow1`) false false)
      (`SceneComponent.SetVisibility` (`self.Arrow`) false false)
      (`SceneComponent.SetVisibility` (`self.Arrow3`) true false)
      (`SceneComponent.SetVisibility` (`self.Arrow7`) true false)
      (`SceneComponent.SetVisibility` (`self.Arrow6`) true false)
      (`SceneComponent.SetVisibility` (`self.Arrow5`) true false)
      (`SceneComponent.SetVisibility` (`self.Arrow4`) true false)
      (`SceneComponent.SetVisibility` (`self.Arrow2`) true false))))