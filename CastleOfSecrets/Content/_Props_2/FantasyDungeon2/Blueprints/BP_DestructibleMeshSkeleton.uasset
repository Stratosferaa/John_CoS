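; Destructible skeleton prop that shows a static mesh at range and swaps to a destructible mesh when the player is near.
; Until broken, Tick compares player distance to a view-distance threshold and toggles visibility.
; The first hit applies radius damage at the impact point and changes the collision object type to avoid player interaction.
; After a short delay it zeroes Impulse and sets Break, stopping the distance-based swap.
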(event `self.ReceiveTick`
  (params (DeltaSeconds :type "Float (single-precision)"))
  (bind _destructible_mesh (`self.Destructible Mesh`))
  (bind _static_mesh (`self.Static Mesh`))
  ;[1 1 1] If object not break
  (if (not (`self.Break`))
    ;[1 1 1] get information how close the player is to the object
    (`/Engine/EditorBlueprintResources/StandardMacros.CompareFloat` (`KismetMathLibrary.Vector_Distance` (`SceneComponent.K2_GetComponentLocation` (`Actor.RootComponent` (`GameplayStatics.GetPlayerCharacter` 0))) (`SceneComponent.K2_GetComponentLocation` (`self.DefaultSceneRoot`))) (`self.Destructable Mesh View Distance`)
      (:`>`
        ;[1 1 1] if the player is close enough, switch the object from static mesh to destructible mesh. if the object is break, then the mesh does not switch
        (`SceneComponent.SetVisibility` _static_mesh true false)
        (`SceneComponent.SetVisibility` _destructible_mesh false false))
      (:`==`
        (`SceneComponent.SetVisibility` _static_mesh false false :!label _label)
        (`SceneComponent.SetVisibility` _destructible_mesh true false))
      (:`<`
        (goto _label)))))

(event `self.Destructible Mesh.OnComponentHit`
  (params (HitComponent :type "PrimitiveComponent Object Reference") (OtherActor :type "Actor Object Reference") (OtherComp :type "PrimitiveComponent Object Reference") (NormalImpulse :type "Vector Structure") (Hit :type "HitResult Structure (by ref)"))
  (bind _destructible_mesh (`self.Destructible Mesh`))
  ;[1 1 1] when object takes damage, it changes the collision channel in order not to interact with the player
  (if (`self.Break`)
    (goto _label)
    (else
      (`self.ApplyRadiusDamage` _destructible_mesh 100.0 (`.ImpactPoint` (`GameplayStatics.BreakHitResult` Hit)) 10.0 0.0 false)
      (`PrimitiveComponent.SetCollisionObjectType` _destructible_mesh "ECC_Visibility")
      (`KismetSystemLibrary.Delay` 0.3)
      (set `self.impulse` 0.0)
      (set `self.Break` true))))

(fn `UserConstructionScript`)