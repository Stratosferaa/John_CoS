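; BP_PhysicsChain is a prop that builds a physically simulated chain along an editable spline.
; The construction script samples the spline at intervals of spacing times chain size, placing a scaled mesh link at each point and a physics constraint slightly behind it.
; Each constraint joins a link to the previous one, and an option disables simulation on the last link to pin that end.
; The event graph is empty.
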(event `self.ReceiveBeginPlay`)

(event `self.ReceiveTick`
  (params (DeltaSeconds :type "Float (single-precision)")))

(fn `UserConstructionScript`
  (bind _chain_size (`self.Chain Size`))
  (bind _spline (`self.Spline`))
  (bind _spacing (`self.Spacing`))
  (bind _mesh (`self.Mesh`))
  (bind _returnvalue (`KismetMathLibrary.Conv_DoubleToVector` _chain_size))
  (bind _returnvalue_2 (* _spacing _chain_size))
  (`KismetArrayLibrary.Array_Clear` (`self.Physics Constrain Transform`))
  (`KismetArrayLibrary.Array_Clear` (`self.Mesh`))
  (`KismetArrayLibrary.Array_Clear` (`self.Base mesh transform`))
  (for _index (range (+ (`.ReturnValue` (`KismetMathLibrary.FMod` (`SplineComponent.GetSplineLength` _spline) _returnvalue_2)) 1))
    (bind _returnvalue_3 (* _index _returnvalue_2))
    (`KismetArrayLibrary.Array_Add` (`self.Base mesh transform`) (`KismetMathLibrary.MakeTransform` (`SplineComponent.GetLocationAtDistanceAlongSpline` _spline _returnvalue_3 "Local") (`SplineComponent.GetRotationAtDistanceAlongSpline` _spline _returnvalue_3 "Local") _returnvalue))
    (bind _returnvalue_4 (- (* _index _returnvalue_2) (/ _spacing 2.0)))
    (`KismetArrayLibrary.Array_Add` (`self.Physics Constrain Transform`) (`KismetMathLibrary.MakeTransform` (`SplineComponent.GetLocationAtDistanceAlongSpline` _spline _returnvalue_4 "Local") (`SplineComponent.GetRotationAtDistanceAlongSpline` _spline _returnvalue_4 "Local") _returnvalue)))
  (for (_array_element _array_index) (`self.Base mesh transform`)
    (bind _returnvalue_5 (`AddComponent|NODE_AddPhysicsConstraintComponent-0` :`RelativeTransform` (`|GetArrayItem` (`self.Physics Constrain Transform`) _array_index)))
    (bind _returnvalue_6 (`AddComponent|NODE_AddStaticMeshComponent-0` :`RelativeTransform` _array_element))
    (`KismetArrayLibrary.Array_Add` (`self.Mesh`) _returnvalue_6)
    (`PhysicsConstraintComponent.SetConstrainedComponents` _returnvalue_5 (`|GetArrayItem` _mesh _array_index) "None" (`|GetArrayItem` _mesh (- _array_index 1)) "None"))
  (if (`self.Lock last point`)
    (`PrimitiveComponent.SetSimulatePhysics` (`|GetArrayItem` (`self.Mesh`) _array_index) false)))