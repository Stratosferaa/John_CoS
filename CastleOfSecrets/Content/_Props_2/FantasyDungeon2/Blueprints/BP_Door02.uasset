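; Double dungeon door that either slides apart or swings open, selected by DoorMoverotation, with automatic or press-E operation set by AutoDoor.
; Collision overlap drives auto open and close, or in manual mode shows a prompt and opens a gate for E; manual doors never close.
; Tick steps both leaves in mirrored, fixed per-frame increments to hard-coded limits, without a Timeline.
; The construction script shows direction arrows matching the chosen motion type.
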(event `Key|E`
  (params (Key :type "Key Structure"))
  ;[1 1 1] Press key E
  (:`Pressed`
    (`/Engine/EditorBlueprintResources/StandardMacros.Gate` true :!label _label
      (:`Exit`
        (set `self.Opened` true)
        (`WidgetLayoutLibrary.RemoveAllWidgets`)
        (set `self.Door Open` true)))))

(event `self.Collision.OnComponentEndOverlap`
  (params (OverlappedComponent :type "PrimitiveComponent Object Reference") (OtherActor :type "Actor Object Reference") (OtherComp :type "PrimitiveComponent Object Reference") (OtherBodyIndex :type Integer))
  ;[1 1 1] Overlap collision
  (set `self.Auto Close` true)
  (set `self.Auto Open` false)
  (`WidgetLayoutLibrary.RemoveAllWidgets`))

(event `self.Collision.OnComponentBeginOverlap`
  (params (OverlappedComponent :type "PrimitiveComponent Object Reference") (OtherActor :type "Actor Object Reference") (OtherComp :type "PrimitiveComponent Object Reference") (OtherBodyIndex :type Integer) (bFromSweep :type Boolean) (SweepResult :type "HitResult Structure (by ref)"))
  ;[1 1 1] Overlap collision
  (set `self.Auto Close` false)
  (set `self.Auto Open` true)
  ;[1 1 1] Press key E
  (if (`self.AutoDoor`)
    _
    (elif (not (`self.Door Open`))
      (bind _returnvalue (`|CreateWidget` "/Game/_Props_2/FantasyDungeon2/Blueprints/BP_PressE_Widget.BP_PressE_Widget_C"))
      (`UserWidget.AddToViewport` _returnvalue 0)
      (`self.EnableInput` (`GameplayStatics.GetPlayerController` 0))
      (goto _label :!via `Open`))))

(event `self.ReceiveTick`
  (params (DeltaSeconds :type "Float (single-precision)"))
  (bind _doorrotation (`self.DoorRotation`))
  (bind _doorr (`self.DoorR`))
  (bind _doorposition (`self.DoorPosition`))
  (bind _doorposition_2 (`self.DoorPosition`))
  (bind _doorposition_3 (`self.DoorPosition`))
  (bind _doorl (`self.DoorL`))
  (bind _doorrotation_2 (`self.DoorRotation`))
  (bind _doorrotation_3 (`self.DoorRotation`))
  (if (`self.AutoDoor`)
    ;[1 1 1] Door open
    (if (`self.Auto Open`)
      (if (`self.Door move/rotation`) :!label _label_2
        ;;[1 1 1] Move
        (`/Engine/EditorBlueprintResources/StandardMacros.CompareFloat` _doorposition_2 303.0
          (:`>`
            (set `self.DoorPosition` 303.0)
            (set `self.Auto Open` false)
            (set `self.Opened` false))
          (:`==`
            (set `self.DoorPosition` (+ _doorposition_2 1.0) :!label _label_3)
            (`SceneComponent.K2_SetRelativeLocation` _doorl (`KismetMathLibrary.MakeVector` 0.0 _doorposition) false false :!label _label_4)
            (`SceneComponent.K2_SetRelativeLocation` _doorr (`KismetMathLibrary.MakeVector` 0.0 (* _doorposition -1.0)) false false))
          (:`<`
            (goto _label_3)))
        (else
          ;;[1 1 1] Rotation
          (`/Engine/EditorBlueprintResources/StandardMacros.CompareFloat` _doorrotation -270.0
            (:`>`
              (set `self.DoorRotation` (- _doorrotation 1.0))
              (`SceneComponent.K2_SetRelativeRotation` _doorl (`KismetMathLibrary.MakeRotator` 0.0 0.0 _doorrotation_2) false false :!label _label_5)
              (`SceneComponent.K2_SetRelativeRotation` _doorr (`KismetMathLibrary.MakeRotator` 0.0 0.0 (+ (* _doorrotation_2 -1.0) 180.0)) false false))
            (:`==`
              (set `self.DoorRotation` -270.0 :!label _label_6)
              (set `self.Auto Open` false)
              (set `self.Opened` false))
            (:`<`
              (goto _label_6)))))
      (else
        ;[1 1 1] Door close
        (if (`self.Auto Close`)
          (if (`self.Door move/rotation`)
            ;;[1 1 1] Move
            (`/Engine/EditorBlueprintResources/StandardMacros.CompareFloat` _doorposition_3 153.0
              (:`>`
                (set `self.DoorPosition` (- _doorposition_3 1.0))
                (goto _label_4))
              (:`==`
                _)
              (:`<`
                _))
            (set `self.DoorPosition` 153.0)
            (set `self.Auto Close` false)
            (else
              ;;[1 1 1] Rotation
              (`/Engine/EditorBlueprintResources/StandardMacros.CompareFloat` _doorrotation_3 -180.0
                (:`>`
                  _)
                (:`==`
                  _)
                (:`<`
                  (set `self.DoorRotation` (+ _doorrotation_3 1.0))
                  (goto _label_5)))
              (set `self.DoorRotation` -180.0)
              (set `self.Auto Close` false))))))
    (elif (`self.Opened`)
      (goto _label_2))))

(fn `UserConstructionScript`
  (if (`self.Door move/rotation`)
    (`SceneComponent.SetVisibility` (`self.Arrow`) true false)
    (`SceneComponent.SetVisibility` (`self.Arrow1`) true false)
    (`SceneComponent.SetVisibility` (`self.Arrow3`) true false)
    (`SceneComponent.SetVisibility` (`self.Arrow2`) true false)
    (`SceneComponent.SetVisibility` (`self.Arrow15`) false false)
    (`SceneComponent.SetVisibility` (`self.Arrow14`) false false)
    (`SceneComponent.SetVisibility` (`self.Arrow13`) false false)
    (`SceneComponent.SetVisibility` (`self.Arrow12`) false false)
    (`SceneComponent.SetVisibility` (`self.Arrow11`) false false)
    (`SceneComponent.SetVisibility` (`self.Arrow5`) false false)
    (`SceneComponent.SetVisibility` (`self.Arrow10`) false false)
    (`SceneComponent.SetVisibility` (`self.Arrow9`) false false)
    (`SceneComponent.SetVisibility` (`self.Arrow8`) false false)
    (`SceneComponent.SetVisibility` (`self.Arrow7`) false false)
    (`SceneComponent.SetVisibility` (`self.Arrow6`) false false)
    (`SceneComponent.SetVisibility` (`self.Arrow4`) false false)
    (else
      (`SceneComponent.SetVisibility` (`self.Arrow`) false false)
      (`SceneComponent.SetVisibility` (`self.Arrow1`) false false)
      (`SceneComponent.SetVisibility` (`self.Arrow3`) false false)
      (`SceneComponent.SetVisibility` (`self.Arrow2`) false false)
      (`SceneComponent.SetVisibility` (`self.Arrow15`) true false)
      (`SceneComponent.SetVisibility` (`self.Arrow14`) true false)
      (`SceneComponent.SetVisibility` (`self.Arrow13`) true false)
      (`SceneComponent.SetVisibility` (`self.Arrow12`) true false)
      (`SceneComponent.SetVisibility` (`self.Arrow11`) true false)
      (`SceneComponent.SetVisibility` (`self.Arrow5`) true false)
      (`SceneComponent.SetVisibility` (`self.Arrow10`) true false)
      (`SceneComponent.SetVisibility` (`self.Arrow9`) true false)
      (`SceneComponent.SetVisibility` (`self.Arrow8`) true false)
      (`SceneComponent.SetVisibility` (`self.Arrow7`) true false)
      (`SceneComponent.SetVisibility` (`self.Arrow6`) true false)
      (`SceneComponent.SetVisibility` (`self.Arrow4`) true false))))