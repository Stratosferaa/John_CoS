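; Construction-script Blueprint that builds spline meshes along an editable spline, apparently a background ring of trees for the cemetery pack.
; For each segment of SplineRoad, it adds a SplineMeshComponent attached to Scene, with start and end positions and tangents taken from adjacent spline points in local space.
; The loop does not create a closing segment from the last point to the first, and the event graph has no active logic.
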(fn `UserConstructionScript`
  (bind _splineroad (`self.SplineRoad`))
  (for _index (range (+ (- (`SplineComponent.GetNumberOfSplinePoints` _splineroad) 2) 1))
    (bind _returnvalue (`AddComponent|NODE_AddSplineMeshComponent-1` :`bManualAttachment` true))
    (`SceneComponent.K2_AttachTo` _returnvalue (`self.Scene`) "None" "KeepRelativeOffset" true)
    (bind (_location _tangent) (`SplineComponent.GetLocationAndTangentAtSplinePoint` _splineroad _index "Local"))
    (bind (_location_2 _tangent_2) (`SplineComponent.GetLocationAndTangentAtSplinePoint` _splineroad (+ _index 1) "Local"))
    (`SplineMeshComponent.SetStartAndEnd` _returnvalue _location _tangent _location_2 _tangent_2 true)))