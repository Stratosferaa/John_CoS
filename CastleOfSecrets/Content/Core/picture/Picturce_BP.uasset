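; Picture Blueprint for an interactive painting that highlights through custom depth and plays a sequence when a paint action succeeds.
; On success it destroys the passed target actor, shows a static mesh and moves it with three chained timelines along Z, X, then Z.
; Between moves the mesh snaps to two scene-component transforms.
; Finally, it hides the mesh and re-enables cloth simulation on the Paint component with a forced reset.
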(event `/Game/Core/Blueprints/Interface/BP_Info.InfoInteraction`
  (params (Char :type "/Game/Main/Character Object Reference") (On :type Boolean) (HitComponent :type "PrimitiveComponent Object Reference"))
  (`PrimitiveComponent.SetRenderCustomDepth` (`self.SM_PaintingDD_SM_PaintingD`) On))

(event `PhysicOn`
  (set `SkeletalMeshComponent.bDisableClothSimulation` false (`self.Paint`))
  (`SkeletalMeshComponent.ForceClothNextUpdateTeleportAndReset` (`self.Paint`)))

(event `SuccesPaint`
  (params (Target :type "Actor Object Reference"))
  (`self.K2_DestroyActor` Target)
  (`SceneComponent.SetVisibility` (`self.StaticMesh`) true false)
  (`self.SuccesMove`))

(event `SuccesMove`
  (bind _staticmesh (`self.StaticMesh`))
  (bind (_returnvalue_x _returnvalue_y _returnvalue_z) (`KismetMathLibrary.BreakVector` (`SceneComponent.K2_GetComponentLocation` (`self.StaticMesh`))))
  (bind (_returnvalue_x_2 _returnvalue_y_2 _returnvalue_z_2) (`KismetMathLibrary.BreakVector` (`SceneComponent.K2_GetComponentLocation` (`self.StaticMesh`))))
  (bind (_returnvalue_x_3 _returnvalue_y_3 _returnvalue_z_3) (`KismetMathLibrary.BreakVector` (`SceneComponent.K2_GetComponentLocation` _staticmesh)))
  (bind (_direction _newtrack_0) (`Timeline|Timeline_0` :!via `PlayFromStart`)
    (:`Update`
      (`SceneComponent.K2_SetWorldLocation` (`self.StaticMesh`) (`KismetMathLibrary.MakeVector` _returnvalue_x _returnvalue_y (+ _returnvalue_z _newtrack_0)) false false))
    (:`Finished`
      (`SceneComponent.K2_SetWorldLocation` (`self.StaticMesh`) (`SceneComponent.K2_GetComponentLocation` (`self.Scene`)) false true)
      (`SceneComponent.K2_SetWorldRotation` (`self.StaticMesh`) (`SceneComponent.K2_GetComponentRotation` (`self.Scene`)) false false)
      (bind (_direction_2 _newtrack_0_2) (`Timeline|Timeline_1` :!via `PlayFromStart`)
        (:`Update`
          (`SceneComponent.K2_SetWorldLocation` (`self.StaticMesh`) (`KismetMathLibrary.MakeVector` (+ _returnvalue_x_2 _newtrack_0_2) _returnvalue_y_2 _returnvalue_z_2) false false))
        (:`Finished`
          (`SceneComponent.K2_SetWorldLocation` (`self.StaticMesh`) (`SceneComponent.K2_GetComponentLocation` (`self.Scene1`)) false true)
          (`SceneComponent.K2_SetWorldRotation` (`self.StaticMesh`) (`SceneComponent.K2_GetComponentRotation` (`self.Scene1`)) false false)
          (bind (_direction_3 _newtrack_0_3) (`Timeline|Timeline_3` :!via `PlayFromStart`)
            (:`Update`
              (`SceneComponent.K2_SetWorldLocation` _staticmesh (`KismetMathLibrary.MakeVector` _returnvalue_x_3 _returnvalue_y_3 (+ _returnvalue_z_3 _newtrack_0_3)) false false))
            (:`Finished`
              (`SceneComponent.SetVisibility` (`self.StaticMesh`) false false)
              (`self.PhysicOn`))))))))

(fn `UserConstructionScript`)