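; Key is an inventory item that can be lit and spread fire to other objects.
; Using it with BP_Matches while unlit lowers the match count, notifies the inventory and sets IsFire, which the crafting event also sets.
; While lit, its box overlap calls FireSpyd on a BP_Door2, or otherwise Fire on a Torch2.
; CraftOrUseItem simply routes into UseItem after calling its parent.
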(event `self.Crafting Event`
  (params (Condition :type Boolean) (Bp_baseitem :type "/Game/Core/Blueprints/Items/BP_BaseItem Object Reference"))
  (set `self.Used?` true)
  (set `self.IsFire` true))

(event `self.Box_0.OnComponentBeginOverlap`
  (params (OverlappedComponent :type "PrimitiveComponent Object Reference") (OtherActor :type "Actor Object Reference") (OtherComp :type "PrimitiveComponent Object Reference") (OtherBodyIndex :type Integer) (bFromSweep :type Boolean) (SweepResult :type "HitResult Structure (by ref)"))
  (if (`self.IsFire`)
    (bind _asbp_door_2 (cast `/Game/Core/Assets/BP_Door2` OtherActor)
      (:`then`
        (`/Game/Core/Assets/BP_Door2.FireSpyd` _asbp_door_2))
      (:`CastFailed`
        (bind _astorch_2 (cast `/Game/Core/Blueprints/TorhRota/Torch2` OtherActor))
        (`/Game/Core/Blueprints/TorhRota/Torch2.Fire` _astorch_2)))))

(fn `CraftOrUseItem`
  (params (Item :type "/Game/Core/Blueprints/Items/BP_BaseItem Object Reference"))
  (`parent.CraftOrUseItem` Item)
  (`self.UseItem` Item))

(fn `UseItem`
  (params (Item :type "Actor Object Reference"))
  (bind _inventory_component (`/Game/Core/Character/Main_Character.Inventory_Component` (`self.Char`)))
  (`parent.UseItem` Item)
  (bind _asbp_matches (cast `/Game/Core/Blueprints/Items/BP_Matches` Item))
  (if (not (`self.IsFire`))
    (bind _paramitem (`/Game/Core/Blueprints/Items/BP_BaseItem.ParamItem` _asbp_matches))
    (setmembers `/Game/Core/Blueprints/Struct/ST_SlotItem` :`StructRef` _paramitem :`Count` (- (`.Count_11_91D6B62A4073784AF592F887AA26A03F` (break `/Game/Core/Blueprints/Struct/ST_SlotItem` _paramitem)) 1))
    ;[0 1 0.1473] Item+++01
    (`/Game/Core/Components/Inventory_Component.ItemAdded` _inventory_component (`KismetArrayLibrary.Array_Find` (`/Game/Core/Components/Inventory_Component.Items` _inventory_component) _asbp_matches))
    (`KismetSystemLibrary.PrintString` "++++++++")
    (set `self.IsFire` true)))

(fn `UserConstructionScript`
  (`parent.UserConstructionScript`))