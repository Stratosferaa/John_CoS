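; BP_Candle_2 is a candle item that the player lights by using matches on it.
; UseItem accepts only a BP_Matches item on an unlit candle, then lowers the match count by one and notifies the character's InventoryComponent.
; It then sets IsFire and shows the Fire and Light components, with no logic here to extinguish them.
; CraftOrUseItem forwards to the same UseItem logic after calling its parent.
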(fn `CraftOrUseItem`
  (params (Item :type "/Game/Core/Blueprints/Items/BP_BaseItem Object Reference"))
  (`parent.CraftOrUseItem` Item)
  (`self.UseItem` Item))

(fn `UseItem`
  (params (Item :type "Actor Object Reference"))
  (bind _inventory_component (`/Game/Core/Character/Main_Character.Inventory_Component` (`self.Char`)))
  (`parent.UseItem` Item)
  (bind _asbp_matches (cast `/Game/Core/Blueprints/Items/BP_Matches` Item))
  (if (not (`self.IsFire`))
    (bind _paramitem (`/Game/Core/Blueprints/Items/BP_BaseItem.ParamItem` _asbp_matches))
    (setmembers `/Game/Core/Blueprints/Struct/ST_SlotItem` :`StructRef` _paramitem :`Count` (- (`.Count_11_91D6B62A4073784AF592F887AA26A03F` (break `/Game/Core/Blueprints/Struct/ST_SlotItem` _paramitem)) 1))
    ;[0 1 0.1473] Item+++01
    (`/Game/Core/Components/Inventory_Component.ItemAdded` _inventory_component (`KismetArrayLibrary.Array_Find` (`/Game/Core/Components/Inventory_Component.Items` _inventory_component) _asbp_matches))
    (`KismetSystemLibrary.PrintString` "++++++++")
    (set `self.IsFire` true)
    (`SceneComponent.SetVisibility` (`self.Fire`) true false)
    (`SceneComponent.SetVisibility` (`self.Light`) true false)))

(fn `UserConstructionScript`
  (`parent.UserConstructionScript`))