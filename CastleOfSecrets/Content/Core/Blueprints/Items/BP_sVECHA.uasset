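; BP_sVECHA is a candle item that lights up when its crafting event fires.
; CraftingEvent shows three candle fire particle effects and two point lights, sets the Used flag and adds an audio component.
; The construction script only calls its parent, and there is no active tick or overlap logic.
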(event `self.Crafting Event`
  (params (Condition :type Boolean) (Bp_baseitem :type "/Game/Core/Blueprints/Items/BP_BaseItem Object Reference"))
  (`SceneComponent.SetVisibility` (`self.ps_Fire_01_02_Candle2`) true false)
  (`SceneComponent.SetVisibility` (`self.ps_Fire_01_02_Candle1`) true false)
  (`SceneComponent.SetVisibility` (`self.ps_Fire_01_02_Candle`) true false)
  (`SceneComponent.SetVisibility` (`self.PointLight`) true false)
  (`SceneComponent.SetVisibility` (`self.PointLight1`) true false)
  (set `self.Used?` true)
  (`AddComponent|NODE_AddAudioComponent-0`))

(fn `UserConstructionScript`
  (`parent.UserConstructionScript`))