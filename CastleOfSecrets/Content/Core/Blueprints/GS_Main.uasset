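; GS_Main, apparently the main game state, holds a Days counter for the game.
; MinusDays decrements Days and broadcasts the new value through the SetSeconds event dispatcher.
; BeginPlay and Sunrise are empty; disconnected leftover nodes would bind to Ultra Dynamic Sky's sunrise event and duplicate the countdown, but never run.
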(event `self.ReceiveBeginPlay`)

(event `Sunrise`)

(fn `MinusDays`
  (`/Engine/EditorBlueprintResources/StandardMacros.DecrementInt` (`self.Days`)
    (:`  `
      (`self.EventSetSeconds` (`self.Days`)))))

(fn `UserConstructionScript`)