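; Interactable barrel that fills a bucket with water, highlighting via custom depth.
; Interaction or box overlap can drop the bucket from the player's inventory at the trigger box, with BuscerValid tracking its presence.
; If Kran (tap) is set, it spawns BP_Water while a timeline raises the bucket's water level.
; Otherwise, timelines lower the physics-disabled bucket, fill it, then lift it and restore physics.
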(event `self.ReceiveBeginPlay`)

(event `/Game/Core/Blueprints/Interface/BP_Info.InfoInteraction`
  (params (Char :type "/Game/Main/Character Object Reference") (On :type Boolean) (HitComponent :type "PrimitiveComponent Object Reference"))
  (`PrimitiveComponent.SetRenderCustomDepth` (`self.SM_Barrel-02-02`) On))

(event `BarNeValid`
  (bind _bp_bucket (`self.BP_Bucket`))
  (bind (_returnvalue_x _returnvalue_y _returnvalue_z) (`KismetMathLibrary.BreakVector` (`SceneComponent.K2_GetComponentLocation` (`self.Box`))))
  (bind _asmain_character (cast `/Game/Main/Character` (`GameplayStatics.GetPlayerCharacter` 0)))
  (set `self.Char` _asmain_character)
  (`/Game/Core/Components/Inventory_Component.DropItem` (`/Game/Main/Character.Inventory_Component` (`self.Char`)) _bp_bucket (0.0 0.0 0.0))
  (`self.K2_SetActorLocation` _bp_bucket (`KismetMathLibrary.MakeVector` _returnvalue_x _returnvalue_y _returnvalue_z) false true))

(event `Interact_1_1`
  (params (Char :type "/Game/Main/Character Object Reference") (Item :type "/Game/Core/Blueprints/Items/BP_BaseItem Object Reference") (HitComponent :type "PrimitiveComponent Object Reference"))
  (if (`self.BuscerValid`)
    (`self.BP_Bucket`
      (:`then`
        (`self.MaterWaterKran`))
      (:`else`
        (bind _buckettarget (`self.- Check Bucket` Item :!label _label))
        (if _buckettarget
          (set `/Game/Core/Components/Inventory_Component.ItemDragAndDrop` null (`/Game/Main/Character.Inventory_Component` Char))
          (else
            (set `self.BuscerValid` true)
            (`self.BarNeValid`)
            (`self.MaterWaterKran`)))))
    (elif (== (`GameplayStatics.GetObjectClass` Item) (`GameplayStatics.GetObjectClass` (`self.BP_Bucket`)))
      (goto _label))))

(event `NoKran`
  (bind _bp_bucket (`self.BP_Bucket`))
  (bind _meshitem (`/Game/Core/Blueprints/Items/BP_BaseItem.MeshItem` (`self.BP_Bucket`)))
  (bind _meshitem_2 (`/Game/Core/Blueprints/Items/BP_BaseItem.MeshItem` (`self.BP_Bucket`)))
  (bind _water (`/Game/Core/Blueprints/Items/BP_Bucket0.water` _bp_bucket))
  (bind _returnvalue (`SceneComponent.K2_GetComponentToWorld` _meshitem))
  (bind _returnvalue_2 (`SceneComponent.K2_GetComponentToWorld` _meshitem_2))
  (`/Engine/EditorBlueprintResources/StandardMacros.DoOnce` false :!label _label_2
    (:`Completed`
      (if (`self.BuscerValid`)
        (`PrimitiveComponent.SetEnableGravity` _meshitem_2 false)
        (`PrimitiveComponent.SetSimulatePhysics` _meshitem_2 false)
        (bind (_direction _newtrack_0) (`Timeline|Timeline_4` :!via `PlayFromStart`)
          (:`Update`
            (`SceneComponent.K2_SetWorldTransform` _meshitem_2 (`KismetMathLibrary.MakeTransform` (`KismetMathLibrary.MakeVector` (.x (.location _returnvalue_2)) (.y (.location _returnvalue_2)) (- (.z (.location _returnvalue_2)) _newtrack_0)) (.rotation _returnvalue_2) (.scale _returnvalue_2)) false true))
          (:`Finished`
            (`GameplayStatics.PlaySound2D` "/Game/_Props/UltraDynamicSky/Sound/Close_Thunder/CloseThunder_5.CloseThunder_5" 0.5 1.0 0.0 null null)
            (bind (_direction_2 _newtrack_0_2) (`Timeline|Timeline_3` :!via `PlayFromStart` :!label _label_3)
              (:`Update`
                (if (<= _water 10.0)
                  (set `/Game/Core/Blueprints/Items/BP_Bucket0.water` (+ _water _newtrack_0_2) _bp_bucket)
                  (`/Game/Core/Blueprints/Items/BP_Bucket0.-UpdateWidget` (`self.BP_Bucket`))
                  (goto _label_2 :!via `Reset`)
                  (else
                    (set `/Game/Core/Blueprints/Items/BP_Bucket0.IsWater` true _bp_bucket)
                    (if (`self.Kran`)
                      (set `self.BuscerValid` false :!label _label_4)
                      (goto _label_3 :!via `Stop`)
                      (else
                        (bind (_direction_3 _newtrack_0_3) (`Timeline|Timeline_5` :!via `PlayFromStart`)
                          (:`Update`
                            (`SceneComponent.K2_SetWorldTransform` _meshitem (`KismetMathLibrary.MakeTransform` (`KismetMathLibrary.MakeVector` (.x (.location _returnvalue)) (.y (.location _returnvalue)) (+ (.z (.location _returnvalue)) _newtrack_0_3)) (.rotation _returnvalue) (.scale _returnvalue)) false true))
                          (:`Finished`
                            (`PrimitiveComponent.SetEnableGravity` _meshitem true)
                            (`PrimitiveComponent.SetSimulatePhysics` _meshitem true)
                            (goto _label_4))))))))
              (:`Finished`
                (if (>= _water 10.0)
                  (set `/Game/Core/Blueprints/Items/BP_Bucket0.IsWater` true _bp_bucket)
                  (goto _label_2 :!via `Reset`)
                  (else
                    (goto _label_2 :!via `Reset`)))))))
        (else
          (`|ExecutionSequence`
            (:`then_0`
              (goto _label_4))
            (:`then_1`
              (goto _label_2 :!via `Reset`))))))))

(event `MaterWaterKran`
  (bind _bp_bucket (`self.BP_Bucket`))
  (bind (_returnvalue_x _returnvalue_y _returnvalue_z) (`KismetMathLibrary.BreakVector` (`SceneComponent.K2_GetComponentLocation` (`self.Box`))))
  (bind _water (`/Game/Core/Blueprints/Items/BP_Bucket0.water` _bp_bucket))
  (if (`self.Kran`)
    (`/Engine/EditorBlueprintResources/StandardMacros.DoOnce` false :!label _label_5
      (:`Completed`
        (if (`self.BuscerValid`) :!label _label_6
          (bind _returnvalue (`|SpawnActorFromClass` "/Game/Core/Blueprints/FireWater/BP_Water.BP_Water_C" (`KismetMathLibrary.MakeTransform` (`KismetMathLibrary.MakeVector` _returnvalue_x _returnvalue_y (+ _returnvalue_z 10.0))) "Undefined" "OverrideRootScale" null null))
          (`GameplayStatics.PlaySound2D` "/Game/_Props/GameMenuInterface/Audio/Menu/soundcliquemenu.soundcliquemenu" 3.0 1.0 0.0 null null)
          (bind (_direction _newtrack_0) (`Timeline|Timeline_0` :!via `PlayFromStart` :!label _label_7)
            (:`Update`
              (if (<= _water 10.0)
                (set `/Game/Core/Blueprints/Items/BP_Bucket0.water` (+ _water _newtrack_0) _bp_bucket)
                (`/Game/Core/Blueprints/Items/BP_Bucket0.-UpdateWidget` _bp_bucket)
                (if (`self.Kran`)
                  (`KismetSystemLibrary.Delay` 1.0)
                  (goto _label_6)
                  (else
                    (goto _label_5)))
                (else
                  (set `/Game/Core/Blueprints/Items/BP_Bucket0.IsWater` true _bp_bucket)
                  (set `self.BuscerValid` false :!label _label_8)
                  (goto _label_7 :!via `Stop`))))
            (:`Finished`
              (if (>= _water 10.0)
                (set `/Game/Core/Blueprints/Items/BP_Bucket0.IsWater` true _bp_bucket))
              (`/Engine/EditorBlueprintResources/StandardMacros.IsValid` _returnvalue
                (:`Is Valid`
                  (`self.K2_DestroyActor` _returnvalue)
                  (goto _label_5 :!via `Reset`))
                (:`Is Not Valid`
                  (goto _label_5 :!via `Reset`)))))
          (else
            (`|ExecutionSequence`
              (:`then_0`
                (goto _label_8))
              (:`then_1`
                (goto _label_5 :!via `Reset`)))))))
    (else
      (`self.NoKran`))))

(event `self.Box.OnComponentBeginOverlap`
  (params (OverlappedComponent :type "PrimitiveComponent Object Reference") (OtherActor :type "Actor Object Reference") (OtherComp :type "PrimitiveComponent Object Reference") (OtherBodyIndex :type Integer) (bFromSweep :type Boolean) (SweepResult :type "HitResult Structure (by ref)"))
  (bind _bp_bucket (`self.BP_Bucket`)
    (:`then`
      _)
    (:`else`
      (`self.BarNeValid`)))
  (set `self.BuscerValid` (or (== (`GameplayStatics.GetObjectClass` OtherActor) (`GameplayStatics.GetObjectClass` _bp_bucket)) (== OtherActor "/Game/Core/Blueprints/Items/BP_Bucket0.BP_Bucket0"))))

(event `self.Box.OnComponentEndOverlap`
  (params (OverlappedComponent :type "PrimitiveComponent Object Reference") (OtherActor :type "Actor Object Reference") (OtherComp :type "PrimitiveComponent Object Reference") (OtherBodyIndex :type Integer))
  (set `self.BuscerValid` false))

(fn `- Check Bucket`
  (params (Target :type "/Game/Core/Blueprints/Items/BP_BaseItem Object Reference"))
  (returns (BucketTarget :type Boolean))
  (switch `/Game/Core/Blueprints/Enum/E_ItemsSpecification` (`/Game/Core/Blueprints/Items/BP_BaseItem.ItemsSpec` Target)
    (:`NewEnumerator4`
      (if (`/Game/Core/Blueprints/Items/BP_Bucket0.IsWater` (`self.BP_Bucket`))
        (return true)
        (else
          (return false))))))

(fn `-UseItem`
  (bind _inventory_component (`/Game/Main/Character.Inventory_Component` (`self.Char`)))
  (`self.BP_Bucket`
    (:`then`
      (if (`self.BuscerValid`) :!label _label
        _
        (else
          (return))))
    (:`else`
      (bind _asbp_bucket_0 (cast `/Game/Core/Blueprints/Items/BP_Bucket0` (`self.GetOwner`))
        (:`then`
          (set `self.BP_Bucket` _asbp_bucket_0)
          (goto _label))
        (:`CastFailed`
          (return)))))
  (`/Game/Core/Components/Inventory_Component.ItemAdded` _inventory_component (`KismetArrayLibrary.Array_Find` (`/Game/Core/Components/Inventory_Component.Items` _inventory_component) (`self.BP_Bucket`)))
  (if (`self.BuscerValid`)
    (`self.BarNeValid`)
    (`self.MaterWaterKran`))
  (return))

(fn `Interact`
  (returns (Valid :type Boolean))
  (`|ExecutionSequence`
    (:`then_0`
      (if (`self.BuscerValid`)
        (`self.BP_Bucket`
          (:`then`
            (`self.MaterWaterKran`))
          (:`else`
            (bind _buckettarget (`self.- Check Bucket` null :!label _label))
            (if (not _buckettarget)
              (set `self.BuscerValid` true)
              (`self.BarNeValid`)
              (`self.MaterWaterKran`))))
        (elif (== (`GameplayStatics.GetObjectClass` null) (`GameplayStatics.GetObjectClass` (`self.BP_Bucket`)))
          (goto _label))))
    (:`then_1`
      (return true))))

(fn `UserConstructionScript`)