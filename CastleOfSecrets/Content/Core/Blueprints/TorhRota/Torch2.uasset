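; Interactable torch that acts as a lever once lit, triggering movement on a linked MoveLocationDown object.
; Fire runs once to show the flame and enable interaction, while InfoInteraction toggles custom depth on the mesh for highlighting.
; Interacting plays a rotation timeline, calls MoveUp on the linked object, then starts a second rotation timeline after a short delay.
; An IsMove flag blocks retriggering until that second timeline has started.
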(event `/Game/Core/Blueprints/Interface/BP_Info.InfoInteraction`
  (params (Char :type "/Game/Main/Character Object Reference") (On :type Boolean) (HitComponent :type "PrimitiveComponent Object Reference"))
  ;[1 1 1] Render
  (`PrimitiveComponent.SetRenderCustomDepth` (`self.SM_Torch`) On))

(event `Interact_1_1`
  (bind (_rotatepositionlast_roll _rotatepositionlast_pitch _rotatepositionlast_yaw) (`KismetMathLibrary.BreakRotator` (`self.RotatePositionLast`)))
  ;[1 1 1] Rotate/MoveChain
  (if (`self.IsFire`)
    (if (not (`self.IsMove`))
      (set `self.IsMove` true)
      (bind (_direction _rotater) (`Timeline|Rotate` :!via `PlayFromStart`)
        (:`Update`
          (`SceneComponent.K2_AddWorldRotation` (`self.SM_Torch`) (`KismetMathLibrary.MakeRotator` _rotatepositionlast_roll _rotater _rotatepositionlast_yaw) false false)
          (set `self.RotatePositionLast` (`KismetMathLibrary.MakeRotator` _rotatepositionlast_roll _rotater _rotatepositionlast_yaw)))
        (:`Finished`
          (`/Game/Core/Blueprints/TorhRota/BP_Chain.MoveUp` (`self.MoveLocationDown`))
          (`KismetSystemLibrary.Delay` 0.2)
          (`self.ReverseTourch`)
          (set `self.IsMove` false))))))

(event `Fire`
  ;[1 1 1] Fire torch
  (`/Engine/EditorBlueprintResources/StandardMacros.DoOnce` false
    (:`Completed`
      (`SceneComponent.SetVisibility` (`self.Torchfire_BP`) true false)
      (set `self.IsFire` true))))

(event `ReverseTourch`
  (bind (_rotatepositionlast_roll _rotatepositionlast_pitch _rotatepositionlast_yaw) (`KismetMathLibrary.BreakRotator` (`self.RotatePositionLast`)))
  (bind (_direction _rotater) (`Timeline|Timeline_0` :!via `PlayFromStart`)
    (:`Update`
      (`SceneComponent.K2_AddWorldRotation` (`self.SM_Torch`) (`KismetMathLibrary.MakeRotator` _rotatepositionlast_roll _rotater _rotatepositionlast_yaw) false false))))

(fn `Interact`
  (returns (Valid :type Boolean))
  (return false))

(fn `UserConstructionScript`)