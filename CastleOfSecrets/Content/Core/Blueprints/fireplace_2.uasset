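; Fireplace actor that switches to a visible, burning state when its CraftingEvent is called.
; The event reveals the flipbook, fireplace mesh, campfire component and two point lights, then starts the small fire sound.
; It also sets the Used flag and adds an audio component at runtime.
; BeginPlay, overlap, Tick and the construction script contain no logic.
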(event `self.Crafting Event`
  (params (Condition :type Boolean) (Bp_baseitem :type "/Game/Core/Blueprints/Items/BP_BaseItem Object Reference"))
  (`SceneComponent.SetVisibility` (`self.ricar_Flipbook`) true false)
  (`SceneComponent.SetVisibility` (`self.SM_Fireplace_Cole`) true false)
  (`SceneComponent.SetVisibility` (`self.P_Campfire`) true false)
  (`SceneComponent.SetVisibility` (`self.PointLight1`) true false)
  (`SceneComponent.SetVisibility` (`self.PointLight`) true false)
  (`AudioComponent.Play` (`self.Fire_Small03_Cue`) 0.0)
  (set `self.Used?` true)
  (`AddComponent|NODE_AddAudioComponent-0`))

(fn `UserConstructionScript`)