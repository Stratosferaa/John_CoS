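; BP_Door is a door that highlights on interaction, can be unlocked with a matching key and swings open.
; InfoInteraction toggles the mesh's custom depth rendering.
; CheckKey clears the locked flag and returns true when a Key item's name matches the door's.
; CraftingEvent plays a timeline once to rotate the mesh a quarter turn, without testing the lock itself.
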(event `/Game/Core/Blueprints/Interface/BP_Info.InfoInteraction`
  (params (Char :type "/Game/Main/Character Object Reference") (On :type Boolean) (HitComponent :type "PrimitiveComponent Object Reference"))
  (`PrimitiveComponent.SetRenderCustomDepth` (`self.DoorMesh`) On))

(event `self.Crafting Event`
  (params (Condition :type Boolean) (Bp_baseitem :type "/Game/Core/Blueprints/Items/BP_BaseItem Object Reference"))
  (`/Engine/EditorBlueprintResources/StandardMacros.DoOnce` false
    (:`Completed`
      (bind (_direction _alpha) (`Timeline|MoveDoor` :!via `PlayFromStart`)
        (:`Update`
          (`SceneComponent.K2_SetRelativeRotation` (`self.DoorMesh`) (`KismetMathLibrary.RLerp` (struct) (struct :`Yaw` -90.0) _alpha) false false))))))

(fn `CheckKey`
  (params (Item :type "/Game/Core/Blueprints/Items/BP_BaseItem Object Reference"))
  (returns (Opened :type Boolean))
  (switch `/Game/Core/Blueprints/Enum/E_ItemsSpecification` (`/Game/Core/Blueprints/Items/BP_BaseItem.ItemsSpec` Item)
    (:`NewEnumerator1`
      (if (== (`/Game/Core/Blueprints/Items/BP_BaseItem.NameKey` Item) (`self.NameForKey`))
        (set `self.DoorIsLocked` false)
        (return true)
        (else
          (return false))))))

(fn `UserConstructionScript`)