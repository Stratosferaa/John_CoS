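; Double-door Blueprint gated by a burnable mesh and a child Metla (broom) actor.
; FireSpyd attaches fire to StaticMesh2, then destroys it after a delay and sets IsFireSpider, letting MetlaMove slide the broom by timeline before enabling its gravity.
; CheckKey unlocks on a matching key name, and InfoInteraction toggles custom-depth highlighting.
; The gated door-swing timeline and spider animation are disconnected, and Interact only returns false.
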(event `self.ReceiveBeginPlay`
  (bind _asmetla (cast `/Game/Core/Blueprints/Items/Metla` (`ChildActorComponent.ChildActor` (`self.ChildActor`))))
  (set `self.As Metla` _asmetla)
  (set `/Game/Core/Blueprints/Items/Metla.BP_door` self _asmetla))

(event `/Game/Core/Blueprints/Interface/BP_Info.InfoInteraction`
  (params (Char :type "/Game/Main/Character Object Reference") (On :type Boolean) (HitComponent :type "PrimitiveComponent Object Reference"))
  (bind _staticmesh (`self.StaticMesh`))
  (`PrimitiveComponent.SetRenderCustomDepth` _staticmesh On)
  (`PrimitiveComponent.SetRenderCustomDepth` (`self.StaticMesh1`) On)
  (`PrimitiveComponent.SetRenderCustomDepth` _staticmesh On))

(event `MetlaMove`
  (bind _as_metla (`self.As Metla`))
  (if (`self.IsFireSpider`)
    (bind (_direction _move) (`Timeline|Timeline_0`)
      (:`Update`
        (`SceneComponent.K2_AddLocalOffset` (`Actor.RootComponent` _as_metla) (`KismetMathLibrary.MakeVector` 0.0 0.0 _move) false false))
      (:`Finished`
        (`PrimitiveComponent.SetCollisionEnabled` (`/Game/Core/Blueprints/Items/BP_BaseItem.MeshItem` _as_metla) "QueryAndPhysics")
        (`PrimitiveComponent.SetEnableGravity` (`/Game/Core/Blueprints/Items/BP_BaseItem.MeshItem` _as_metla) true)
        (set `self.IsMoveMetla` true)))))

(event `FireSpyd`
  (bind _staticmesh2 (`self.StaticMesh2`))
  (`/Engine/EditorBlueprintResources/StandardMacros.DoOnce` false
    (:`Completed`
      (bind _returnvalue (`GameplayStatics.SpawnEmitterAttached` "/Game/_Props/FirePack/Particles/P_Fire.P_Fire" _staticmesh2))
      (bind (_returnvalue_x _returnvalue_y _returnvalue_z) (`KismetMathLibrary.BreakVector` (`SceneComponent.K2_GetComponentScale` _returnvalue)))
      (`SceneComponent.SetWorldScale3D` _returnvalue (`KismetMathLibrary.MakeVector` (- _returnvalue_x 0.5) (- _returnvalue_y 0.5) (- _returnvalue_z 0.5)))
      (`KismetSystemLibrary.Delay` 5.0)
      (`ActorComponent.K2_DestroyComponent` _staticmesh2)
      (`SceneComponent.SetVisibility` _returnvalue false false)
      (set `self.IsFireSpider` true))))

(fn `CheckKey`
  (params (Item :type "/Game/Core/Blueprints/Items/BP_BaseItem Object Reference"))
  (returns (Opened :type Boolean))
  (switch `/Game/Core/Blueprints/Enum/E_ItemsSpecification` (`/Game/Core/Blueprints/Items/BP_BaseItem.ItemsSpec` Item)
    (:`NewEnumerator1`
      (if (== (`/Game/Core/Blueprints/Items/BP_BaseItem.NameKey` Item) (`self.NameForKey`))
        (set `self.DoorIsLocked` false)
        (return true)
        (else
          (return false))))))

(fn `Dosslove`
  (params (ParameterValue :type "Float (double-precision)") (InputPin :type "MeshComponent Object Reference"))
  (`MeshComponent.SetScalarParameterValueOnMaterials` InputPin "Dissolve" ParameterValue))

(fn `Interact`
  (returns (Valid :type Boolean))
  (return false))

(fn `UserConstructionScript`)