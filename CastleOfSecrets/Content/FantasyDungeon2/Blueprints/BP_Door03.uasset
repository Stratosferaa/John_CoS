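; BP_Door03 is a dungeon door of seven pieces that sink to open, either automatically or on pressing E.
; With AutoDoor set, overlapping the collision lowers the pieces and leaving raises them.
; Otherwise overlap shows a prompt widget and opens a gate for E, which lowers the door without re-closing it.
; Tick steps each piece's Z at its own speed, with the slowest piece's branch applying all positions and ending the motion.
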(event `Key|E`
  (params (Key :type "Key Structure"))
  ;[1 1 1] Press key E
  (:`Pressed`
    (`/Engine/EditorBlueprintResources/StandardMacros.Gate` true :!label _label
      (:`Exit`
        (set `self.Opened` true)
        (`WidgetLayoutLibrary.RemoveAllWidgets`)
        (set `self.Door Open` true)))))

(event `self.Collision.OnComponentEndOverlap`
  (params (OverlappedComponent :type "PrimitiveComponent Object Reference") (OtherActor :type "Actor Object Reference") (OtherComp :type "PrimitiveComponent Object Reference") (OtherBodyIndex :type Integer))
  ;[1 1 1] Overlap collision
  (set `self.Auto Close` true)
  (set `self.Auto Open` false)
  (`WidgetLayoutLibrary.RemoveAllWidgets`))

(event `self.Collision.OnComponentBeginOverlap`
  (params (OverlappedComponent :type "PrimitiveComponent Object Reference") (OtherActor :type "Actor Object Reference") (OtherComp :type "PrimitiveComponent Object Reference") (OtherBodyIndex :type Integer) (bFromSweep :type Boolean) (SweepResult :type "HitResult Structure (by ref)"))
  ;[1 1 1] Overlap collision
  (set `self.Auto Close` false)
  (set `self.Auto Open` true)
  ;[1 1 1] Press key E
  (if (`self.AutoDoor`)
    _
    (elif (not (`self.Door Open`))
      (bind _returnvalue (`|CreateWidget` "/Game/FantasyDungeon2/Blueprints/BP_PressE_Widget.BP_PressE_Widget_C"))
      (`UserWidget.AddToViewport` _returnvalue 0)
      (`self.EnableInput` (`GameplayStatics.GetPlayerController` 0))
      (goto _label :!via `Open`))))

(event `self.ReceiveTick`
  (params (DeltaSeconds :type "Float (single-precision)"))
  (bind _doorposition5 (`self.DoorPosition5`))
  (bind _doorposition2 (`self.DoorPosition2`))
  (bind _doorposition3 (`self.DoorPosition3`))
  (bind _doorposition6 (`self.DoorPosition6`))
  (bind _doorposition1 (`self.DoorPosition1`))
  (bind _doorposition2_2 (`self.DoorPosition2`))
  (bind _doorposition3_2 (`self.DoorPosition3`))
  (bind _doorposition4 (`self.DoorPosition4`))
  (bind _doorposition1_2 (`self.DoorPosition1`))
  (bind _doorposition5_2 (`self.DoorPosition5`))
  (bind _doorposition6_2 (`self.DoorPosition6`))
  (bind _doorposition7 (`self.DoorPosition7`))
  (bind _doorposition7_2 (`self.DoorPosition7`))
  (bind _doorposition4_2 (`self.DoorPosition4`))
  (if (`self.AutoDoor`)
    ;[1 1 1] Door open
    (if (`self.Auto Open`)
      ;;[1 1 1] Move
      (`/Engine/EditorBlueprintResources/StandardMacros.CompareFloat` _doorposition1 -383.0 :!label _label_2
        (:`>`
          (set `self.DoorPosition1` (- _doorposition1 2.0) :!label _label_3))
        (:`==`
          (goto _label_3))
        (:`<`
          (set `self.DoorPosition1` -383.5)))
      (`/Engine/EditorBlueprintResources/StandardMacros.CompareFloat` _doorposition2_2 -383.0
        (:`>`
          (set `self.DoorPosition2` (- _doorposition2_2 1.5) :!label _label_4))
        (:`==`
          (goto _label_4))
        (:`<`
          (set `self.DoorPosition2` -383.5)))
      (`/Engine/EditorBlueprintResources/StandardMacros.CompareFloat` _doorposition3_2 -383.0
        (:`>`
          (set `self.DoorPosition3` (- _doorposition3_2 1.8) :!label _label_5))
        (:`==`
          (goto _label_5))
        (:`<`
          (set `self.DoorPosition3` -383.5)))
      (`/Engine/EditorBlueprintResources/StandardMacros.CompareFloat` _doorposition4 -383.0
        (:`>`
          (set `self.DoorPosition4` (- _doorposition4 1.9) :!label _label_6))
        (:`==`
          (goto _label_6))
        (:`<`
          (set `self.DoorPosition4` -383.5)))
      (`/Engine/EditorBlueprintResources/StandardMacros.CompareFloat` _doorposition5_2 -383.0
        (:`>`
          (set `self.DoorPosition5` (- _doorposition5_2 1.7) :!label _label_7))
        (:`==`
          (goto _label_7))
        (:`<`
          (set `self.DoorPosition5` -383.5)))
      (`/Engine/EditorBlueprintResources/StandardMacros.CompareFloat` _doorposition6_2 -383.0
        (:`>`
          (set `self.DoorPosition6` (- _doorposition6_2 2.1) :!label _label_8))
        (:`==`
          (goto _label_8))
        (:`<`
          (set `self.DoorPosition6` -383.5)))
      (`/Engine/EditorBlueprintResources/StandardMacros.CompareFloat` _doorposition7 -383.0
        (:`>`
          (set `self.DoorPosition7` (- _doorposition7 1.4) :!label _label_9)
          (`SceneComponent.K2_SetRelativeLocation` (`self.Door03_1`) (`KismetMathLibrary.MakeVector` 0.0 0.0 (`self.DoorPosition1`)) false false :!label _label_10)
          (`SceneComponent.K2_SetRelativeLocation` (`self.Door03_2`) (`KismetMathLibrary.MakeVector` 0.0 0.0 (`self.DoorPosition2`)) false false)
          (`SceneComponent.K2_SetRelativeLocation` (`self.Door03_3`) (`KismetMathLibrary.MakeVector` 0.0 0.0 (`self.DoorPosition3`)) false false)
          (`SceneComponent.K2_SetRelativeLocation` (`self.Door03_4`) (`KismetMathLibrary.MakeVector` 0.0 0.0 (`self.DoorPosition4`)) false false)
          (`SceneComponent.K2_SetRelativeLocation` (`self.Door03_5`) (`KismetMathLibrary.MakeVector` 0.0 0.0 (`self.DoorPosition5`)) false false)
          (`SceneComponent.K2_SetRelativeLocation` (`self.Door03_6`) (`KismetMathLibrary.MakeVector` 0.0 0.0 (`self.DoorPosition6`)) false false)
          (`SceneComponent.K2_SetRelativeLocation` (`self.Door03_7`) (`KismetMathLibrary.MakeVector` 0.0 0.0 (`self.DoorPosition7`)) false false))
        (:`==`
          (goto _label_9))
        (:`<`
          (set `self.DoorPosition7` -383.5)
          (set `self.Auto Open` false)
          (set `self.Opened` false)))
      (else
        ;[1 1 1] Door close
        (if (`self.Auto Close`)
          ;;[1 1 1] Move
          (`/Engine/EditorBlueprintResources/StandardMacros.CompareFloat` _doorposition1_2
            (:`>`
              (set `self.DoorPosition1` 0.2))
            (:`==`
              (set `self.DoorPosition1` (+ _doorposition1_2 2.0) :!label _label_11))
            (:`<`
              (goto _label_11)))
          (`/Engine/EditorBlueprintResources/StandardMacros.CompareFloat` _doorposition2
            (:`>`
              (set `self.DoorPosition2` 0.2))
            (:`==`
              (set `self.DoorPosition2` (+ _doorposition2 1.5) :!label _label_12))
            (:`<`
              (goto _label_12)))
          (`/Engine/EditorBlueprintResources/StandardMacros.CompareFloat` _doorposition3
            (:`>`
              (set `self.DoorPosition3` 0.2))
            (:`==`
              (set `self.DoorPosition3` (+ _doorposition3 1.8) :!label _label_13))
            (:`<`
              (goto _label_13)))
          (`/Engine/EditorBlueprintResources/StandardMacros.CompareFloat` _doorposition4_2
            (:`>`
              (set `self.DoorPosition4` 0.2))
            (:`==`
              (set `self.DoorPosition4` (+ _doorposition4_2 1.9) :!label _label_14))
            (:`<`
              (goto _label_14)))
          (`/Engine/EditorBlueprintResources/StandardMacros.CompareFloat` _doorposition5
            (:`>`
              (set `self.DoorPosition5` 0.2))
            (:`==`
              (set `self.DoorPosition5` (+ _doorposition5 1.7) :!label _label_15))
            (:`<`
              (goto _label_15)))
          (`/Engine/EditorBlueprintResources/StandardMacros.CompareFloat` _doorposition6
            (:`>`
              (set `self.DoorPosition6` 0.2))
            (:`==`
              (set `self.DoorPosition6` (+ _doorposition6 2.1) :!label _label_16))
            (:`<`
              (goto _label_16)))
          (`/Engine/EditorBlueprintResources/StandardMacros.CompareFloat` _doorposition7_2
            (:`>`
              (set `self.DoorPosition7` 0.2)
              (set `self.Auto Close` false))
            (:`==`
              (set `self.DoorPosition7` (+ _doorposition7_2 1.4) :!label _label_17)
              (goto _label_10))
            (:`<`
              (goto _label_17))))))
    (elif (`self.Opened`)
      (goto _label_2))))

(fn `UserConstructionScript`)