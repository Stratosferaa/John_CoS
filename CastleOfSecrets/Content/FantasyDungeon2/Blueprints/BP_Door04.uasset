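; BP_Door04 is a dungeon door that the player opens by pressing E, with a selectable entrance mesh set in the construction script.
; Overlapping the collision while the door is unopened shows a prompt widget, enables input and opens a gate for the key.
; Once triggered, Tick first slides Door042 along local Y, then yaws Door to 90 degrees in fixed per-frame steps.
; No closing logic exists.
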(event `Key|E`
  (params (Key :type "Key Structure"))
  ;[1 1 1] Press key E
  (:`Pressed`
    (`/Engine/EditorBlueprintResources/StandardMacros.Gate` true :!label _label
      (:`Exit`
        (set `self.Opened` true)
        (`WidgetLayoutLibrary.RemoveAllWidgets`)
        (set `self.Door Open` true)))))

(event `self.Collision.OnComponentEndOverlap`
  (params (OverlappedComponent :type "PrimitiveComponent Object Reference") (OtherActor :type "Actor Object Reference") (OtherComp :type "PrimitiveComponent Object Reference") (OtherBodyIndex :type Integer))
  ;[1 1 1] Overlap collision
  (`WidgetLayoutLibrary.RemoveAllWidgets`))

(event `self.Collision.OnComponentBeginOverlap`
  (params (OverlappedComponent :type "PrimitiveComponent Object Reference") (OtherActor :type "Actor Object Reference") (OtherComp :type "PrimitiveComponent Object Reference") (OtherBodyIndex :type Integer) (bFromSweep :type Boolean) (SweepResult :type "HitResult Structure (by ref)"))
  ;[1 1 1] Overlap collision
  ;[1 1 1] Press key E
  (if (not (`self.Door Open`))
    (bind _returnvalue (`|CreateWidget` "/Game/FantasyDungeon2/Blueprints/BP_PressE_Widget.BP_PressE_Widget_C"))
    (`UserWidget.AddToViewport` _returnvalue 0)
    (`self.EnableInput` (`GameplayStatics.GetPlayerController` 0))
    (goto _label :!via `Open`)))

(event `self.ReceiveTick`
  (params (DeltaSeconds :type "Float (single-precision)"))
  (bind _doorrotation (`self.DoorRotation`))
  (bind _doorposition (`self.DoorPosition`))
  ;[1 1 1] Door open
  (if (`self.Opened`)
    (`/Engine/EditorBlueprintResources/StandardMacros.CompareFloat` _doorposition -15.0
      (:`>`
        (set `self.DoorPosition` (- _doorposition 1.0))
        (`SceneComponent.K2_SetRelativeLocation` (`self.Door04_2`) (`KismetMathLibrary.MakeVector` 0.0 (`self.DoorPosition`)) false false))
      (:`==`
        (set `self.DoorPosition` -15.0 :!label _label_2)
        ;;[1 1 1] Rotation
        (`/Engine/EditorBlueprintResources/StandardMacros.CompareFloat` _doorrotation 90.0
          (:`>`
            (set `self.DoorRotation` 90.0 :!label _label_3)
            (set `self.Opened` false))
          (:`==`
            (goto _label_3))
          (:`<`
            (set `self.DoorRotation` (+ _doorrotation 1.0))
            (`SceneComponent.K2_SetRelativeRotation` (`self.Door`) (`KismetMathLibrary.MakeRotator` 0.0 0.0 (`self.DoorRotation`)) false false))))
      (:`<`
        (goto _label_2)))))

(fn `UserConstructionScript`
  (bind _entrance (`self.Entrance`))
  (switch `int` (`self.EntranceVar`)
    (:`Default`
      (`StaticMeshComponent.SetStaticMesh` _entrance "/Game/FantasyDungeon2/Meshes/Door/SM_Entrance01.SM_Entrance01" :!label _label))
    (:`0`
      (goto _label))
    (:`1`
      (`StaticMeshComponent.SetStaticMesh` _entrance "/Game/FantasyDungeon2/Meshes/Door/SM_Entrance02.SM_Entrance02"))))