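; Breakable clay pot prop that shatters when hit, with fifteen mesh variants selected or randomized once in the construction script.
; Until broken, Tick compares player distance to a view threshold, showing the static mesh when far and the destructible mesh when near as a cheap LOD swap.
; A hit on the destructible applies radius damage at the impact point, switches its collision object type to avoid the player, and marks it broken after a short delay.
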(event `self.ReceiveTick`
  (params (DeltaSeconds :type "Float (single-precision)"))
  (bind _destructible_mesh (`self.Destructible Mesh`))
  (bind _static_mesh (`self.Static Mesh`))
  ;[1 1 1] If object not break
  (if (not (`self.Break`))
    ;[1 1 1] get information how close the player is to the object
    (`/Engine/EditorBlueprintResources/StandardMacros.CompareFloat` (`KismetMathLibrary.Vector_Distance` (`SceneComponent.K2_GetComponentLocation` (`Actor.RootComponent` (`GameplayStatics.GetPlayerCharacter` 0))) (`SceneComponent.K2_GetComponentLocation` (`self.DefaultSceneRoot`))) (`self.Destructable Mesh View Distance`)
      (:`>`
        ;[1 1 1] if the player is close enough, switch the object from static mesh to destructible mesh. if the object is break, then the mesh does not switch
        (`SceneComponent.SetVisibility` _static_mesh true false)
        (`SceneComponent.SetVisibility` _destructible_mesh false false))
      (:`==`
        (`SceneComponent.SetVisibility` _static_mesh false false :!label _label)
        (`SceneComponent.SetVisibility` _destructible_mesh true false))
      (:`<`
        (goto _label)))))

(event `self.Destructible Mesh.OnComponentHit`
  (params (HitComponent :type "PrimitiveComponent Object Reference") (OtherActor :type "Actor Object Reference") (OtherComp :type "PrimitiveComponent Object Reference") (NormalImpulse :type "Vector Structure") (Hit :type "HitResult Structure (by ref)"))
  (bind _destructible_mesh (`self.Destructible Mesh`))
  ;[1 1 1] when object takes damage, it changes the collision channel in order not to interact with the player
  (if (`self.Break`)
    (goto _label)
    (else
      (`DestructibleComponent.ApplyRadiusDamage` _destructible_mesh 100.0 (`.ImpactPoint` (`GameplayStatics.BreakHitResult` Hit)) 10.0 0.0 false)
      (`PrimitiveComponent.SetCollisionObjectType` _destructible_mesh "ECC_Visibility")
      (`KismetSystemLibrary.Delay` 0.3)
      (set `self.impulse` 0.0)
      (set `self.Break` true))))

(fn `UserConstructionScript`
  (bind _destructible_mesh (`self.Destructible Mesh`))
  (bind _static_mesh (`self.Static Mesh`))
  ;[1 1 1] Comment
  (if (`self.RandomMesh`)
    (set `self.ClayPot Mesh` (`KismetMathLibrary.RandomIntegerInRange` 1 15))
    (set `self.RandomMesh` false))
  ;[1 1 1] Select ClayPotMesh
  (switch `int` (`self.ClayPot Mesh`)
    (:`Default`
      (`DestructibleComponent.SetDestructibleMesh` _destructible_mesh "/Game/FantasyDungeon2/Meshes/Props/ClayPot/DM_ClayPot_1.DM_ClayPot_1" :!label _label)
      (`StaticMeshComponent.SetStaticMesh` _static_mesh "/Game/FantasyDungeon2/Meshes/Props/ClayPot/SM_ClayPot_1.SM_ClayPot_1"))
    (:`0`
      (goto _label))
    (:`1`
      (goto _label))
    (:`2`
      (`DestructibleComponent.SetDestructibleMesh` _destructible_mesh "/Game/FantasyDungeon2/Meshes/Props/ClayPot/DM_ClayPot_2.DM_ClayPot_2")
      (`StaticMeshComponent.SetStaticMesh` _static_mesh "/Game/FantasyDungeon2/Meshes/Props/ClayPot/SM_ClayPot_2.SM_ClayPot_2"))
    (:`3`
      (`DestructibleComponent.SetDestructibleMesh` _destructible_mesh "/Game/FantasyDungeon2/Meshes/Props/ClayPot/DM_ClayPot_3.DM_ClayPot_3")
      (`StaticMeshComponent.SetStaticMesh` _static_mesh "/Game/FantasyDungeon2/Meshes/Props/ClayPot/SM_ClayPot_3.SM_ClayPot_3"))
    (:`4`
      (`DestructibleComponent.SetDestructibleMesh` _destructible_mesh "/Game/FantasyDungeon2/Meshes/Props/ClayPot/DM_ClayPot_4.DM_ClayPot_4")
      (`StaticMeshComponent.SetStaticMesh` _static_mesh "/Game/FantasyDungeon2/Meshes/Props/ClayPot/SM_ClayPot_4.SM_ClayPot_4"))
    (:`5`
      (`DestructibleComponent.SetDestructibleMesh` _destructible_mesh "/Game/FantasyDungeon2/Meshes/Props/ClayPot/DM_ClayPot_5.DM_ClayPot_5")
      (`StaticMeshComponent.SetStaticMesh` _static_mesh "/Game/FantasyDungeon2/Meshes/Props/ClayPot/SM_ClayPot_5.SM_ClayPot_5"))
    (:`6`
      (`DestructibleComponent.SetDestructibleMesh` _destructible_mesh "/Game/FantasyDungeon2/Meshes/Props/ClayPot/DM_ClayPot_6.DM_ClayPot_6")
      (`StaticMeshComponent.SetStaticMesh` _static_mesh "/Game/FantasyDungeon2/Meshes/Props/ClayPot/SM_ClayPot_6.SM_ClayPot_6"))
    (:`7`
      (`DestructibleComponent.SetDestructibleMesh` _destructible_mesh "/Game/FantasyDungeon2/Meshes/Props/ClayPot/DM_ClayPot_7.DM_ClayPot_7")
      (`StaticMeshComponent.SetStaticMesh` _static_mesh "/Game/FantasyDungeon2/Meshes/Props/ClayPot/SM_ClayPot_7.SM_ClayPot_7"))
    (:`8`
      (`DestructibleComponent.SetDestructibleMesh` _destructible_mesh "/Game/FantasyDungeon2/Meshes/Props/ClayPot/DM_ClayPot_8.DM_ClayPot_8")
      (`StaticMeshComponent.SetStaticMesh` _static_mesh "/Game/FantasyDungeon2/Meshes/Props/ClayPot/SM_ClayPot_8.SM_ClayPot_8"))
    (:`9`
      (`DestructibleComponent.SetDestructibleMesh` _destructible_mesh "/Game/FantasyDungeon2/Meshes/Props/ClayPot/DM_ClayPot_9.DM_ClayPot_9")
      (`StaticMeshComponent.SetStaticMesh` _static_mesh "/Game/FantasyDungeon2/Meshes/Props/ClayPot/SM_ClayPot_9.SM_ClayPot_9"))
    (:`10`
      (`DestructibleComponent.SetDestructibleMesh` _destructible_mesh "/Game/FantasyDungeon2/Meshes/Props/ClayPot/DM_ClayPot_10.DM_ClayPot_10")
      (`StaticMeshComponent.SetStaticMesh` _static_mesh "/Game/FantasyDungeon2/Meshes/Props/ClayPot/SM_ClayPot_10.SM_ClayPot_10"))
    (:`11`
      (`DestructibleComponent.SetDestructibleMesh` _destructible_mesh "/Game/FantasyDungeon2/Meshes/Props/ClayPot/DM_ClayPot_11.DM_ClayPot_11")
      (`StaticMeshComponent.SetStaticMesh` _static_mesh "/Game/FantasyDungeon2/Meshes/Props/ClayPot/SM_ClayPot_11.SM_ClayPot_11"))
    (:`12`
      (`DestructibleComponent.SetDestructibleMesh` _destructible_mesh "/Game/FantasyDungeon2/Meshes/Props/ClayPot/DM_ClayPot_12.DM_ClayPot_12")
      (`StaticMeshComponent.SetStaticMesh` _static_mesh "/Game/FantasyDungeon2/Meshes/Props/ClayPot/SM_ClayPot_12.SM_ClayPot_12"))
    (:`13`
      (`DestructibleComponent.SetDestructibleMesh` _destructible_mesh "/Game/FantasyDungeon2/Meshes/Props/ClayPot/DM_ClayPot_13.DM_ClayPot_13")
      (`StaticMeshComponent.SetStaticMesh` _static_mesh "/Game/FantasyDungeon2/Meshes/Props/ClayPot/SM_ClayPot_13.SM_ClayPot_13"))
    (:`14`
      (`DestructibleComponent.SetDestructibleMesh` _destructible_mesh "/Game/FantasyDungeon2/Meshes/Props/ClayPot/DM_ClayPot_14.DM_ClayPot_14")
      (`StaticMeshComponent.SetStaticMesh` _static_mesh "/Game/FantasyDungeon2/Meshes/Props/ClayPot/SM_ClayPot_14.SM_ClayPot_14"))
    (:`15`
      (`DestructibleComponent.SetDestructibleMesh` _destructible_mesh "/Game/FantasyDungeon2/Meshes/Props/ClayPot/DM_ClayPot_15.DM_ClayPot_15")
      (`StaticMeshComponent.SetStaticMesh` _static_mesh "/Game/FantasyDungeon2/Meshes/Props/ClayPot/SM_ClayPot_15.SM_ClayPot_15")))
  (`PrimitiveComponent.SetCollisionObjectType` _destructible_mesh "ECC_Destructible"))