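; BP_StaticChain is a static chain prop that lays repeated mesh instances along a spline.
; The construction script adds a Hierarchical Instanced Static Mesh component and fills it with instances placed at even distances along the spline's length.
; Each instance takes the spline's local position and rotation, with ChainSize setting its scale and also multiplying Spacing to set the step between instances.
; The event graph holds no active logic.
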(fn `UserConstructionScript`
  (bind _chain_size (`self.Chain Size`))
  (bind _spline (`self.Spline`))
  (bind _returnvalue (* (`self.Spacing`) _chain_size))
  (bind _returnvalue_2 (`AddComponent|NODE_AddHierarchicalInstancedStaticMeshComponent-0`))
  (for _index (range (+ (`.ReturnValue` (`KismetMathLibrary.FMod` (`SplineComponent.GetSplineLength` _spline) _returnvalue)) 1))
    (bind _returnvalue_3 (* _index _returnvalue))
    (`InstancedStaticMeshComponent.AddInstance` _returnvalue_2 (`KismetMathLibrary.MakeTransform` (`SplineComponent.GetLocationAtDistanceAlongSpline` _spline _returnvalue_3 "Local") (`SplineComponent.GetRotationAtDistanceAlongSpline` _spline _returnvalue_3 "Local") (`KismetMathLibrary.Conv_DoubleToVector` _chain_size)))))