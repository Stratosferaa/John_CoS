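; Rain effect actor that spawns a rain particle at its location on BeginPlay and scatters splash particles on surfaces it finds.
; Each tick, a small multi box trace runs from randomly offset X/Y points within MaxRange of the actor, offset by TraceDistance, on the Visibility channel.
; Each hit spawns a splash emitter, with a short Delay inside the hit loop before a DestroyComponent call.
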(event `self.ReceiveBeginPlay`
  (`GameplayStatics.SpawnEmitterAtLocation` "/Game/_Props/Rain_Assets/Particles/Rain_Particle.Rain_Particle" (`self.K2_GetActorLocation`)))

(event `self.ReceiveTick`
  (params (DeltaSeconds :type "Float (single-precision)"))
  (bind _maxrange (`self.MaxRange`))
  (bind _returnvalue (`KismetMathLibrary.MakeVector` (+ (`KismetMathLibrary.Conv_IntToDouble` (`KismetMathLibrary.RandomIntegerInRange` 0 _maxrange)) (.x (`self.K2_GetActorLocation`))) (+ (`KismetMathLibrary.Conv_IntToDouble` (`KismetMathLibrary.RandomIntegerInRange` 0 _maxrange)) (.y (`self.K2_GetActorLocation`))) (.z (`self.K2_GetActorLocation`))))
  (bind _outhits (`KismetSystemLibrary.BoxTraceMulti` :`Start` _returnvalue :`End` (- _returnvalue (`self.Trace_Distance`)) :`HalfSize` (2.0 2.0 2.0) :`TraceChannel` "TraceTypeQuery1" :`bTraceComplex` true :`DrawTime` 0.1))
  (for _array_element _outhits
    (bind _returnvalue_2 (`GameplayStatics.SpawnEmitterAtLocation` "/Game/_Props/Rain_Assets/Particles/Splashes_Particle.Splashes_Particle" (`.Location` (`GameplayStatics.BreakHitResult` _array_element))))
    (`KismetSystemLibrary.Delay` 0.1)
    (`ActorComponent.K2_DestroyComponent` _returnvalue_2)))

(fn `UserConstructionScript`)