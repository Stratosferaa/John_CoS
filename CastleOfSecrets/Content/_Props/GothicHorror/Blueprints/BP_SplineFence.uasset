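; Spline fence prop meant to lay poles, ribs and two connector rows along a spline.
; The construction script spaces points by connector length and stores transforms with seeded rotation disorder, then calls BuildFence.
; BuildFence's entry is unwired, so its instancing logic never runs.
; That logic would use hierarchical instanced meshes, stretching connectors between points, placing poles at intervals and randomly raising ribs.
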(fn `BuildFence`
  ;[1 1 1] Check and Init Poles
)

(fn `CalculatePolesAndRibsTransforms`
  (bind _spline (`self.Spline`))
  (bind _returnvalue (`KismetMathLibrary.MakeRandomStream` (`self.NextSeed`)))
  (set `self.NextSeed` (`self.Seed`))
  (`KismetArrayLibrary.Array_Clear` (`self.Ribs Locations`))
  (`KismetArrayLibrary.Array_Clear` (`self.Ribs Rotations`))
  (for _index (range (`self.Spline Ribs Count`))
    (bind _returnvalue_2 (* _index (`self.ConnectionLength`)))
    (bind _returnvalue_3 (`SplineComponent.GetLocationAtDistanceAlongSpline` _spline _returnvalue_2 "World"))
    ;[1 1 1] Poles and Ribs
    (`KismetArrayLibrary.Array_Add` (`self.Ribs Locations`) _returnvalue_3)
    (bind _returnvalue_4 (`KismetMathLibrary.ComposeRotators` (`SplineComponent.GetRotationAtDistanceAlongSpline` _spline _returnvalue_2 "World") (* (`KismetMathLibrary.MakeRotator` (`KismetMathLibrary.RandomFloatInRangeFromStream` -5.0 5.0 _returnvalue) (`KismetMathLibrary.RandomFloatInRangeFromStream` -5.0 5.0 _returnvalue) (`KismetMathLibrary.RandomFloatInRangeFromStream` -5.0 5.0 _returnvalue)) (`self.Disorder`))))
    (`KismetArrayLibrary.Array_Add` (`self.Ribs Rotations`) _returnvalue_4)
    (set `self.NextSeed` (+ (`self.NextSeed`) 1)))
  ;[1 1 1] Ending Pole
  (`KismetArrayLibrary.Array_Add` (`self.Ribs Locations`) _returnvalue_3)
  (`KismetArrayLibrary.Array_Add` (`self.Ribs Rotations`) _returnvalue_4))

(fn `UserConstructionScript`
  (set `self.ConnectionLength` (.x (`.Max` (break `Box` (`StaticMesh.GetBoundingBox` (`self.Connector Mesh`))))))
  (set `self.Spline Ribs Count` (`KismetMathLibrary.FFloor` (/ (`SplineComponent.GetSplineLength` (`self.Spline`)) (`self.ConnectionLength`))))
  (`self.CalculatePolesAndRibsTransforms`)
  (`self.BuildFence`))