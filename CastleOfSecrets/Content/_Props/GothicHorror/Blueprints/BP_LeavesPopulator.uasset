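; BP_LeavesPopulator is a prop Blueprint that scatters leaf instances over the surface of a base mesh.
; Its construction script reads vertices and normals from LOD 0, section 0, then randomly adds HISM instances at normal-offset vertices according to LeavesAmount.
; Leaves combine random rotation with the normal, optionally compensating for actor transform.
; A growth curve scales them by vertex height relative to the mesh bounds.
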(fn `UserConstructionScript`
  (bind _base_mesh (`self.Base Mesh`))
  (bind (_x _y) (`KismetMathLibrary.BreakVector2D` (`self.Leaves Yaw Random`)))
  (bind (_x_2 _y_2) (`KismetMathLibrary.BreakVector2D` (`self.Leaves Roll Random`)))
  (bind (_x_3 _y_3) (`KismetMathLibrary.BreakVector2D` (`self.Leaves Pitch Random`)))
  (bind _returnvalue (`KismetMathLibrary.MakeRotator` (`KismetMathLibrary.RandomFloatInRange` _x_2 _y_2) (`KismetMathLibrary.RandomFloatInRange` _x_3 _y_3) (`KismetMathLibrary.RandomFloatInRange` _x _y)))
  (if (`self.Refresh`)
    _
    (else
      _))
  (set `self.Refresh` false)
  ;[1 1 1] Set Base Mesh
  (`StaticMeshComponent.SetStaticMesh` (`self.Mesh`) _base_mesh)
  (bind (_vertices _triangles _normals) (`KismetProceduralMeshLibrary.GetSectionFromStaticMesh` _base_mesh))
  (bind _returnvalue_2 (`AddComponent|NODE_AddHierarchicalInstancedStaticMeshComponent-0`))
  (`StaticMeshComponent.SetStaticMesh` _returnvalue_2 (`self.Leaf Mesh`))
  (for _index (range (+ (`KismetArrayLibrary.Array_Length` _vertices) 1))
    ;[1 1 1] Leaves Amount
    (if (< (`KismetMathLibrary.RandomFloat`) (`self.Leaves Amount`))
      ;[1 1 1] World Space Leaves Orientation
      (if (`self.WS Leaves Orientation`)
        (bind _output (`|GetArrayItem` _vertices _index))
        (bind _output_2 (`|GetArrayItem` _normals _index))
        (bind _returnvalue_3 (+ _output (* _output_2 (`self.Leaves Offset`))))
        (bind _returnvalue_4 (`KismetMathLibrary.Conv_VectorToRotator` _output_2))
        (bind _returnvalue_5 (* (1.0 1.0 1.0) (`KismetMathLibrary.FClamp` (`CurveFloat.GetFloatValue` (`self.TD Growth Curve`) (/ (.z _output) (.z (`.Max` (break `Box` (`StaticMesh.GetBoundingBox` _base_mesh)))))))))
        (`InstancedStaticMeshComponent.AddInstance` _returnvalue_2 (`KismetMathLibrary.MakeTransform` _returnvalue_3 (`KismetMathLibrary.InverseTransformRotation` (`self.GetTransform`) (`KismetMathLibrary.ComposeRotators` _returnvalue _returnvalue_4)) _returnvalue_5))
        (else
          (`InstancedStaticMeshComponent.AddInstance` _returnvalue_2 (`KismetMathLibrary.MakeTransform` _returnvalue_3 (`KismetMathLibrary.ComposeRotators` _returnvalue _returnvalue_4) _returnvalue_5)))))))