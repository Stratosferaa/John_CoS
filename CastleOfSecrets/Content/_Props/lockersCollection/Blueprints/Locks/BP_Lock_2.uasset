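; BP_Lock_2 is a clickable keypad lock prop from the lockers collection, with twelve button meshes and a separate lock element.
; Each button click calls TouchEvent with the button, a shared delta and its digit as a string, with buttons 10 and 12 sending an empty string.
; Clicking the lock element calls HandleEvent; the logic behind both calls is defined outside this graph.
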(event `self.SM_Lock_2_button_1.OnClicked`
  (params (TouchedComponent :type "PrimitiveComponent Object Reference") (ButtonPressed :type "Key Structure"))
  (`self.Touch_Event` TouchedComponent 0.2 "1"))

(event `self.SM_Lock_2_button_2.OnClicked`
  (params (TouchedComponent :type "PrimitiveComponent Object Reference") (ButtonPressed :type "Key Structure"))
  (`self.Touch_Event` TouchedComponent 0.2 "2"))

(event `self.SM_Lock_2_button_3.OnClicked`
  (params (TouchedComponent :type "PrimitiveComponent Object Reference") (ButtonPressed :type "Key Structure"))
  (`self.Touch_Event` TouchedComponent 0.2 "3"))

(event `self.SM_Lock_2_button_4.OnClicked`
  (params (TouchedComponent :type "PrimitiveComponent Object Reference") (ButtonPressed :type "Key Structure"))
  (`self.Touch_Event` TouchedComponent 0.2 "4"))

(event `self.SM_Lock_2_button_5.OnClicked`
  (params (TouchedComponent :type "PrimitiveComponent Object Reference") (ButtonPressed :type "Key Structure"))
  (`self.Touch_Event` TouchedComponent 0.2 "5"))

(event `self.SM_Lock_2_button_6.OnClicked`
  (params (TouchedComponent :type "PrimitiveComponent Object Reference") (ButtonPressed :type "Key Structure"))
  (`self.Touch_Event` TouchedComponent 0.2 "6"))

(event `self.SM_Lock_2_button_7.OnClicked`
  (params (TouchedComponent :type "PrimitiveComponent Object Reference") (ButtonPressed :type "Key Structure"))
  (`self.Touch_Event` TouchedComponent 0.2 "7"))

(event `self.SM_Lock_2_button_8.OnClicked`
  (params (TouchedComponent :type "PrimitiveComponent Object Reference") (ButtonPressed :type "Key Structure"))
  (`self.Touch_Event` TouchedComponent 0.2 "8"))

(event `self.SM_Lock_2_button_9.OnClicked`
  (params (TouchedComponent :type "PrimitiveComponent Object Reference") (ButtonPressed :type "Key Structure"))
  (`self.Touch_Event` TouchedComponent 0.2 "9"))

(event `self.SM_Lock_2_button_10.OnClicked`
  (params (TouchedComponent :type "PrimitiveComponent Object Reference") (ButtonPressed :type "Key Structure"))
  (`self.Touch_Event` TouchedComponent))

(event `self.SM_Lock_2_button_11.OnClicked`
  (params (TouchedComponent :type "PrimitiveComponent Object Reference") (ButtonPressed :type "Key Structure"))
  (`self.Touch_Event` TouchedComponent 0.2 "0"))

(event `self.SM_Lock_2_button_12.OnClicked`
  (params (TouchedComponent :type "PrimitiveComponent Object Reference") (ButtonPressed :type "Key Structure"))
  (`self.Touch_Event` TouchedComponent))

(event `self.SM_Lock_2_element.OnClicked`
  (params (TouchedComponent :type "PrimitiveComponent Object Reference") (ButtonPressed :type "Key Structure"))
  (`self.Handle_Event` TouchedComponent))

(fn `UserConstructionScript`)