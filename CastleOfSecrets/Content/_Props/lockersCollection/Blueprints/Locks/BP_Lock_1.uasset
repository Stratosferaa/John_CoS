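; BP_Lock_1 is a rotary-dial lock prop, built on a parent lock Blueprint, whose number the player selects.
; Select_Number uses a timeline to rotate the dial mesh along the shortest path to the chosen number.
; In SimpleEnter mode, clickable left/right boxes step a wrapping number; otherwise the player widget supplies it and it is added when rotation finishes.
; While this lock is selected, Tick toggles box collision and widget controls through DoOnce gates.
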(event `self.ReceiveBeginPlay`
  (bind _look_position (`self.Look_Position`))
  (`parent.ReceiveBeginPlay`)
  (set `self.Custom_Lock` true)
  (`SceneComponent.K2_SetWorldLocation` _look_position (`KismetMathLibrary.MakeVector` (.x (`SceneComponent.K2_GetComponentLocation` _look_position)) (.y (`SceneComponent.K2_GetComponentLocation` _look_position)) (+ (.z (`SceneComponent.K2_GetComponentLocation` _look_position)) 0.15)) false false))

(event `Select_Number`
  (bind _w_maingame (`/Game/_Props/lockersCollection/DemoContent/FirstPersonBP/Blueprints/FirstPersonCharacter.W_MainGame` (`self.Player`)))
  (bind _w_maingame_2 (`/Game/_Props/lockersCollection/DemoContent/FirstPersonBP/Blueprints/FirstPersonCharacter.W_MainGame` (`self.Player`)))
  (set `self.Current_Rotation` (`SceneComponent.RelativeRotation` (`self.SM_Lock_1_element`)))
  (set `self.Selected_Rotation` (`KismetMathLibrary.MakeRotator` 0.0 (select `bool` (`Widget.GetIsEnabled` (`/Game/_Props/lockersCollection/Blueprints/UI/W_MainGame_Widget.Editable_Text_Box` _w_maingame_2)) :`false` (* (`KismetMathLibrary.Conv_IntToDouble` (`self.Current_Num`)) 40.0) :`true` (* (`/Game/_Props/lockersCollection/Blueprints/UI/W_MainGame_Widget.Current_Number` _w_maingame_2) 4.0))))
  (bind (_direction _newtrack_0) (`Timeline|Timeline_1` :!via `PlayFromStart`)
    (:`Update`
      (`SceneComponent.K2_SetRelativeRotation` (`self.SM_Lock_1_element`) (`KismetMathLibrary.RLerp` (`self.Current_Rotation`) (`self.Selected_Rotation`) _newtrack_0 true) false false))
    (:`Finished`
      (if (`Widget.GetIsEnabled` (`/Game/_Props/lockersCollection/Blueprints/UI/W_MainGame_Widget.Editable_Text_Box` _w_maingame))
        (`self.-AddNumber` (`KismetStringLibrary.Conv_IntToString` (`/Game/_Props/lockersCollection/Blueprints/UI/W_MainGame_Widget.Current_Number` _w_maingame)))))))

(event `self.Box_L.OnClicked`
  (params (TouchedComponent :type "PrimitiveComponent Object Reference") (ButtonPressed :type "Key Structure"))
  (if (`self.Simple_Enter`)
    (bind _output_get (set `self.Current_Num` (+ (`self.Current_Num`) 10)))
    (`self.Select_Number`)
    (if (>= _output_get 90)
      (set `self.Current_Num` 0))))

(event `self.Box_R.OnClicked`
  (params (TouchedComponent :type "PrimitiveComponent Object Reference") (ButtonPressed :type "Key Structure"))
  (bind _returnvalue (- (`self.Current_Num`) 10))
  (if (`self.Simple_Enter`)
    (if (<= _returnvalue -1)
      (set `self.Current_Num` 80)
      (else
        (bind _output_get (set `self.Current_Num` _returnvalue))))
    (`self.Select_Number`)
    (if (== _output_get 90)
      (set `self.Current_Num` 0))))

(event `self.ReceiveTick`
  (params (DeltaSeconds :type "Float (single-precision)"))
  (bind _w_maingame (`/Game/_Props/lockersCollection/DemoContent/FirstPersonBP/Blueprints/FirstPersonCharacter.W_MainGame` (`self.Player`)))
  (bind _selected_lock (`/Game/_Props/lockersCollection/DemoContent/FirstPersonBP/Blueprints/FirstPersonCharacter.Selected_Lock` (`self.Player`))
    (:`then`
      (if (== _selected_lock self)
        (if (`self.Simple_Enter`)
          (`/Engine/EditorBlueprintResources/StandardMacros.DoOnce` false
            (:`Completed`
              (`PrimitiveComponent.SetCollisionEnabled` (`self.Box_L`) "QueryOnly")
              (`PrimitiveComponent.SetCollisionEnabled` (`self.Box_R`) "QueryOnly")
              (`Widget.SetIsEnabled` (`/Game/_Props/lockersCollection/Blueprints/UI/W_MainGame_Widget.Editable_Text_Box` _w_maingame) false)
              (`Widget.SetIsEnabled` (`/Game/_Props/lockersCollection/Blueprints/UI/W_MainGame_Widget.Up_Down_Btns` _w_maingame) false)))
          (else
            (`/Engine/EditorBlueprintResources/StandardMacros.DoOnce` false
              (:`Completed`
                (`PrimitiveComponent.SetCollisionEnabled` (`self.Box_L`) "NoCollision")
                (`PrimitiveComponent.SetCollisionEnabled` (`self.Box_R`) "NoCollision")
                (`Widget.SetIsEnabled` (`/Game/_Props/lockersCollection/Blueprints/UI/W_MainGame_Widget.Up_Down_Btns` _w_maingame) true)
                (`Widget.SetIsEnabled` (`/Game/_Props/lockersCollection/Blueprints/UI/W_MainGame_Widget.Editable_Text_Box` _w_maingame) true)))))))
    (:`else`)))

(fn `UserConstructionScript`
  (`parent.UserConstructionScript`))