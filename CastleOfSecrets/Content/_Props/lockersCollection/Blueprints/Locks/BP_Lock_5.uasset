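; BP_Lock_5 is a clickable keypad lock, filed as a prop in the lockers collection.
; Click events on twelve button meshes call TouchEvent with the pressed component, a fixed delta and either a digit or an empty string.
; A thirteenth button calls HandleButtonEvent instead.
; BeginPlay runs the parent's logic, then enables and calls ViewportPassword; the handlers' logic lives outside this graph.
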(event `self.ReceiveBeginPlay`
  (`parent.ReceiveBeginPlay`)
  (set `self.ViewportPassword` true)
  (`self.-ViewportPassword`))

(event `self.SM_Lock_5_button_1.OnClicked`
  (params (TouchedComponent :type "PrimitiveComponent Object Reference") (ButtonPressed :type "Key Structure"))
  (`self.Touch_Event` TouchedComponent 0.1 "1"))

(event `self.SM_Lock_5_button_2.OnClicked`
  (params (TouchedComponent :type "PrimitiveComponent Object Reference") (ButtonPressed :type "Key Structure"))
  (`self.Touch_Event` TouchedComponent 0.1 "2"))

(event `self.SM_Lock_5_button_3.OnClicked`
  (params (TouchedComponent :type "PrimitiveComponent Object Reference") (ButtonPressed :type "Key Structure"))
  (`self.Touch_Event` TouchedComponent 0.1 "3"))

(event `self.SM_Lock_5_button_4.OnClicked`
  (params (TouchedComponent :type "PrimitiveComponent Object Reference") (ButtonPressed :type "Key Structure"))
  (`self.Touch_Event` TouchedComponent 0.1 "4"))

(event `self.SM_Lock_5_button_5.OnClicked`
  (params (TouchedComponent :type "PrimitiveComponent Object Reference") (ButtonPressed :type "Key Structure"))
  (`self.Touch_Event` TouchedComponent 0.1 "5"))

(event `self.SM_Lock_5_button_6.OnClicked`
  (params (TouchedComponent :type "PrimitiveComponent Object Reference") (ButtonPressed :type "Key Structure"))
  (`self.Touch_Event` TouchedComponent 0.1 "6"))

(event `self.SM_Lock_5_button_7.OnClicked`
  (params (TouchedComponent :type "PrimitiveComponent Object Reference") (ButtonPressed :type "Key Structure"))
  (`self.Touch_Event` TouchedComponent 0.1 "7"))

(event `self.SM_Lock_5_button_8.OnClicked`
  (params (TouchedComponent :type "PrimitiveComponent Object Reference") (ButtonPressed :type "Key Structure"))
  (`self.Touch_Event` TouchedComponent 0.1 "8"))

(event `self.SM_Lock_5_button_9.OnClicked`
  (params (TouchedComponent :type "PrimitiveComponent Object Reference") (ButtonPressed :type "Key Structure"))
  (`self.Touch_Event` TouchedComponent 0.1 "9"))

(event `self.SM_Lock_5_button_10.OnClicked`
  (params (TouchedComponent :type "PrimitiveComponent Object Reference") (ButtonPressed :type "Key Structure"))
  (`self.Touch_Event` TouchedComponent 0.1))

(event `self.SM_Lock_5_button_11.OnClicked`
  (params (TouchedComponent :type "PrimitiveComponent Object Reference") (ButtonPressed :type "Key Structure"))
  (`self.Touch_Event` TouchedComponent 0.1 "0"))

(event `self.SM_Lock_5_button_12.OnClicked`
  (params (TouchedComponent :type "PrimitiveComponent Object Reference") (ButtonPressed :type "Key Structure"))
  (`self.Touch_Event` TouchedComponent 0.1))

(event `self.SM_Lock_5_button_13.OnClicked`
  (params (TouchedComponent :type "PrimitiveComponent Object Reference") (ButtonPressed :type "Key Structure"))
  (`self.Handle_Button_Event` TouchedComponent))

(fn `UserConstructionScript`)