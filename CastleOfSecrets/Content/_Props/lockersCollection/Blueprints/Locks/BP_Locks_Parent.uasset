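; Base Blueprint for locker combination locks, handling keypad entry, password checking and open or closed state.
; Touch_Event animates button presses and appends or clears digits, refreshing a six-slot text display via ViewportPassword.
; Handle and handle-button events compare the entry to Password, animate timelines, toggle LockOpened and set OPENED or CLOSED feedback.
; Interact_Lock offers the lock only while both doors are closed and KeysLock is off; other interaction functions are default stubs.
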(event `self.ReceiveBeginPlay`
  (`|ExecutionSequence`
    (:`then_0`
      (bind _asfirst_person_character (cast `/Game/_Props/lockersCollection/DemoContent/FirstPersonBP/Blueprints/FirstPersonCharacter` (`GameplayStatics.GetPlayerCharacter` 0)))
      (set `self.Player` _asfirst_person_character))
    (:`then_1`
      (`SceneComponent.K2_SetWorldLocation` (`self.Look_Position`) (+ (`self.GetActorRightVector`) (`self.K2_GetActorLocation`)) false false))))

(event `Touch_Event`
  (params (Button :type "PrimitiveComponent Object Reference") (Delta :type "Float (double-precision)" :default 0.2) (Number :type String))
  (bind _tl_click (`self.TL_Click`))
  (bind _relativelocation (`SceneComponent.RelativeLocation` (`self.Clicked_Btn`)))
  ;[1 1 1] Touch_Event
  (if (not (`self.Lock_Opened`))
    (if (not (`TimelineComponent.IsPlaying` (`self.TL_Click`)))
      (set `self.Clicked_Btn` Button)
      (set `self.Start_Location` _relativelocation)
      (set `self.End_Location` (`KismetMathLibrary.MakeVector` (.x _relativelocation) (- (.y _relativelocation) Delta) (.z _relativelocation)))
      (bind (_direction _newtrack_0) (`Timeline|TL_Click` :!via `PlayFromStart`)
        (:`Update`
          (`SceneComponent.K2_SetRelativeLocation` (`self.Clicked_Btn`) (`KismetMathLibrary.VLerp` (`self.Start_Location`) (`self.End_Location`) _newtrack_0) false false)
          ;[1 1 1] Add Number for press
          (if (>= (`TimelineComponent.GetPlaybackPosition` _tl_click) (/ (`TimelineComponent.GetTimelineLength` _tl_click) 2.0))
            (`/Engine/EditorBlueprintResources/StandardMacros.DoOnce` false :!label _label
              (:`Completed`
                (if (not (`KismetStringLibrary.EqualEqual_StrStr` Number))
                  (`self.-AddNumber` Number)
                  (`self.-ViewportPassword`)
                  (else
                    (set `self.Entered_Password` "")
                    (`self.-ViewportPassword`)))))))
        (:`Finished`
          (goto _label :!via `Reset`))))))

(event `Handle_Event`
  (params (Handle_Mesh :type "PrimitiveComponent Object Reference"))
  ;[1 1 1] Handle Clike Event
  (if (not (`self.Lock_Opened`))
    (if (`KismetStringLibrary.EqualEqual_StrStr` (`self.Password`) (`self.Entered_Password`))
      (set `self.Lock_Opened` true)
      (bind (_direction _newtrack_0) (`Timeline|TL_Handle_Rotate` :!label _label_2)
        (:`Update`
          (`SceneComponent.K2_SetRelativeRotation` Handle_Mesh (`KismetMathLibrary.MakeRotator` (.roll (`SceneComponent.RelativeRotation` Handle_Mesh)) (`KismetMathLibrary.Lerp` 0.0 90.0 _newtrack_0) (.yaw (`SceneComponent.RelativeRotation` Handle_Mesh))) false false))
        (:`Finished`
          (set `self.Entered_Password` (`KismetMathLibrary.SelectString` "OPENED" "" (`self.Lock_Opened`)))))
      (else
        (bind (_direction_2 _newtrack_0_2) (`Timeline|Timeline_0` :!via `PlayFromStart`)
          (:`Update`
            (`SceneComponent.K2_SetRelativeRotation` Handle_Mesh (`KismetMathLibrary.MakeRotator` (.roll (`SceneComponent.RelativeRotation` Handle_Mesh)) (`KismetMathLibrary.Lerp` 0.0 15.0 _newtrack_0_2) (.yaw (`SceneComponent.RelativeRotation` Handle_Mesh))) false false))
          (:`Finished`
            (set `self.Entered_Password` "CLOSED")
            (`KismetSystemLibrary.Delay` 0.5)
            (set `self.Entered_Password` "")))))
    (else
      (set `self.Lock_Opened` false)
      (goto _label_2 :!via `ReverseFromEnd`))))

(event `Handle_Button_Event`
  (params (Handle_Button :type "PrimitiveComponent Object Reference"))
  (bind _relativelocation (`SceneComponent.RelativeLocation` Handle_Button))
  ;[1 1 1] Handle_Button_Event
  (`/Engine/EditorBlueprintResources/StandardMacros.IsValid` Handle_Button
    (:`Is Valid`
      (if (not (`TimelineComponent.IsPlaying` (`self.TL_Handle_Button`)))
        (set `self.Start_Location` _relativelocation)
        (set `self.End_Location` (`KismetMathLibrary.MakeVector` (.x _relativelocation) (- (.y _relativelocation) 0.1) (.z _relativelocation)))
        (if (not (`self.Lock_Opened`))
          (bind (_direction _newtrack_0) (`Timeline|TL_Handle_Button` :!via `PlayFromStart` :!label _label_3)
            (:`Update`
              (`SceneComponent.K2_SetRelativeLocation` Handle_Button (`KismetMathLibrary.VLerp` (`self.Start_Location`) (`self.End_Location`) _newtrack_0) false false))
            (:`Finished`
              (if (`KismetStringLibrary.EqualEqual_StrStr` (`self.Password`) (`self.Entered_Password`)) :!label _label_4
                (set `self.Lock_Opened` true))
              (if (`self.Lock_Opened`)
                (set `self.Entered_Password` (`KismetMathLibrary.SelectString` "OPENED" "" (`self.Lock_Opened`)))
                (`self.-ViewportPassword`)
                (else
                  (set `self.Entered_Password` "CLOSED")
                  (`self.-ViewportPassword`)
                  (`KismetSystemLibrary.Delay` 0.5)
                  (set `self.Entered_Password` "")
                  (`self.-ViewportPassword`)))))
          (else
            (set `self.Lock_Opened` false)
            (goto _label_3 :!via `PlayFromStart`)))))
    (:`Is Not Valid`
      (if (not (`self.Lock_Opened`))
        (goto _label_4)
        (else
          (set `self.Lock_Opened` false)
          (goto _label_4))))))

(fn `-AddNumber`
  (params (Number :type String))
  (bind _entered_password (`self.Entered_Password`))
  (if (<= (`KismetStringLibrary.Len` _entered_password) 6)
    (set `self.Entered_Password` (`KismetStringLibrary.Concat_StrStr` _entered_password Number))))

(fn `-ViewportPassword`
  (bind _viewport_password (`self.Viewport_Password`))
  (bind _entered_password (`self.Entered_Password`))
  (bind _returnvalue (`KismetStringLibrary.Len` _entered_password))
  (`SceneComponent.SetVisibility` _viewport_password (`self.ViewportPassword`) false)
  (`TextRenderComponent.K2_SetText` _viewport_password (`|FormatText` "{1} {2} {3} {4} {5} {6}" (`|FormatText` (select `bool` (>= _returnvalue 1) :`false` "_" :`true` (`KismetTextLibrary.Conv_StringToText` (`KismetStringLibrary.GetSubstring` _entered_password)))) (`|FormatText` (select `bool` (>= _returnvalue 2) :`false` "_" :`true` (`KismetTextLibrary.Conv_StringToText` (`KismetStringLibrary.GetSubstring` _entered_password 1)))) (`|FormatText` (select `bool` (>= _returnvalue 3) :`false` "_" :`true` (`KismetTextLibrary.Conv_StringToText` (`KismetStringLibrary.GetSubstring` _entered_password 2)))) (`|FormatText` (select `bool` (>= _returnvalue 4) :`false` "_" :`true` (`KismetTextLibrary.Conv_StringToText` (`KismetStringLibrary.GetSubstring` _entered_password 3)))) (`|FormatText` (select `bool` (>= _returnvalue 5) :`false` "_" :`true` (`KismetTextLibrary.Conv_StringToText` (`KismetStringLibrary.GetSubstring` _entered_password 4)))) (`|FormatText` (select `bool` (>= _returnvalue 6) :`false` "_" :`true` (`KismetTextLibrary.Conv_StringToText` (`KismetStringLibrary.GetSubstring` _entered_password 5)))))))

(fn `Doors`
  (params (HitComp :type "PrimitiveComponent Object Reference"))
  (returns (Success :type Boolean))
  (return false))

(fn `Interact_Key`
  (returns (Success :type Boolean) (Key_Num :type Integer))
  (return false 0))

(fn `Interact_Lock`
  (returns (Success :type Boolean) (Selected_Lock :type "/Game/_Props/lockersCollection/Blueprints/Locks/BP_Locks_Parent Object Reference"))
  (if (and (not (`self.Door_1_Open?`)) (not (`self.Door_2_Open?`)))
    (if (not (`self.Keys_Lock`))
      (return true self)
      (else
        (return false null)))
    (else
      (return false self))))

(fn `Key_Lock`
  (returns (Success :type Boolean))
  (return false))

(fn `Key_Lock_info`
  (returns (Success :type Boolean) (Lock_Opened :type Boolean) (Key :type Integer))
  (return false false 0))

(fn `UserConstructionScript`)