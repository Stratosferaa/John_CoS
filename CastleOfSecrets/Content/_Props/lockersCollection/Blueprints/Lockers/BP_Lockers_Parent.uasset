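; Parent Blueprint for lockable lockers with up to two hinged doors, an extra hinged element and an optional handle.
; Construction picks the lock child actor and handle mesh, attaches them to Door1 and clears non-numeric passwords.
; Tick syncs state with the lock, using DoOnce edges to spin the handle and notify the player for keyless locks.
; Timelines swing parts once unlocked; key and lock interaction functions are stubs returning false.
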(event `self.ReceiveTick`
  (params (DeltaSeconds :type "Float (single-precision)"))
  (bind _opened (`self.Opened`))
  (`|ExecutionSequence`
    (:`then_0`
      (bind _asbp_locks_parent (cast `/Game/_Props/lockersCollection/Blueprints/Locks/BP_Locks_Parent` (`ChildActorComponent.ChildActor` (`self.Lock`))))
      (set `self.Opened` (`/Game/_Props/lockersCollection/Blueprints/Locks/BP_Locks_Parent.Lock_Opened` _asbp_locks_parent))
      (set `/Game/_Props/lockersCollection/Blueprints/Locks/BP_Locks_Parent.Door_1_Open?` (`self.Door_1_Opened`) _asbp_locks_parent)
      (set `/Game/_Props/lockersCollection/Blueprints/Locks/BP_Locks_Parent.Door_2_Open?` (`self.Door_2_Opened`) _asbp_locks_parent)
      (set `/Game/_Props/lockersCollection/Blueprints/Locks/BP_Locks_Parent.Simple_Enter` (`self.Simple_Enter`) _asbp_locks_parent))
    (:`then_1`
      (if _opened
        (`/Engine/EditorBlueprintResources/StandardMacros.DoOnce` false :!label _label
          (:`Completed`
            (bind _asbp_locks_parent_2 (cast `/Game/_Props/lockersCollection/Blueprints/Locks/BP_Locks_Parent` (`ChildActorComponent.ChildActor` (`self.Lock`))))
            (if (not (`/Game/_Props/lockersCollection/Blueprints/Locks/BP_Locks_Parent.Keys_Lock` _asbp_locks_parent_2))
              (`/Game/_Props/lockersCollection/DemoContent/FirstPersonBP/Blueprints/FirstPersonCharacter.-Lock_Interact` (`self.Player`) _asbp_locks_parent_2))
            (`self.Handle_Rot_Event` false)))
        (else
          (goto _label :!via `Reset`))))
    (:`then_2`
      (if _opened
        (goto _label_2 :!via `Reset`)
        (else
          (`/Engine/EditorBlueprintResources/StandardMacros.DoOnce` true :!label _label_2
            (:`Completed`
              (`self.Handle_Rot_Event` true))))))))

(event `self.ReceiveBeginPlay`
  (bind _asfirst_person_character (cast `/Game/_Props/lockersCollection/DemoContent/FirstPersonBP/Blueprints/FirstPersonCharacter` (`GameplayStatics.GetPlayerCharacter` 0)))
  (set `self.Player` _asfirst_person_character)
  (bind _asbp_locks_parent (cast `/Game/_Props/lockersCollection/Blueprints/Locks/BP_Locks_Parent` (`ChildActorComponent.ChildActor` (`self.Lock`))))
  (set `/Game/_Props/lockersCollection/Blueprints/Locks/BP_Locks_Parent.Password` (`self.Password`) _asbp_locks_parent))

(event `Open_Door_1`
  (params (Reverse :type Boolean))
  (bind _returnvalue (not Reverse))
  (if (`self.Opened`)
    (if _returnvalue
      (set `self.Door_1_Opened` true)
      (bind (_direction _newtrack_0) (`Timeline|TL_Open_Door_1` :!label _label_3)
        (:`Update`
          (`SceneComponent.K2_SetRelativeRotation` (`self.Door_1`) (`KismetMathLibrary.MakeRotator` 0.0 0.0 (`KismetMathLibrary.Lerp` 0.0 (`self.End_Rot_Door_1`) _newtrack_0)) false false))
        (:`Finished`
          (if (not _returnvalue)
            (set `self.Door_1_Opened` false))))
      (else
        (goto _label_3 :!via `Reverse`)))))

(event `Handle_Rot_Event`
  (params (Reverse :type Boolean))
  (bind _pitch (.pitch (`SceneComponent.RelativeRotation` (`self.Handle`))))
  (`self.Handle`
    (:`then`
      (if (not Reverse)
        (set `self.HandleOriginY` _pitch)
        (set `self.HandleEndY` (+ _pitch -360.0))
        (bind (_direction _newtrack_0) (`Timeline|TL_Handle` :!via `PlayFromStart` :!label _label_4)
          (:`Update`
            (`SceneComponent.K2_SetRelativeRotation` (`self.Handle`) (`KismetMathLibrary.MakeRotator` 0.0 (`KismetMathLibrary.Lerp` (`self.HandleOriginY`) (`self.HandleEndY`) _newtrack_0)) false false)))
        (else
          (goto _label_4 :!via `ReverseFromEnd`))))
    (:`else`)))

(event `Open_Door_2`
  (params (Reverse :type Boolean) (X :type Boolean))
  (bind _returnvalue (not Reverse))
  (if (`self.Opened`)
    (if _returnvalue
      (set `self.Door_2_Opened` true)
      (bind (_direction _newtrack_0) (`Timeline|Timeline_0` :!label _label_5)
        (:`Update`
          (`SceneComponent.K2_SetRelativeRotation` (`self.Door_2`) (`KismetMathLibrary.MakeRotator` (`KismetMathLibrary.Lerp` 0.0 (`KismetMathLibrary.SelectFloat` (`self.End_Rot_Door_2_X`) 0.0 X) _newtrack_0) 0.0 (`KismetMathLibrary.Lerp` 0.0 (`KismetMathLibrary.SelectFloat` 0.0 (`self.End_Rot_Door_1`) X) _newtrack_0)) false false))
        (:`Finished`
          (if (not _returnvalue)
            (set `self.Door_2_Opened` false))))
      (else
        (goto _label_5 :!via `Reverse`)))))

(event `Open_Element`
  (params (Reverse :type Boolean))
  (bind _returnvalue (not Reverse))
  (if (`self.Opened`)
    (if _returnvalue
      (set `self.Door_element_Opened` true)
      (bind (_direction _newtrack_0) (`Timeline|Timeline_1` :!label _label_6)
        (:`Update`
          (`SceneComponent.K2_SetRelativeRotation` (`self.Element`) (`KismetMathLibrary.MakeRotator` (`KismetMathLibrary.Lerp` 0.0 80.0 _newtrack_0)) false false))
        (:`Finished`
          (if (not _returnvalue)
            (set `self.Door_element_Opened` false))))
      (else
        (goto _label_6 :!via `Reverse`)))))

(fn `Doors`
  (params (HitComp :type "PrimitiveComponent Object Reference"))
  (returns (Success :type Boolean))
  (bind _door_2 (`self.Door_2`))
  (if (== HitComp (`self.Door_1`))
    (if (not (`self.Door_1_Opened`))
      (`self.Open_Door_1` false)
      (return true)
      (elif (not (`self.Door_2_Opened`))
        (`self.Open_Door_1` true)
        (return true)))
    (else
      (`/Engine/EditorBlueprintResources/StandardMacros.IsValid` _door_2
        (:`Is Valid`
          (if (== HitComp _door_2)
            (if (not (`self.Door_2_Opened`))
              (`self.Open_Door_2` false)
              (return true)
              (else
                (`self.Open_Door_2` true)
                (return true)))))))))

(fn `Interact_Key`
  (returns (Success :type Boolean) (Key_Num :type Integer))
  (return false 0))

(fn `Interact_Lock`
  (returns (Success :type Boolean) (Selected_Lock :type "/Game/_Props/lockersCollection/Blueprints/Locks/BP_Locks_Parent Object Reference"))
  (return false null))

(fn `Key_Lock`
  (returns (Success :type Boolean))
  (return false))

(fn `Key_Lock_info`
  (returns (Success :type Boolean) (Lock_Opened :type Boolean) (Key :type Integer))
  (return false false 0))

(fn `UserConstructionScript`
  (bind _handle (`self.Handle`))
  (bind _lock (`self.Lock`))
  (bind _output (`|GetArrayItem` (`self.Locks`) (`self.Selected_Lock`)))
  (bind _output_2 (`|GetArrayItem` (`self.Handles_List`) (`self.Selected_Handle`)))
  (`|ExecutionSequence`
    (:`then_0`
      (set `self.Selected_Lock` (`KismetMathLibrary.Clamp` (`self.Selected_Lock`) 0 (`KismetArrayLibrary.Array_LastIndex` (`self.Locks`))))
      (if (not (== (`ChildActorComponent.ChildActorClass` (`self.Lock`)) _output))
        (`ChildActorComponent.SetChildActorClass` _lock _output)
        (`SceneComponent.K2_AttachToComponent` _lock (`self.Door_1`) "None" "KeepRelative" "KeepRelative" "KeepRelative" true)))
    (:`then_1`
      (if (`self.Have_Handle?`)
        (set `self.Selected_Handle` (`KismetMathLibrary.Clamp` (`self.Selected_Handle`) 0 (`KismetArrayLibrary.Array_LastIndex` (`self.Handles_List`))))
        (if (not (== (`self.Handle`) _output_2))
          (`StaticMeshComponent.SetStaticMesh` _handle _output_2)
          (`SceneComponent.K2_AttachToComponent` _handle (`self.Door_1`) "None" "KeepRelative" "KeepRelative" "KeepRelative" true))))
    (:`then_2`
      (if (not (`KismetStringLibrary.IsNumeric` (`self.Password`)))
        (set `self.Password` "")))))