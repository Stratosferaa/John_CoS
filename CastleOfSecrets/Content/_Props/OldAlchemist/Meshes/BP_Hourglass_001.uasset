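; Animated hourglass prop that runs its sand from top to bottom once play begins.
; A single timeline drives lerped scales of the top sand, pile and mountain meshes, also moving the pile and toggling mountain visibility.
; The dust stream shows while the timeline runs and hides when it finishes.
; The construction script derives play rate from Minutes and advances the timeline's time when AlreadyUsed is set.
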(event `self.ReceiveBeginPlay`
  (bind _p_dust_stream_001 (`self.P_Dust_Stream_001`))
  (`SceneComponent.SetVisibility` _p_dust_stream_001 true false)
  (bind (_direction _newtrack_0 _newtrack_1 _newtrack_2 _newtrack_3) (`Timeline|Timeline_0`)
    (:`Update`
      (`SceneComponent.SetRelativeScale3D` (`self.1`) (`KismetMathLibrary.VLerp` (`KismetMathLibrary.VLerp` (`self.Top Empty`) (`self.Top Full`) _newtrack_0) (0.0 0.0 0.0) _newtrack_1))
      (bind _returnvalue (`KismetMathLibrary.VLerp` (`self.Pile full`) (0.0 0.0 0.0) _newtrack_2))
      (`SceneComponent.SetRelativeScale3D` (`self.2`) _returnvalue)
      (`SceneComponent.SetRelativeScale3D` (`self.3`) (`KismetMathLibrary.VLerp` (`self.Mountain empty`) (1.0 1.0 1.0) _newtrack_3))
      (`SceneComponent.K2_SetRelativeLocation` (`self.2`) (`KismetMathLibrary.VLerp` (`self.Pile position start`) (`self.Pile position end`) _newtrack_3) false false)
      (`SceneComponent.SetRelativeScale3D` (`self.2`) (`KismetMathLibrary.VLerp` _returnvalue (`self.Pile complete`) _newtrack_3))
      (`SceneComponent.SetVisibility` (`self.3`) (> _newtrack_3 0.0) false))
    (:`Finished`
      (`SceneComponent.SetVisibility` _p_dust_stream_001 false false))))

(event `self.ReceiveTick`
  (params (DeltaSeconds :type "Float (single-precision)")))

(fn `UserConstructionScript`
  (bind _timeline_0 (`self.Timeline_0`))
  (`TimelineComponent.SetPlayRate` _timeline_0 (/ 1.0 (`self.Minutes`)))
  (if (`self.Already used`)
    (`TimelineComponent.SetNewTime` _timeline_0 60.0)))