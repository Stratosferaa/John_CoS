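; BP_Sand_Bath_001 is an alchemist's sand bath prop with two particle systems and a point light that can be switched on or off.
; The construction script sets the visibility of both particle systems and the light from the TurnONOFF flag.
; On BeginPlay, a timeline drives the light's relative position with half-scaled movement around a fixed offset, making it waver.
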(event `self.ReceiveBeginPlay`
  (bind (_direction _light_movement) (`Timeline|Timeline_0`)
    (:`Update`
      (`SceneComponent.K2_SetRelativeLocation` (`self.PointLight`) (+ (`KismetMathLibrary.MakeVector` 0.0 12.058725 33.397415) (* _light_movement 0.5)) false false))))

(fn `UserConstructionScript`
  (`SceneComponent.SetVisibility` (`self.ParticleSystem1`) (`self.Turn ON/OFF`) false)
  (`SceneComponent.SetVisibility` (`self.PointLight`) (`self.Turn ON/OFF`) false)
  (`SceneComponent.SetVisibility` (`self.ParticleSystem`) (`self.Turn ON/OFF`) false))