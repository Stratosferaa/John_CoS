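; Configurable alchemist spiral furnace prop, assembled entirely in the Construction Script with no runtime logic.
; Exposed variables toggle the fire particles and light, show and vertically scale the chimney, and show or hide decorative glassware and liquid meshes.
; Three liquid meshes each get a dynamic instance of the glassware liquid material, driven by the bubbling, top and bottom color, and opacity settings.
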(fn `UserConstructionScript`
  (bind _sm_glassware_001_liquid (`self.SM_Glassware_001_liquid`))
  (bind _c1 (`self.c1`))
  (`SceneComponent.SetVisibility` (`self.P_Athanor_Fire_001`) (`self.Turn ON/OFF`) false)
  (`SceneComponent.SetVisibility` (`self.ParticleSystem`) (`self.Turn ON/OFF`) false)
  (`SceneComponent.SetVisibility` (`self.ParticleSystem1`) (`self.Turn ON/OFF`) false)
  (`SceneComponent.SetVisibility` (`self.ParticleSystem2`) (`self.Turn ON/OFF`) false)
  (`SceneComponent.SetVisibility` (`self.PointLight`) (`self.Turn ON/OFF`) false)
  (`SceneComponent.SetVisibility` _c1 (`self.Add Cimney`) false)
  (`SceneComponent.SetRelativeScale3D` _c1 (`KismetMathLibrary.MakeVector` 1.0 1.0 (`self.Cimney Height`)))
  (`SceneComponent.SetVisibility` (`self.StaticMesh4`) (`self.Decorative_Bottles`) false)
  (`SceneComponent.SetVisibility` (`self.2`) (`self.Decorative_Bottles`) false)
  (`SceneComponent.SetVisibility` (`self.3`) (`self.Decorative_Bottles`) false)
  (`SceneComponent.SetVisibility` (`self.4`) (`self.Decorative_Bottles`) false)
  (`SceneComponent.SetVisibility` (`self.StaticMesh`) (`self.Decorative_Bottles`) false)
  (`SceneComponent.SetVisibility` (`self.StaticMesh1`) (`self.Decorative_Bottles`) false)
  (`SceneComponent.SetVisibility` (`self.StaticMesh2`) (`self.Decorative_Bottles`) false)
  (`SceneComponent.SetVisibility` (`self.StaticMesh3`) (`self.Decorative_Bottles`) false)
  (`SceneComponent.SetVisibility` (`self.SM_Glassware_004`) (`self.Decorative_Bottles`) false)
  (`SceneComponent.SetVisibility` (`self.SM_Glassware_001`) (`self.Decorative_Bottles`) false)
  (`SceneComponent.SetVisibility` (`self.1`) (`self.Decorative_Bottles`) false)
  (`SceneComponent.SetVisibility` (`self.StaticMesh7`) (`self.Decorative_Bottles`) false)
  (`SceneComponent.SetVisibility` (`self.StaticMesh5`) (`self.Decorative_Bottles`) false)
  (`SceneComponent.SetVisibility` (`self.SM_Jar_Lid_001`) (`self.Decorative_Bottles`) false)
  (`SceneComponent.SetVisibility` (`self.StaticMesh6`) (`self.Decorative_Bottles`) false)
  (`SceneComponent.SetVisibility` (`self.StaticMesh8`) (`self.Decorative_Bottles`) false)
  (`SceneComponent.SetVisibility` (`self.StaticMesh9`) (`self.Decorative_Bottles`) false)
  (`SceneComponent.SetVisibility` (`self.StaticMesh10`) (`self.Decorative_Bottles`) false)
  (`SceneComponent.SetVisibility` (`self.StaticMesh11`) (`self.Decorative_Bottles`) false)
  (`SceneComponent.SetVisibility` (`self.StaticMesh12`) (`self.Decorative_Bottles`) false)
  (`SceneComponent.SetVisibility` (`self.StaticMesh13`) (`self.Decorative_Bottles`) false)
  (`SceneComponent.SetVisibility` (`self.StaticMesh18`) (`self.Decorative_Bottles`) false)
  (`SceneComponent.SetVisibility` (`self.StaticMesh19`) (`self.Decorative_Bottles`) false)
  (`SceneComponent.SetVisibility` (`self.StaticMesh16`) (`self.Decorative_Bottles`) false)
  (`SceneComponent.SetVisibility` (`self.StaticMesh14`) (`self.Decorative_Bottles`) false)
  (`SceneComponent.SetVisibility` (`self.StaticMesh15`) (`self.Decorative_Bottles`) false)
  (`SceneComponent.SetVisibility` (`self.StaticMesh17`) (`self.Decorative_Bottles`) false)
  (if (`self.Add Liquid`)
    (`SceneComponent.SetVisibility` _sm_glassware_001_liquid true false)
    (`SceneComponent.SetVisibility` (`self.StaticMesh21`) true false)
    (`SceneComponent.SetVisibility` (`self.StaticMesh22`) true false)
    (else
      (`SceneComponent.SetVisibility` _sm_glassware_001_liquid false false)
      (`SceneComponent.SetVisibility` (`self.StaticMesh21`) false false)
      (`SceneComponent.SetVisibility` (`self.StaticMesh22`) false false)))
  (bind _returnvalue (`PrimitiveComponent.CreateDynamicMaterialInstance` (`self.SM_Glassware_001_liquid`) 0 "/Game/_Props/OldAlchemist/Materials/Meshspecific/MI_Glassware_Liquid_001.MI_Glassware_Liquid_001" "None"))
  (bind _returnvalue_2 (`PrimitiveComponent.CreateDynamicMaterialInstance` (`self.StaticMesh21`) 0 "/Game/_Props/OldAlchemist/Materials/Meshspecific/MI_Glassware_Liquid_001.MI_Glassware_Liquid_001" "None"))
  (bind _returnvalue_3 (`PrimitiveComponent.CreateDynamicMaterialInstance` (`self.StaticMesh22`) 0 "/Game/_Props/OldAlchemist/Materials/Meshspecific/MI_Glassware_Liquid_001.MI_Glassware_Liquid_001" "None"))
  (`MaterialInstanceDynamic.SetScalarParameterValue` _returnvalue "Bubbling_Intensity" (`self.Liquid Bubbling Amount`))
  (`MaterialInstanceDynamic.SetScalarParameterValue` _returnvalue_2 "Bubbling_Intensity" (`self.Liquid Bubbling Amount`))
  (`MaterialInstanceDynamic.SetScalarParameterValue` _returnvalue_3 "Bubbling_Intensity" (`self.Liquid Bubbling Amount`))
  (`MaterialInstanceDynamic.SetScalarParameterValue` _returnvalue "Bubbling_MAX" (`self.Bubbling MAX`))
  (`MaterialInstanceDynamic.SetScalarParameterValue` _returnvalue_2 "Bubbling_MAX" (`self.Bubbling MAX`))
  (`MaterialInstanceDynamic.SetScalarParameterValue` _returnvalue_3 "Bubbling_MAX" (`self.Bubbling MAX`))
  (`MaterialInstanceDynamic.SetScalarParameterValue` _returnvalue "Bubbling_MIN" (`self.Bubbling MIN`))
  (`MaterialInstanceDynamic.SetScalarParameterValue` _returnvalue_2 "Bubbling_MIN" (`self.Bubbling MIN`))
  (`MaterialInstanceDynamic.SetScalarParameterValue` _returnvalue_3 "Bubbling_MIN" (`self.Bubbling MIN`))
  (`MaterialInstanceDynamic.SetVectorParameterValue` _returnvalue "Color_Top" (`self.Liquid Color Top`))
  (`MaterialInstanceDynamic.SetVectorParameterValue` _returnvalue_2 "Color_Top" (`self.Liquid Color Top`))
  (`MaterialInstanceDynamic.SetVectorParameterValue` _returnvalue_3 "Color_Top" (`self.Liquid Color Top`))
  (`MaterialInstanceDynamic.SetVectorParameterValue` _returnvalue "Color_Bottom" (`self.Liquid Color Bottom`))
  (`MaterialInstanceDynamic.SetVectorParameterValue` _returnvalue_2 "Color_Bottom" (`self.Liquid Color Bottom`))
  (`MaterialInstanceDynamic.SetVectorParameterValue` _returnvalue_3 "Color_Bottom" (`self.Liquid Color Bottom`))
  (`MaterialInstanceDynamic.SetScalarParameterValue` _returnvalue "Opacity Top" (`self.Liquid Opacity Top`))
  (`MaterialInstanceDynamic.SetScalarParameterValue` _returnvalue_2 "Opacity Top" (`self.Liquid Opacity Top`))
  (`MaterialInstanceDynamic.SetScalarParameterValue` _returnvalue_3 "Opacity Top" (`self.Liquid Opacity Top`))
  (`MaterialInstanceDynamic.SetScalarParameterValue` _returnvalue "Opacity Bottom" (`self.Liquid Opacity Bottom`))
  (`MaterialInstanceDynamic.SetScalarParameterValue` _returnvalue_2 "Opacity Bottom" (`self.Liquid Opacity Bottom`))
  (`MaterialInstanceDynamic.SetScalarParameterValue` _returnvalue_3 "Opacity Bottom" (`self.Liquid Opacity Bottom`)))