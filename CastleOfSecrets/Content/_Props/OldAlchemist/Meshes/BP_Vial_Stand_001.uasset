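; Alchemist prop stand of six vials that randomizes its look in the construction script, with no active runtime logic.
; Each vial gets dynamic glass, liquid and tag materials from shared variables, plus random top color, tag sign, tag height, rotation and fill.
; Random fill overwrites LiquidAmount, and a final per-vial visibility pass overrides the individual lid, tag and liquid toggles.
; RefreshMesh only resets itself, acting as a re-roll toggle.
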(fn `UserConstructionScript`
  (bind _tag_01 (`self.Tag_01`))
  (bind _tag_02 (`self.Tag_02`))
  (bind _tag_03 (`self.Tag_03`))
  (bind _tag_04 (`self.Tag_04`))
  (bind _tag_05 (`self.Tag_05`))
  (bind _tag_06 (`self.Tag_06`))
  (if (`self.Refresh Mesh`)
    _
    (else
      _))
  (set `self.Refresh Mesh` false)
  (`SceneComponent.SetVisibility` (`self.liquid_01`) (`KismetMathLibrary.RandomBool`) false)
  (`PrimitiveComponent.SetTranslucentSortPriority` (`self.Vial_01`) 1)
  (bind _returnvalue (`PrimitiveComponent.CreateDynamicMaterialInstance` (`self.liquid_01`) 0 "/Game/_Props/OldAlchemist/Materials/Meshspecific/MI_Glassware_Liquid_001.MI_Glassware_Liquid_001" "None"))
  (`MaterialInstanceDynamic.SetScalarParameterValue` _returnvalue "Bubbling_Intensity" (`self.Liquid Bubbling Amount`))
  (`MaterialInstanceDynamic.SetScalarParameterValue` _returnvalue "Bubbling_MAX" (`self.Bubbling MAX`))
  (`MaterialInstanceDynamic.SetScalarParameterValue` _returnvalue "Bubbling_MIN" (`self.Bubbling MIN`))
  (`MaterialInstanceDynamic.SetVectorParameterValue` _returnvalue "Color_Top" (`KismetMathLibrary.Conv_VectorToLinearColor` (`KismetMathLibrary.MakeVector` (`KismetMathLibrary.RandomFloatInRange` 0.0 1.0) (`KismetMathLibrary.RandomFloatInRange` 0.0 1.0) (`KismetMathLibrary.RandomFloatInRange` 0.0 1.0))))
  (`MaterialInstanceDynamic.SetVectorParameterValue` _returnvalue "Color_Bottom" (`self.Liquid Color Bottom`))
  (`MaterialInstanceDynamic.SetScalarParameterValue` _returnvalue "Opacity Top" (`self.Liquid Opacity Top`))
  (`MaterialInstanceDynamic.SetScalarParameterValue` _returnvalue "Opacity Bottom" (`self.Liquid Opacity Bottom`))
  (`SceneComponent.SetVisibility` (`self.Lid_01`) (`KismetMathLibrary.RandomBool`) false)
  (bind _returnvalue_2 (`PrimitiveComponent.CreateDynamicMaterialInstance` (`self.Vial_01`) 0 "/Game/_Props/OldAlchemist/Materials/Meshspecific/MI_Glassware_007.MI_Glassware_007" "None"))
  (`MaterialInstanceDynamic.SetVectorParameterValue` _returnvalue_2 "Color Multiplier" (`self.Glass Color Multiplier`))
  (`MaterialInstanceDynamic.SetScalarParameterValue` _returnvalue_2 "Hue shift percentage" (`self.Glass Hue Shift`))
  (bind _returnvalue_3 (`PrimitiveComponent.CreateDynamicMaterialInstance` _tag_01 0 "/Game/_Props/OldAlchemist/Materials/Meshspecific/MI_Tags_001.MI_Tags_001" "None"))
  (`MaterialInstanceDynamic.SetScalarParameterValue` _returnvalue_3 "Flip between signs" (`KismetMathLibrary.RandomFloatInRange` 0.0 1.0))
  (`SceneComponent.SetVisibility` _tag_01 (`KismetMathLibrary.RandomBool`) false)
  (`SceneComponent.SetRelativeScale3D` (`self.liquid_01`) (`KismetMathLibrary.MakeVector` 1.0 1.0 (`self.Liquid Amount`)))
  (`SceneComponent.K2_SetRelativeLocation` (`self.Tag_01`) (`KismetMathLibrary.MakeVector` 0.025693 0.023674 (`KismetMathLibrary.RandomFloatInRange` 2.442998 10.559464)) false false)
  (`SceneComponent.K2_SetRelativeRotation` (`self.Vial_01`) (`KismetMathLibrary.MakeRotator` (`KismetMathLibrary.RandomFloatInRange` 0.0 2.0) (`KismetMathLibrary.RandomFloatInRange` 0.0 2.0) (`KismetMathLibrary.RandomFloatInRange` 0.0 360.0)) false false)
  (`SceneComponent.SetRelativeScale3D` (`self.liquid_01`) (`KismetMathLibrary.MakeVector` 1.0 1.0 (`KismetMathLibrary.RandomFloatInRange` 0.110981 1.692634)))
  (`SceneComponent.SetVisibility` (`self.Tag_01`) (`KismetMathLibrary.RandomBool`) true)
  (`SceneComponent.SetVisibility` (`self.liquid_01`) (`KismetMathLibrary.RandomBool`) true)
  (`SceneComponent.SetVisibility` (`self.Lid_01`) (`KismetMathLibrary.RandomBool`) true)
  (`SceneComponent.SetVisibility` (`self.Vial_01`) (`KismetMathLibrary.RandomBool`) true)
  (`SceneComponent.SetVisibility` (`self.Liquid_02`) (`KismetMathLibrary.RandomBool`) false)
  (`PrimitiveComponent.SetTranslucentSortPriority` (`self.Vial_02`) 1)
  (bind _returnvalue_4 (`PrimitiveComponent.CreateDynamicMaterialInstance` (`self.Liquid_02`) 0 "/Game/_Props/OldAlchemist/Materials/Meshspecific/MI_Glassware_Liquid_001.MI_Glassware_Liquid_001" "None"))
  (`MaterialInstanceDynamic.SetScalarParameterValue` _returnvalue_4 "Bubbling_Intensity" (`self.Liquid Bubbling Amount`))
  (`MaterialInstanceDynamic.SetScalarParameterValue` _returnvalue_4 "Bubbling_MAX" (`self.Bubbling MAX`))
  (`MaterialInstanceDynamic.SetScalarParameterValue` _returnvalue_4 "Bubbling_MIN" (`self.Bubbling MIN`))
  (`MaterialInstanceDynamic.SetVectorParameterValue` _returnvalue_4 "Color_Top" (`KismetMathLibrary.Conv_VectorToLinearColor` (`KismetMathLibrary.MakeVector` (`KismetMathLibrary.RandomFloatInRange` 0.0 1.0) (`KismetMathLibrary.RandomFloatInRange` 0.0 1.0) (`KismetMathLibrary.RandomFloatInRange` 0.0 1.0))))
  (`MaterialInstanceDynamic.SetVectorParameterValue` _returnvalue_4 "Color_Bottom" (`self.Liquid Color Bottom`))
  (`MaterialInstanceDynamic.SetScalarParameterValue` _returnvalue_4 "Opacity Top" (`self.Liquid Opacity Top`))
  (`MaterialInstanceDynamic.SetScalarParameterValue` _returnvalue_4 "Opacity Bottom" (`self.Liquid Opacity Bottom`))
  (`SceneComponent.SetVisibility` (`self.Lid_02`) (`KismetMathLibrary.RandomBool`) false)
  (bind _returnvalue_5 (`PrimitiveComponent.CreateDynamicMaterialInstance` (`self.Vial_02`) 0 "/Game/_Props/OldAlchemist/Materials/Meshspecific/MI_Glassware_007.MI_Glassware_007" "None"))
  (`MaterialInstanceDynamic.SetVectorParameterValue` _returnvalue_5 "Color Multiplier" (`self.Glass Color Multiplier`))
  (`MaterialInstanceDynamic.SetScalarParameterValue` _returnvalue_5 "Hue shift percentage" (`self.Glass Hue Shift`))
  (bind _returnvalue_6 (`PrimitiveComponent.CreateDynamicMaterialInstance` _tag_02 0 "/Game/_Props/OldAlchemist/Materials/Meshspecific/MI_Tags_001.MI_Tags_001" "None"))
  (`MaterialInstanceDynamic.SetScalarParameterValue` _returnvalue_6 "Flip between signs" (`KismetMathLibrary.RandomFloatInRange` 0.0 1.0))
  (`SceneComponent.SetVisibility` _tag_02 (`KismetMathLibrary.RandomBool`) false)
  (`SceneComponent.SetRelativeScale3D` (`self.Liquid_02`) (`KismetMathLibrary.MakeVector` 1.0 1.0 (`self.Liquid Amount`)))
  (`SceneComponent.K2_SetRelativeLocation` (`self.Tag_02`) (`KismetMathLibrary.MakeVector` 0.025693 0.023674 (`KismetMathLibrary.RandomFloatInRange` 2.442998 10.559464)) false false)
  (`SceneComponent.K2_SetRelativeRotation` (`self.Vial_02`) (`KismetMathLibrary.MakeRotator` (`KismetMathLibrary.RandomFloatInRange` 0.0 2.0) (`KismetMathLibrary.RandomFloatInRange` 0.0 2.0) (`KismetMathLibrary.RandomFloatInRange` 0.0 360.0)) false false)
  (`SceneComponent.SetRelativeScale3D` (`self.Liquid_02`) (`KismetMathLibrary.MakeVector` 1.0 1.0 (`KismetMathLibrary.RandomFloatInRange` 0.110981 1.692634)))
  (`SceneComponent.SetVisibility` (`self.Vial_02`) (`KismetMathLibrary.RandomBool`) true)
  (`SceneComponent.SetVisibility` (`self.Lid_02`) (`KismetMathLibrary.RandomBool`) true)
  (`SceneComponent.SetVisibility` (`self.Tag_02`) (`KismetMathLibrary.RandomBool`) true)
  (`SceneComponent.SetVisibility` (`self.Liquid_02`) (`KismetMathLibrary.RandomBool`) true)
  (`SceneComponent.SetVisibility` (`self.Liquid_03`) (`KismetMathLibrary.RandomBool`) false)
  (`PrimitiveComponent.SetTranslucentSortPriority` (`self.Vial_03`) 1)
  (bind _returnvalue_7 (`PrimitiveComponent.CreateDynamicMaterialInstance` (`self.Liquid_03`) 0 "/Game/_Props/OldAlchemist/Materials/Meshspecific/MI_Glassware_Liquid_001.MI_Glassware_Liquid_001" "None"))
  (`MaterialInstanceDynamic.SetScalarParameterValue` _returnvalue_7 "Bubbling_Intensity" (`self.Liquid Bubbling Amount`))
  (`MaterialInstanceDynamic.SetScalarParameterValue` _returnvalue_7 "Bubbling_MAX" (`self.Bubbling MAX`))
  (`MaterialInstanceDynamic.SetScalarParameterValue` _returnvalue_7 "Bubbling_MIN" (`self.Bubbling MIN`))
  (`MaterialInstanceDynamic.SetVectorParameterValue` _returnvalue_7 "Color_Top" (`KismetMathLibrary.Conv_VectorToLinearColor` (`KismetMathLibrary.MakeVector` (`KismetMathLibrary.RandomFloatInRange` 0.0 1.0) (`KismetMathLibrary.RandomFloatInRange` 0.0 1.0) (`KismetMathLibrary.RandomFloatInRange` 0.0 1.0))))
  (`MaterialInstanceDynamic.SetVectorParameterValue` _returnvalue_7 "Color_Bottom" (`self.Liquid Color Bottom`))
  (`MaterialInstanceDynamic.SetScalarParameterValue` _returnvalue_7 "Opacity Top" (`self.Liquid Opacity Top`))
  (`MaterialInstanceDynamic.SetScalarParameterValue` _returnvalue_7 "Opacity Bottom" (`self.Liquid Opacity Bottom`))
  (`SceneComponent.SetVisibility` (`self.Lid_03`) (`KismetMathLibrary.RandomBool`) false)
  (bind _returnvalue_8 (`PrimitiveComponent.CreateDynamicMaterialInstance` (`self.Vial_03`) 0 "/Game/_Props/OldAlchemist/Materials/Meshspecific/MI_Glassware_007.MI_Glassware_007" "None"))
  (`MaterialInstanceDynamic.SetVectorParameterValue` _returnvalue_8 "Color Multiplier" (`self.Glass Color Multiplier`))
  (`MaterialInstanceDynamic.SetScalarParameterValue` _returnvalue_8 "Hue shift percentage" (`self.Glass Hue Shift`))
  (bind _returnvalue_9 (`PrimitiveComponent.CreateDynamicMaterialInstance` _tag_03 0 "/Game/_Props/OldAlchemist/Materials/Meshspecific/MI_Tags_001.MI_Tags_001" "None"))
  (`MaterialInstanceDynamic.SetScalarParameterValue` _returnvalue_9 "Flip between signs" (`KismetMathLibrary.RandomFloatInRange` 0.0 1.0))
  (`SceneComponent.SetVisibility` _tag_03 (`KismetMathLibrary.RandomBool`) false)
  (`SceneComponent.SetRelativeScale3D` (`self.Liquid_03`) (`KismetMathLibrary.MakeVector` 1.0 1.0 (`self.Liquid Amount`)))
  (`SceneComponent.K2_SetRelativeLocation` (`self.Tag_03`) (`KismetMathLibrary.MakeVector` 0.025693 0.023674 (`KismetMathLibrary.RandomFloatInRange` 2.442998 10.559464)) false false)
  (`SceneComponent.K2_SetRelativeRotation` (`self.Vial_03`) (`KismetMathLibrary.MakeRotator` (`KismetMathLibrary.RandomFloatInRange` 0.0 2.0) (`KismetMathLibrary.RandomFloatInRange` 0.0 2.0) (`KismetMathLibrary.RandomFloatInRange` 0.0 360.0)) false false)
  (`SceneComponent.SetRelativeScale3D` (`self.Liquid_03`) (`KismetMathLibrary.MakeVector` 1.0 1.0 (`KismetMathLibrary.RandomFloatInRange` 0.110981 1.692634)))
  (`SceneComponent.SetVisibility` (`self.Vial_03`) (`KismetMathLibrary.RandomBool`) true)
  (`SceneComponent.SetVisibility` (`self.Lid_03`) (`KismetMathLibrary.RandomBool`) true)
  (`SceneComponent.SetVisibility` (`self.Liquid_03`) (`KismetMathLibrary.RandomBool`) true)
  (`SceneComponent.SetVisibility` (`self.Tag_03`) (`KismetMathLibrary.RandomBool`) true)
  (`SceneComponent.SetVisibility` (`self.Liquid_04`) (`KismetMathLibrary.RandomBool`) false)
  (`PrimitiveComponent.SetTranslucentSortPriority` (`self.Vial_04`) 1)
  (bind _returnvalue_10 (`PrimitiveComponent.CreateDynamicMaterialInstance` (`self.Liquid_04`) 0 "/Game/_Props/OldAlchemist/Materials/Meshspecific/MI_Glassware_Liquid_001.MI_Glassware_Liquid_001" "None"))
  (`MaterialInstanceDynamic.SetScalarParameterValue` _returnvalue_10 "Bubbling_Intensity" (`self.Liquid Bubbling Amount`))
  (`MaterialInstanceDynamic.SetScalarParameterValue` _returnvalue_10 "Bubbling_MAX" (`self.Bubbling MAX`))
  (`MaterialInstanceDynamic.SetScalarParameterValue` _returnvalue_10 "Bubbling_MIN" (`self.Bubbling MIN`))
  (`MaterialInstanceDynamic.SetVectorParameterValue` _returnvalue_10 "Color_Top" (`KismetMathLibrary.Conv_VectorToLinearColor` (`KismetMathLibrary.MakeVector` (`KismetMathLibrary.RandomFloatInRange` 0.0 1.0) (`KismetMathLibrary.RandomFloatInRange` 0.0 1.0) (`KismetMathLibrary.RandomFloatInRange` 0.0 1.0))))
  (`MaterialInstanceDynamic.SetVectorParameterValue` _returnvalue_10 "Color_Bottom" (`self.Liquid Color Bottom`))
  (`MaterialInstanceDynamic.SetScalarParameterValue` _returnvalue_10 "Opacity Top" (`self.Liquid Opacity Top`))
  (`MaterialInstanceDynamic.SetScalarParameterValue` _returnvalue_10 "Opacity Bottom" (`self.Liquid Opacity Bottom`))
  (`SceneComponent.SetVisibility` (`self.Lid_04`) (`KismetMathLibrary.RandomBool`) false)
  (bind _returnvalue_11 (`PrimitiveComponent.CreateDynamicMaterialInstance` (`self.Vial_04`) 0 "/Game/_Props/OldAlchemist/Materials/Meshspecific/MI_Glassware_007.MI_Glassware_007" "None"))
  (`MaterialInstanceDynamic.SetVectorParameterValue` _returnvalue_11 "Color Multiplier" (`self.Glass Color Multiplier`))
  (`MaterialInstanceDynamic.SetScalarParameterValue` _returnvalue_11 "Hue shift percentage" (`self.Glass Hue Shift`))
  (bind _returnvalue_12 (`PrimitiveComponent.CreateDynamicMaterialInstance` _tag_04 0 "/Game/_Props/OldAlchemist/Materials/Meshspecific/MI_Tags_001.MI_Tags_001" "None"))
  (`MaterialInstanceDynamic.SetScalarParameterValue` _returnvalue_12 "Flip between signs" (`KismetMathLibrary.RandomFloatInRange` 0.0 1.0))
  (`SceneComponent.SetVisibility` _tag_04 (`KismetMathLibrary.RandomBool`) false)
  (`SceneComponent.SetRelativeScale3D` (`self.Liquid_04`) (`KismetMathLibrary.MakeVector` 1.0 1.0 (`self.Liquid Amount`)))
  (`SceneComponent.K2_SetRelativeLocation` (`self.Tag_04`) (`KismetMathLibrary.MakeVector` 0.025693 0.023674 (`KismetMathLibrary.RandomFloatInRange` 2.442998 10.559464)) false false)
  (`SceneComponent.K2_SetRelativeRotation` (`self.Vial_04`) (`KismetMathLibrary.MakeRotator` (`KismetMathLibrary.RandomFloatInRange` 0.0 2.0) (`KismetMathLibrary.RandomFloatInRange` 0.0 2.0) (`KismetMathLibrary.RandomFloatInRange` 0.0 360.0)) false false)
  (`SceneComponent.SetRelativeScale3D` (`self.Liquid_04`) (`KismetMathLibrary.MakeVector` 1.0 1.0 (`KismetMathLibrary.RandomFloatInRange` 0.110981 1.692634)))
  (`SceneComponent.SetVisibility` (`self.Vial_04`) (`KismetMathLibrary.RandomBool`) true)
  (`SceneComponent.SetVisibility` (`self.Lid_04`) (`KismetMathLibrary.RandomBool`) true)
  (`SceneComponent.SetVisibility` (`self.Tag_04`) (`KismetMathLibrary.RandomBool`) true)
  (`SceneComponent.SetVisibility` (`self.Liquid_04`) (`KismetMathLibrary.RandomBool`) true)
  (`SceneComponent.SetVisibility` (`self.Liquid_05`) (`KismetMathLibrary.RandomBool`) false)
  (`PrimitiveComponent.SetTranslucentSortPriority` (`self.Vial_05`) 1)
  (bind _returnvalue_13 (`PrimitiveComponent.CreateDynamicMaterialInstance` (`self.Liquid_05`) 0 "/Game/_Props/OldAlchemist/Materials/Meshspecific/MI_Glassware_Liquid_001.MI_Glassware_Liquid_001" "None"))
  (`MaterialInstanceDynamic.SetScalarParameterValue` _returnvalue_13 "Bubbling_Intensity" (`self.Liquid Bubbling Amount`))
  (`MaterialInstanceDynamic.SetScalarParameterValue` _returnvalue_13 "Bubbling_MAX" (`self.Bubbling MAX`))
  (`MaterialInstanceDynamic.SetScalarParameterValue` _returnvalue_13 "Bubbling_MIN" (`self.Bubbling MIN`))
  (`MaterialInstanceDynamic.SetVectorParameterValue` _returnvalue_13 "Color_Top" (`KismetMathLibrary.Conv_VectorToLinearColor` (`KismetMathLibrary.MakeVector` (`KismetMathLibrary.RandomFloatInRange` 0.0 1.0) (`KismetMathLibrary.RandomFloatInRange` 0.0 1.0) (`KismetMathLibrary.RandomFloatInRange` 0.0 1.0))))
  (`MaterialInstanceDynamic.SetVectorParameterValue` _returnvalue_13 "Color_Bottom" (`self.Liquid Color Bottom`))
  (`MaterialInstanceDynamic.SetScalarParameterValue` _returnvalue_13 "Opacity Top" (`self.Liquid Opacity Top`))
  (`MaterialInstanceDynamic.SetScalarParameterValue` _returnvalue_13 "Opacity Bottom" (`self.Liquid Opacity Bottom`))
  (`SceneComponent.SetVisibility` (`self.Lid_05`) (`KismetMathLibrary.RandomBool`) false)
  (bind _returnvalue_14 (`PrimitiveComponent.CreateDynamicMaterialInstance` (`self.Vial_05`) 0 "/Game/_Props/OldAlchemist/Materials/Meshspecific/MI_Glassware_007.MI_Glassware_007" "None"))
  (`MaterialInstanceDynamic.SetVectorParameterValue` _returnvalue_14 "Color Multiplier" (`self.Glass Color Multiplier`))
  (`MaterialInstanceDynamic.SetScalarParameterValue` _returnvalue_14 "Hue shift percentage" (`self.Glass Hue Shift`))
  (bind _returnvalue_15 (`PrimitiveComponent.CreateDynamicMaterialInstance` _tag_05 0 "/Game/_Props/OldAlchemist/Materials/Meshspecific/MI_Tags_001.MI_Tags_001" "None"))
  (`MaterialInstanceDynamic.SetScalarParameterValue` _returnvalue_15 "Flip between signs" (`KismetMathLibrary.RandomFloatInRange` 0.0 1.0))
  (`SceneComponent.SetVisibility` _tag_05 (`KismetMathLibrary.RandomBool`) false)
  (`SceneComponent.SetRelativeScale3D` (`self.Liquid_05`) (`KismetMathLibrary.MakeVector` 1.0 1.0 (`self.Liquid Amount`)))
  (`SceneComponent.K2_SetRelativeLocation` (`self.Tag_05`) (`KismetMathLibrary.MakeVector` 0.025693 0.023674 (`KismetMathLibrary.RandomFloatInRange` 2.442998 10.559464)) false false)
  (`SceneComponent.K2_SetRelativeRotation` (`self.Vial_05`) (`KismetMathLibrary.MakeRotator` (`KismetMathLibrary.RandomFloatInRange` 0.0 2.0) (`KismetMathLibrary.RandomFloatInRange` 0.0 2.0) (`KismetMathLibrary.RandomFloatInRange` 0.0 360.0)) false false)
  (`SceneComponent.SetRelativeScale3D` (`self.Liquid_05`) (`KismetMathLibrary.MakeVector` 1.0 1.0 (`KismetMathLibrary.RandomFloatInRange` 0.110981 1.692634)))
  (`SceneComponent.SetVisibility` (`self.Vial_05`) (`KismetMathLibrary.RandomBool`) true)
  (`SceneComponent.SetVisibility` (`self.Lid_05`) (`KismetMathLibrary.RandomBool`) true)
  (`SceneComponent.SetVisibility` (`self.Tag_05`) (`KismetMathLibrary.RandomBool`) true)
  (`SceneComponent.SetVisibility` (`self.Liquid_05`) (`KismetMathLibrary.RandomBool`) true)
  (`SceneComponent.SetVisibility` (`self.Liquid_06`) (`KismetMathLibrary.RandomBool`) false)
  (`PrimitiveComponent.SetTranslucentSortPriority` (`self.Vial_06`) 1)
  (bind _returnvalue_16 (`PrimitiveComponent.CreateDynamicMaterialInstance` (`self.Liquid_06`) 0 "/Game/_Props/OldAlchemist/Materials/Meshspecific/MI_Glassware_Liquid_001.MI_Glassware_Liquid_001" "None"))
  (`MaterialInstanceDynamic.SetScalarParameterValue` _returnvalue_16 "Bubbling_Intensity" (`self.Liquid Bubbling Amount`))
  (`MaterialInstanceDynamic.SetScalarParameterValue` _returnvalue_16 "Bubbling_MAX" (`self.Bubbling MAX`))
  (`MaterialInstanceDynamic.SetScalarParameterValue` _returnvalue_16 "Bubbling_MIN" (`self.Bubbling MIN`))
  (`MaterialInstanceDynamic.SetVectorParameterValue` _returnvalue_16 "Color_Top" (`KismetMathLibrary.Conv_VectorToLinearColor` (`KismetMathLibrary.MakeVector` (`KismetMathLibrary.RandomFloatInRange` 0.0 1.0) (`KismetMathLibrary.RandomFloatInRange` 0.0 1.0) (`KismetMathLibrary.RandomFloatInRange` 0.0 1.0))))
  (`MaterialInstanceDynamic.SetVectorParameterValue` _returnvalue_16 "Color_Bottom" (`self.Liquid Color Bottom`))
  (`MaterialInstanceDynamic.SetScalarParameterValue` _returnvalue_16 "Opacity Top" (`self.Liquid Opacity Top`))
  (`MaterialInstanceDynamic.SetScalarParameterValue` _returnvalue_16 "Opacity Bottom" (`self.Liquid Opacity Bottom`))
  (`SceneComponent.SetVisibility` (`self.Lid_06`) (`KismetMathLibrary.RandomBool`) false)
  (bind _returnvalue_17 (`PrimitiveComponent.CreateDynamicMaterialInstance` (`self.Vial_06`) 0 "/Game/_Props/OldAlchemist/Materials/Meshspecific/MI_Glassware_007.MI_Glassware_007" "None"))
  (`MaterialInstanceDynamic.SetVectorParameterValue` _returnvalue_17 "Color Multiplier" (`self.Glass Color Multiplier`))
  (`MaterialInstanceDynamic.SetScalarParameterValue` _returnvalue_17 "Hue shift percentage" (`self.Glass Hue Shift`))
  (bind _returnvalue_18 (`PrimitiveComponent.CreateDynamicMaterialInstance` _tag_06 0 "/Game/_Props/OldAlchemist/Materials/Meshspecific/MI_Tags_001.MI_Tags_001" "None"))
  (`MaterialInstanceDynamic.SetScalarParameterValue` _returnvalue_18 "Flip between signs" (`KismetMathLibrary.RandomFloatInRange` 0.0 1.0))
  (`SceneComponent.SetVisibility` _tag_06 (`KismetMathLibrary.RandomBool`) false)
  (`SceneComponent.SetRelativeScale3D` (`self.Liquid_06`) (`KismetMathLibrary.MakeVector` 1.0 1.0 (`self.Liquid Amount`)))
  (`SceneComponent.K2_SetRelativeLocation` (`self.Tag_06`) (`KismetMathLibrary.MakeVector` 0.025693 0.023674 (`KismetMathLibrary.RandomFloatInRange` 2.442998 10.559464)) false false)
  (`SceneComponent.K2_SetRelativeRotation` (`self.Vial_06`) (`KismetMathLibrary.MakeRotator` (`KismetMathLibrary.RandomFloatInRange` 0.0 2.0) (`KismetMathLibrary.RandomFloatInRange` 0.0 2.0) (`KismetMathLibrary.RandomFloatInRange` 0.0 360.0)) false false)
  (`SceneComponent.SetRelativeScale3D` (`self.Liquid_06`) (`KismetMathLibrary.MakeVector` 1.0 1.0 (`KismetMathLibrary.RandomFloatInRange` 0.110981 1.692634)))
  (`SceneComponent.SetVisibility` (`self.Vial_06`) (`KismetMathLibrary.RandomBool`) true)
  (`SceneComponent.SetVisibility` (`self.Lid_06`) (`KismetMathLibrary.RandomBool`) true)
  (`SceneComponent.SetVisibility` (`self.Liquid_06`) (`KismetMathLibrary.RandomBool`) true)
  (`SceneComponent.SetVisibility` (`self.Tag_06`) (`KismetMathLibrary.RandomBool`) true))