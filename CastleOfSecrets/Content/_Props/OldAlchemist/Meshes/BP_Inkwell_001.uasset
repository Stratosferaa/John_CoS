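; Inkwell prop Blueprint from the OldAlchemist set with configurable ink level, lid and quill feather, all applied in the construction script.
; A dynamic material instance on the well receives InkAmount as its liquid fill parameter.
; Lid toggles the lid mesh's visibility, while Feather overrides it by reusing that component to show a repositioned feather mesh.
; The event graph has no active logic.
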(fn `UserConstructionScript`
  (bind _sm_jar_lid_001 (`self.SM_Jar_Lid_001`))
  (bind _sm_jar_lid_001_2 (`self.SM_Jar_Lid_001`))
  (bind _returnvalue (`PrimitiveComponent.CreateDynamicMaterialInstance` (`self.well`) 0 "/Game/_Props/OldAlchemist/Materials/Meshspecific/MI_Inkwell_001.MI_Inkwell_001" "None"))
  (`MaterialInstanceDynamic.SetScalarParameterValue` _returnvalue "Liquid amount 0=empty 1=full" (`self.Ink Amount`))
  (if (`self.Lid`)
    (`SceneComponent.SetVisibility` _sm_jar_lid_001_2 true false)
    (else
      (`SceneComponent.SetVisibility` _sm_jar_lid_001_2 false false)))
  (if (`self.Feather`)
    (`SceneComponent.SetVisibility` (`self.SM_Jar_Lid_001`) true false)
    (`StaticMeshComponent.SetStaticMesh` _sm_jar_lid_001 "/Game/_Props/OldAlchemist/Meshes/Mesh_Components/SM_Feather_001.SM_Feather_001")
    (`SceneComponent.K2_SetRelativeTransform` _sm_jar_lid_001 (`KismetMathLibrary.MakeTransform` (0.114851 0.872192 6.551649) (struct :`Pitch` 32.216995 :`Yaw` 82.499947 :`Roll` -2.405853) (1.0 1.0 1.0)) false false)))