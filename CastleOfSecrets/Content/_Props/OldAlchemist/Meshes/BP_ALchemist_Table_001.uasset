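; Alchemist table prop with nine drawer meshes that can be posed per instance in the editor.
; The construction script slides each drawer along its local X axis, lerping a fixed offset by that drawer's MoveDrawer value.
; Each RemoveDrawer flag feeds its drawer's visibility directly, so true shows the drawer despite the name.
; It has no runtime logic, as the event graph holds only disabled stub events.
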(fn `UserConstructionScript`
  (bind _sm_alchimist_table_002 (`self.SM_Alchimist_Table_002`))
  (bind _sm_alchimist_table_003 (`self.SM_Alchimist_Table_003`))
  (bind _sm_alchimist_table_004 (`self.SM_Alchimist_Table_004`))
  (bind _sm_alchimist_table_005 (`self.SM_Alchimist_Table_005`))
  (bind _sm_alchimist_table_006 (`self.SM_Alchimist_Table_006`))
  (bind _sm_alchimist_table_007 (`self.SM_Alchimist_Table_007`))
  (bind _sm_alchimist_table_008 (`self.SM_Alchimist_Table_008`))
  (bind _sm_alchimist_table_009 (`self.SM_Alchimist_Table_009`))
  (bind _sm_alchimist_table_010 (`self.SM_Alchimist_Table_010`))
  (`SceneComponent.K2_AddLocalOffset` _sm_alchimist_table_002 (`KismetMathLibrary.VLerp` (0.0 0.0 0.0) (-33.334686 0.0 0.0) (`self.Move Drawer N°1`)) false false)
  (`SceneComponent.SetVisibility` _sm_alchimist_table_002 (`self.Remove Drawer N°1`) false)
  (`SceneComponent.K2_AddLocalOffset` _sm_alchimist_table_003 (`KismetMathLibrary.VLerp` (0.0 0.0 0.0) (-33.334686 0.0 0.0) (`self.Move Drawer N°2`)) false false)
  (`SceneComponent.SetVisibility` _sm_alchimist_table_003 (`self.Remove Drawer N°2`) false)
  (`SceneComponent.K2_AddLocalOffset` _sm_alchimist_table_004 (`KismetMathLibrary.VLerp` (0.0 0.0 0.0) (-33.334686 0.0 0.0) (`self.Move Drawer N°3`)) false false)
  (`SceneComponent.SetVisibility` _sm_alchimist_table_004 (`self.Remove Drawer N°3`) false)
  (`SceneComponent.K2_AddLocalOffset` _sm_alchimist_table_005 (`KismetMathLibrary.VLerp` (0.0 0.0 0.0) (-33.334686 0.0 0.0) (`self.Move Drawer N°4`)) false false)
  (`SceneComponent.SetVisibility` _sm_alchimist_table_005 (`self.Remove Drawer N°4`) false)
  (`SceneComponent.K2_AddLocalOffset` _sm_alchimist_table_006 (`KismetMathLibrary.VLerp` (0.0 0.0 0.0) (-33.334686 0.0 0.0) (`self.Move Drawer N°5`)) false false)
  (`SceneComponent.SetVisibility` _sm_alchimist_table_006 (`self.Remove Drawer N°5`) false)
  (`SceneComponent.K2_AddLocalOffset` _sm_alchimist_table_007 (`KismetMathLibrary.VLerp` (0.0 0.0 0.0) (-33.334686 0.0 0.0) (`self.Move Drawer N°6`)) false false)
  (`SceneComponent.SetVisibility` _sm_alchimist_table_007 (`self.Remove Drawer N°6`) false)
  (`SceneComponent.K2_AddLocalOffset` _sm_alchimist_table_008 (`KismetMathLibrary.VLerp` (0.0 0.0 0.0) (-33.334686 0.0 0.0) (`self.Move Drawer N°7`)) false false)
  (`SceneComponent.SetVisibility` _sm_alchimist_table_008 (`self.Remove Drawer N°7`) false)
  (`SceneComponent.K2_AddLocalOffset` _sm_alchimist_table_009 (`KismetMathLibrary.VLerp` (0.0 0.0 0.0) (-33.334686 0.0 0.0) (`self.Move Drawer N°8`)) false false)
  (`SceneComponent.SetVisibility` _sm_alchimist_table_009 (`self.Remove Drawer N°8`) false)
  (`SceneComponent.K2_AddLocalOffset` _sm_alchimist_table_010 (`KismetMathLibrary.VLerp` (0.0 0.0 0.0) (-33.334686 0.0 0.0) (`self.Move Drawer N°9`)) false false)
  (`SceneComponent.SetVisibility` _sm_alchimist_table_010 (`self.Remove Drawer N°9`) false))