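; BP_Bottle_004 is a configurable alchemist bottle prop with optional liquid, cork lid and tag, set up entirely in the construction script.
; Exposed variables toggle part visibility and drive dynamic material instances for liquid bubbling, colors and opacity, plus glass tint and hue shift.
; The tag material gets row and column counts and a random sign-flip value, re-rolled on each construction; the glass mesh gets a raised translucent sort priority.
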(fn `UserConstructionScript`
  (bind _liquid (`self.liquid`))
  (if (`self.Add Liquid`)
    (`SceneComponent.SetVisibility` _liquid true false)
    (else
      (`SceneComponent.SetVisibility` _liquid false false)))
  (`PrimitiveComponent.SetTranslucentSortPriority` (`self.test`) 1)
  (bind _returnvalue (`PrimitiveComponent.CreateDynamicMaterialInstance` (`self.liquid`) 0 "/Game/_Props/OldAlchemist/Materials/Meshspecific/MI_Glassware_Liquid_001.MI_Glassware_Liquid_001" "None"))
  (`MaterialInstanceDynamic.SetScalarParameterValue` _returnvalue "Bubbling_Intensity" (`self.Liquid Bubbling Amount`))
  (`MaterialInstanceDynamic.SetScalarParameterValue` _returnvalue "Bubbling_MAX" (`self.Bubbling MAX`))
  (`MaterialInstanceDynamic.SetScalarParameterValue` _returnvalue "Bubbling_MIN" (`self.Bubbling MIN`))
  (`MaterialInstanceDynamic.SetVectorParameterValue` _returnvalue "Color_Top" (`self.Liquid Color Top`))
  (`MaterialInstanceDynamic.SetVectorParameterValue` _returnvalue "Color_Bottom" (`self.Liquid Color Bottom`))
  (`MaterialInstanceDynamic.SetScalarParameterValue` _returnvalue "Opacity Top" (`self.Liquid Opacity Top`))
  (`MaterialInstanceDynamic.SetScalarParameterValue` _returnvalue "Opacity Bottom" (`self.Liquid Opacity Bottom`))
  (`SceneComponent.SetVisibility` (`self.SM_Jar_Lid_001`) (`self.Cork`) false)
  (bind _returnvalue_2 (`PrimitiveComponent.CreateDynamicMaterialInstance` (`self.test`) 0 "/Game/_Props/OldAlchemist/Materials/Meshspecific/MI_Glassware_004.MI_Glassware_004" "None"))
  (`MaterialInstanceDynamic.SetVectorParameterValue` _returnvalue_2 "Color Multiplier" (`self.Glass Color Multiplier`))
  (`MaterialInstanceDynamic.SetScalarParameterValue` _returnvalue_2 "Hue shift percentage" (`self.Glass Hue Shift`))
  (bind _returnvalue_3 (`PrimitiveComponent.CreateDynamicMaterialInstance` (`self.t1`) 1 "/Game/_Props/OldAlchemist/Materials/Meshspecific/MI_Tags_001.MI_Tags_001" "None"))
  (`MaterialInstanceDynamic.SetScalarParameterValue` _returnvalue_3 "Flip between signs" (`KismetMathLibrary.RandomFloatInRange` 0.0 1.0))
  (`MaterialInstanceDynamic.SetScalarParameterValue` _returnvalue_3 "Number of Rows" (`self.Rows`))
  (`MaterialInstanceDynamic.SetScalarParameterValue` _returnvalue_3 "Number of columns" (`self.Culumns`))
  (`SceneComponent.SetVisibility` (`self.t1`) (`self.Tag`) false))