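; Configurable book prop with left and right text pages, built entirely in the Construction Script.
; A dynamic material instance on the book mesh applies cover colors, hue shifts and surface settings, plus selectable decorations, decoration metal and cover style texture sets.
; Left and right page options swap the text page meshes, whose own dynamic materials receive a shared text color multiplier.
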(fn `UserConstructionScript`
  (bind _sm_book_text_page_001_001 (`self.SM_Book_Text_Page_001_001`))
  (bind _sm_book_text_page_002_001 (`self.SM_Book_Text_Page_002_001`))
  (bind _returnvalue (`PrimitiveComponent.CreateDynamicMaterialInstance` (`self.SM_book_001`) 0 "/Game/_Props/OldAlchemist/Materials/Meshspecific/MI_Books_001.MI_Books_001" "None"))
  (`MaterialInstanceDynamic.SetVectorParameterValue` _returnvalue "Cover center color add" (`self.Center Add Color`))
  (`MaterialInstanceDynamic.SetVectorParameterValue` _returnvalue "Cover center color multiplier" (`self.Center Multiply Color`))
  (`MaterialInstanceDynamic.SetScalarParameterValue` _returnvalue "Cover Center Hue Shift" (`self.Center Hue Shift`))
  (`MaterialInstanceDynamic.SetVectorParameterValue` _returnvalue "Cover sides color add" (`self.Sides Add Color`))
  (`MaterialInstanceDynamic.SetVectorParameterValue` _returnvalue "Cover sides color multiplier" (`self.Sides Multiply Color`))
  (`MaterialInstanceDynamic.SetScalarParameterValue` _returnvalue "Cover Sides Hue Shift" (`self.Sides Hue Shift`))
  (`MaterialInstanceDynamic.SetScalarParameterValue` _returnvalue "Normal Intensity" (`self.Normal Intensity`))
  (switch `int` (`self.Pick Book Decorations`)
    (:`0`
      (`MaterialInstanceDynamic.SetScalarParameterValue` _returnvalue "Activate Decorations" 0.0))
    (:`1`
      _)
    (:`2`
      (`MaterialInstanceDynamic.SetScalarParameterValue` _returnvalue "Decorations Switch" 1.0)
      (`MaterialInstanceDynamic.SetTextureParameterValue` _returnvalue "Decorations_Normal" "/Game/_Props/OldAlchemist/Textures/T_Books_Details_002_N.T_Books_Details_002_N"))
    (:`3`
      (`MaterialInstanceDynamic.SetScalarParameterValue` _returnvalue "Decorations Switch" 2.0)
      (`MaterialInstanceDynamic.SetTextureParameterValue` _returnvalue "Decorations_Normal" "/Game/_Props/OldAlchemist/Textures/T_Books_Details_003_N.T_Books_Details_003_N")))
  (`MaterialInstanceDynamic.SetScalarParameterValue` _returnvalue "Roughness Multiplier" (`self.Roughness Multiplier`))
  (`MaterialInstanceDynamic.SetScalarParameterValue` _returnvalue "Specular" (`self.Specular`))
  (switch `/Game/_Props/OldAlchemist/Meshes/Enumerators/ENUM_Books_002` (`self.Pick Decoration Metal`)
    (:`NewEnumerator1`
      (`MaterialInstanceDynamic.SetVectorParameterValue` _returnvalue "Detail_Color" (struct :`R` 0.65 :`G` 0.65 :`B` 0.65 :`A` 1.0)))
    (:`NewEnumerator2`
      _)
    (:`NewEnumerator3`
      (`MaterialInstanceDynamic.SetVectorParameterValue` _returnvalue "Detail_Color" (struct :`R` 0.415 :`G` 0.254697 :`B` 0.127331 :`A` 1.0)))
    (:`NewEnumerator4`
      (`MaterialInstanceDynamic.SetVectorParameterValue` _returnvalue "Detail_Color" (struct :`R` 0.25 :`G` 0.25 :`B` 0.25 :`A` 1.0))))
  (switch `/Game/_Props/OldAlchemist/Meshes/Enumerators/ENUM_Books_001` (`self.Pick Book Style`)
    (:`NewEnumerator0`
      (`MaterialInstanceDynamic.SetTextureParameterValue` _returnvalue "Color" "/Game/_Props/OldAlchemist/Textures/T_Books_002_C.T_Books_002_C")
      (`MaterialInstanceDynamic.SetTextureParameterValue` _returnvalue "Normal" "/Game/_Props/OldAlchemist/Textures/T_Books_002_N.T_Books_002_N")
      (`MaterialInstanceDynamic.SetTextureParameterValue` _returnvalue "R=Roughness G=Metallic B=AO" "/Game/_Props/OldAlchemist/Textures/T_Books_002_S.T_Books_002_S"))
    (:`NewEnumerator2`
      (`MaterialInstanceDynamic.SetTextureParameterValue` _returnvalue "Color" "/Game/_Props/OldAlchemist/Textures/T_Books_003_C.T_Books_003_C")
      (`MaterialInstanceDynamic.SetTextureParameterValue` _returnvalue "Normal" "/Game/_Props/OldAlchemist/Textures/T_Books_003_N.T_Books_003_N")
      (`MaterialInstanceDynamic.SetTextureParameterValue` _returnvalue "R=Roughness G=Metallic B=AO" "/Game/_Props/OldAlchemist/Textures/T_Books_003_S.T_Books_003_S")
      (`MaterialInstanceDynamic.SetTextureParameterValue` _returnvalue "Mask" "/Game/_Props/OldAlchemist/Textures/T_Books_003_S2.T_Books_003_S2"))
    (:`NewEnumerator3`
      (`MaterialInstanceDynamic.SetTextureParameterValue` _returnvalue "Color" "/Game/_Props/OldAlchemist/Textures/T_Books_004_C.T_Books_004_C")
      (`MaterialInstanceDynamic.SetTextureParameterValue` _returnvalue "Normal" "/Game/_Props/OldAlchemist/Textures/T_Books_004_N.T_Books_004_N")
      (`MaterialInstanceDynamic.SetTextureParameterValue` _returnvalue "R=Roughness G=Metallic B=AO" "/Game/_Props/OldAlchemist/Textures/T_Books_004_S.T_Books_004_S")))
  (switch `int` (`self.Left Page`)
    (:`1`
      _)
    (:`2`
      (`StaticMeshComponent.SetStaticMesh` _sm_book_text_page_001_001 "/Game/_Props/OldAlchemist/Meshes/Mesh_Components/SM_Book_Text_Page_003_002.SM_Book_Text_Page_003_002"))
    (:`3`
      (`StaticMeshComponent.SetStaticMesh` _sm_book_text_page_001_001 "/Game/_Props/OldAlchemist/Meshes/Mesh_Components/SM_Book_Text_Page_003_003.SM_Book_Text_Page_003_003"))
    (:`4`
      (`StaticMeshComponent.SetStaticMesh` _sm_book_text_page_001_001 "/Game/_Props/OldAlchemist/Meshes/Mesh_Components/SM_Book_Text_Page_003_004.SM_Book_Text_Page_003_004")))
  (switch `int` (`self.Right Page`)
    (:`2`
      (`StaticMeshComponent.SetStaticMesh` _sm_book_text_page_002_001 "/Game/_Props/OldAlchemist/Meshes/Mesh_Components/SM_Book_Text_Page_004_002.SM_Book_Text_Page_004_002"))
    (:`3`
      (`StaticMeshComponent.SetStaticMesh` _sm_book_text_page_002_001 "/Game/_Props/OldAlchemist/Meshes/Mesh_Components/SM_Book_Text_Page_004_003.SM_Book_Text_Page_004_003"))
    (:`4`
      (`StaticMeshComponent.SetStaticMesh` _sm_book_text_page_002_001 "/Game/_Props/OldAlchemist/Meshes/Mesh_Components/SM_Book_Text_Page_004_004.SM_Book_Text_Page_004_004")))
  (bind _returnvalue_2 (`PrimitiveComponent.CreateDynamicMaterialInstance` _sm_book_text_page_002_001 0 "/Game/_Props/OldAlchemist/Materials/Meshspecific/MI_Book_Text_001.MI_Book_Text_001" "None"))
  (bind _returnvalue_3 (`PrimitiveComponent.CreateDynamicMaterialInstance` _sm_book_text_page_001_001 0 "/Game/_Props/OldAlchemist/Materials/Meshspecific/MI_Book_Text_001.MI_Book_Text_001" "None"))
  (`MaterialInstanceDynamic.SetVectorParameterValue` _returnvalue_3 "Color multyplier" (`self.Text Color Multiplier`))
  (`MaterialInstanceDynamic.SetVectorParameterValue` _returnvalue_2 "Color multyplier" (`self.Text Color Multiplier`)))