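; Alchemist athanor prop with fire, embers, a drip, a tag and a glass container of bubbling liquid.
; The construction script drives dynamic materials and visibility from variables, randomizing the tag sign.
; TurnONOFF toggles effects and lights, overriding the Drip setting, and stops bubbling when off.
; At runtime, a timeline moves the point light while Tick, throttled by a short Delay, randomizes its color for flicker.
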(event `self.ReceiveBeginPlay`
  (bind (_direction _light_movement) (`Timeline|Timeline_0`)
    (:`Update`
      (`SceneComponent.K2_SetRelativeLocation` (`self.PointLight`) (+ (`KismetMathLibrary.MakeVector` 0.0 0.0 30.604214) (* _light_movement 0.5)) false false))))

(event `self.ReceiveTick`
  (params (DeltaSeconds :type "Float (single-precision)"))
  (bind _returnvalue (`KismetMathLibrary.RandomFloatInRange` 0.8 1.0))
  (`KismetSystemLibrary.Delay` 0.01)
  (`LightComponent.SetLightColor` (`self.PointLight`) (`KismetMathLibrary.Conv_VectorToLinearColor` (`KismetMathLibrary.MakeVector` (* (`KismetMathLibrary.RandomFloatInRange` 1.0 1.0) _returnvalue) (* (`KismetMathLibrary.RandomFloatInRange` 0.4 0.7) _returnvalue) (* (`KismetMathLibrary.RandomFloatInRange` 0.6 0.7) _returnvalue))) true))

(fn `UserConstructionScript`
  (bind _staticmesh1 (`self.StaticMesh1`))
  (bind _turn_on_off (`self.Turn ON/OFF`))
  (`SceneComponent.SetVisibility` (`self.P_Drip_001`) (`self.Drip`) false)
  (bind _returnvalue (`PrimitiveComponent.CreateDynamicMaterialInstance` (`self.StaticMesh`) 0 "/Game/_Props/OldAlchemist/Materials/Meshspecific/MI_Glassware_Liquid_001.MI_Glassware_Liquid_001" "None"))
  (`MaterialInstanceDynamic.SetScalarParameterValue` _returnvalue "Bubbling_Intensity" (`self.Liquid Bubbling Amount`))
  (`MaterialInstanceDynamic.SetScalarParameterValue` _returnvalue "Bubbling_MAX" (`self.Bubbling MAX`))
  (`MaterialInstanceDynamic.SetScalarParameterValue` _returnvalue "Bubbling_MIN" (`self.Bubbling MIN`))
  (`MaterialInstanceDynamic.SetVectorParameterValue` _returnvalue "Color_Top" (`self.Liquid Color Top`))
  (`MaterialInstanceDynamic.SetVectorParameterValue` _returnvalue "Color_Bottom" (`self.Liquid Color Bottom`))
  (`MaterialInstanceDynamic.SetScalarParameterValue` _returnvalue "Opacity Top" (`self.Liquid Opacity Top`))
  (`MaterialInstanceDynamic.SetScalarParameterValue` _returnvalue "Opacity Bottom" (`self.Liquid Opacity Bottom`))
  (bind _returnvalue_2 (`PrimitiveComponent.CreateDynamicMaterialInstance` (`self.SM_Bottle_005`) 0 "/Game/_Props/OldAlchemist/Materials/Meshspecific/MI_Glassware_008.MI_Glassware_008" "None"))
  (`MaterialInstanceDynamic.SetVectorParameterValue` _returnvalue_2 "Color Multiplier" (`self.Glass Color Multiplier`))
  (`MaterialInstanceDynamic.SetScalarParameterValue` _returnvalue_2 "Hue shift percentage" (`self.Glass Hue Shift`))
  (bind _returnvalue_3 (`PrimitiveComponent.CreateDynamicMaterialInstance` _staticmesh1 0 "/Game/_Props/OldAlchemist/Materials/Meshspecific/MI_Tags_001.MI_Tags_001" "None"))
  (`MaterialInstanceDynamic.SetScalarParameterValue` _returnvalue_3 "Flip between signs" (`KismetMathLibrary.RandomFloatInRange` 0.0 1.0))
  (`SceneComponent.SetVisibility` _staticmesh1 (`self.Tag`) false)
  (`SceneComponent.SetVisibility` (`self.SM_Bottle_005`) (`self.Container`) false)
  (`SceneComponent.SetVisibility` (`self.StaticMesh`) (`self.Container`) false)
  (`SceneComponent.SetVisibility` (`self.P_Athanor_Fire_001`) _turn_on_off false)
  (`SceneComponent.SetVisibility` (`self.PointLight`) _turn_on_off false)
  (`SceneComponent.SetVisibility` (`self.PointLight1`) _turn_on_off false)
  (`SceneComponent.SetVisibility` (`self.P_Drip_001`) _turn_on_off false)
  (`SceneComponent.SetVisibility` (`self.P_Athanor_Embers_001`) _turn_on_off false)
  (if (not _turn_on_off)
    (`MaterialInstanceDynamic.SetScalarParameterValue` _returnvalue "Bubbling_Intensity" 0.0)))