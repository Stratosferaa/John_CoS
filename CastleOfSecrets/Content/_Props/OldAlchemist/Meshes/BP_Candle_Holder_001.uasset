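; Candle holder prop with a configurable candle, flame effect and flickering light.
; The construction script picks one of five wax colours and one of three candle variants, with options for lit state, shadow casting and hiding the candle or holder.
; At BeginPlay a timeline starts from a random position and drives the intensity of all three lights, so flicker varies between instances.
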(event `self.ReceiveBeginPlay`
  (`TimelineComponent.SetPlaybackPosition` (`self.Timeline_0`) (`KismetMathLibrary.RandomFloatInRange` 0.0 5.0) false true)
  (bind (_direction _light_intensity) (`Timeline|Timeline_0`)
    (:`Update`
      (`LightComponent.SetIntensity` (`self.Light_003`) _light_intensity)
      (`LightComponent.SetIntensity` (`self.Light_001`) _light_intensity)
      (`LightComponent.SetIntensity` (`self.Light_002`) _light_intensity))))

(fn `UserConstructionScript`
  (bind _light_003 (`self.Light_003`))
  (bind _light_001 (`self.Light_001`))
  (bind _light_002 (`self.Light_002`))
  (switch `/Game/_Props/OldAlchemist/Meshes/Enumerators/ENUM_Candle_Material_001` (`self.Choose Wax Color`)
    (:`NewEnumerator0`
      (`PrimitiveComponent.SetMaterial` (`self.candle_001`) 0 "/Game/_Props/OldAlchemist/Materials/Meshspecific/MI_Candle_001.MI_Candle_001")
      (`PrimitiveComponent.SetMaterial` (`self.candle_002`) 0 "/Game/_Props/OldAlchemist/Materials/Meshspecific/MI_Candle_001.MI_Candle_001")
      (`PrimitiveComponent.SetMaterial` (`self.candle_003`) 0 "/Game/_Props/OldAlchemist/Materials/Meshspecific/MI_Candle_001.MI_Candle_001"))
    (:`NewEnumerator1`
      (`PrimitiveComponent.SetMaterial` (`self.candle_001`) 0 "/Game/_Props/OldAlchemist/Materials/Meshspecific/MI_Candle_002.MI_Candle_002")
      (`PrimitiveComponent.SetMaterial` (`self.candle_002`) 0 "/Game/_Props/OldAlchemist/Materials/Meshspecific/MI_Candle_002.MI_Candle_002")
      (`PrimitiveComponent.SetMaterial` (`self.candle_003`) 0 "/Game/_Props/OldAlchemist/Materials/Meshspecific/MI_Candle_002.MI_Candle_002"))
    (:`NewEnumerator2`
      (`PrimitiveComponent.SetMaterial` (`self.candle_001`) 0 "/Game/_Props/OldAlchemist/Materials/Meshspecific/MI_Candle_003.MI_Candle_003")
      (`PrimitiveComponent.SetMaterial` (`self.candle_002`) 0 "/Game/_Props/OldAlchemist/Materials/Meshspecific/MI_Candle_003.MI_Candle_003")
      (`PrimitiveComponent.SetMaterial` (`self.candle_003`) 0 "/Game/_Props/OldAlchemist/Materials/Meshspecific/MI_Candle_003.MI_Candle_003"))
    (:`NewEnumerator3`
      (`PrimitiveComponent.SetMaterial` (`self.candle_001`) 0 "/Game/_Props/OldAlchemist/Materials/Meshspecific/MI_Candle_004.MI_Candle_004")
      (`PrimitiveComponent.SetMaterial` (`self.candle_002`) 0 "/Game/_Props/OldAlchemist/Materials/Meshspecific/MI_Candle_004.MI_Candle_004")
      (`PrimitiveComponent.SetMaterial` (`self.candle_003`) 0 "/Game/_Props/OldAlchemist/Materials/Meshspecific/MI_Candle_004.MI_Candle_004"))
    (:`NewEnumerator4`
      (`PrimitiveComponent.SetMaterial` (`self.candle_001`) 0 "/Game/_Props/OldAlchemist/Materials/Meshspecific/MI_Candle_005.MI_Candle_005")
      (`PrimitiveComponent.SetMaterial` (`self.candle_002`) 0 "/Game/_Props/OldAlchemist/Materials/Meshspecific/MI_Candle_005.MI_Candle_005")
      (`PrimitiveComponent.SetMaterial` (`self.candle_003`) 0 "/Game/_Props/OldAlchemist/Materials/Meshspecific/MI_Candle_005.MI_Candle_005")))
  (switch `int` (`self.Choose Candle`)
    (:`1`
      (`SceneComponent.SetVisibility` (`self.candle_001`) true false)
      (`SceneComponent.SetVisibility` (`self.P_Candle_Flame_001`) true false)
      (`SceneComponent.SetVisibility` (`self.Light_001`) true false)
      (`SceneComponent.SetVisibility` (`self.candle_003`) false false)
      (`SceneComponent.SetVisibility` (`self.candle_002`) false false)
      (`SceneComponent.SetVisibility` (`self.P_Candle_Flame_002`) false false)
      (`SceneComponent.SetVisibility` (`self.Light_002`) false false)
      (`SceneComponent.SetVisibility` (`self.Light_003`) false false)
      (`SceneComponent.SetVisibility` (`self.P_Candle_Flame_003`) false false)
      (`LightComponentBase.SetCastShadows` _light_001 (`self.Cast Shadows`))
      (`SceneComponent.SetVisibility` _light_001 (`self.ON/OFF`) false)
      (`SceneComponent.SetVisibility` (`self.P_Candle_Flame_001`) (`self.ON/OFF`) false))
    (:`2`
      (`SceneComponent.SetVisibility` (`self.candle_002`) true false)
      (`SceneComponent.SetVisibility` (`self.Light_002`) true false)
      (`SceneComponent.SetVisibility` (`self.P_Candle_Flame_002`) true false)
      (`SceneComponent.SetVisibility` (`self.candle_003`) false false)
      (`SceneComponent.SetVisibility` (`self.candle_001`) false false)
      (`SceneComponent.SetVisibility` (`self.P_Candle_Flame_001`) false false)
      (`SceneComponent.SetVisibility` (`self.Light_001`) false false)
      (`SceneComponent.SetVisibility` (`self.P_Candle_Flame_003`) false false)
      (`SceneComponent.SetVisibility` (`self.Light_003`) false false)
      (`LightComponentBase.SetCastShadows` _light_002 (`self.Cast Shadows`))
      (`SceneComponent.SetVisibility` _light_002 (`self.ON/OFF`) false)
      (`SceneComponent.SetVisibility` (`self.P_Candle_Flame_002`) (`self.ON/OFF`) false))
    (:`3`
      (`SceneComponent.SetVisibility` (`self.candle_003`) true false)
      (`SceneComponent.SetVisibility` (`self.P_Candle_Flame_003`) true false)
      (`SceneComponent.SetVisibility` (`self.Light_003`) true false)
      (`SceneComponent.SetVisibility` (`self.candle_002`) false false)
      (`SceneComponent.SetVisibility` (`self.candle_001`) false false)
      (`SceneComponent.SetVisibility` (`self.P_Candle_Flame_001`) false false)
      (`SceneComponent.SetVisibility` (`self.Light_001`) false false)
      (`SceneComponent.SetVisibility` (`self.Light_002`) false false)
      (`SceneComponent.SetVisibility` (`self.P_Candle_Flame_002`) false false)
      (`LightComponentBase.SetCastShadows` _light_003 (`self.Cast Shadows`))
      (`SceneComponent.SetVisibility` _light_003 (`self.ON/OFF`) false)
      (`SceneComponent.SetVisibility` (`self.P_Candle_Flame_003`) (`self.ON/OFF`) false)))
  (if (`self.Remove Candle`)
    (`SceneComponent.SetVisibility` (`self.candle_003`) false false)
    (`SceneComponent.SetVisibility` (`self.candle_001`) false false)
    (`SceneComponent.SetVisibility` (`self.candle_002`) false false)
    (`SceneComponent.SetVisibility` (`self.Light_001`) false false)
    (`SceneComponent.SetVisibility` (`self.P_Candle_Flame_002`) false false)
    (`SceneComponent.SetVisibility` (`self.P_Candle_Flame_003`) false false)
    (`SceneComponent.SetVisibility` (`self.Light_002`) false false)
    (`SceneComponent.SetVisibility` (`self.Light_003`) false false)
    (`SceneComponent.SetVisibility` (`self.P_Candle_Flame_001`) false false)
    (set `self.ON/OFF` false))
  (if (`self.Remove Holder`)
    (`SceneComponent.SetVisibility` (`self.SM_Candleholder_001`) false false)))