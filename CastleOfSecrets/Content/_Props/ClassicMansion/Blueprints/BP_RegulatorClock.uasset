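; BP_RegulatorClock is a mansion prop clock with moving hands, a swinging pendulum, ticking and a chime.
; When IsWorking is set, BeginPlay poses the hands from Hour and Minute, then plays the 1Second timeline.
; The timeline's track lerps the pendulum swing, while its event advances both hands by one second's rotation and plays a tick.
; That event also rings the bell when the minute hand's roll is nearly zero, avoiding Tick entirely.
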(event `self.ReceiveBeginPlay`
  (bind _sm_clockhourhand (`self.SM_ClockHourHand`))
  (bind _sm_clockminutehand (`self.SM_ClockMinuteHand`))
  (bind _minute (`self.Minute`))
  (bind _sm_clockpendulum (`self.SM_ClockPendulum`))
  (bind _returnvalue (`SceneComponent.K2_GetComponentLocation` _sm_clockpendulum))
  (bind _relativerotation_roll (`KismetMathLibrary.BreakRotator` (`SceneComponent.RelativeRotation` _sm_clockminutehand)))
  (if (`self.IsWorking`)
    (`SceneComponent.K2_SetRelativeRotation` _sm_clockhourhand (`KismetMathLibrary.MakeRotator` (* (`self.Hour`) -30.0)) false false)
    (`SceneComponent.K2_AddRelativeRotation` _sm_clockhourhand (`KismetMathLibrary.MakeRotator` (* _minute -0.5)) false false)
    (`SceneComponent.K2_SetRelativeRotation` _sm_clockminutehand (`KismetMathLibrary.MakeRotator` (* _minute -6.0)) false false)
    (bind (_direction _newtrack_0) (`Timeline|1Second`)
      (:`Update`
        (`SceneComponent.K2_SetRelativeRotation` _sm_clockpendulum (`KismetMathLibrary.RLerp` (struct :`Roll` 3.0) (struct :`Roll` -3.0) _newtrack_0 true) false false))
      (:`NewTrack_1`
        (`SceneComponent.K2_AddRelativeRotation` _sm_clockhourhand (`KismetMathLibrary.MakeRotator` -0.008333) false false)
        (`SceneComponent.K2_AddRelativeRotation` _sm_clockminutehand (`KismetMathLibrary.MakeRotator` -0.1) false false)
        (`GameplayStatics.PlaySoundAtLocation` "/Game/_Props/ClassicMansion/Audio/Cues/SC_ClockTick.SC_ClockTick" _returnvalue (struct) 0.2 1.0 0.0 null null null)
        (if (`KismetMathLibrary.NearlyEqual_FloatFloat` _relativerotation_roll 0.0 0.001)
          (`GameplayStatics.PlaySoundAtLocation` "/Game/_Props/ClassicMansion/Audio/Cues/SC_ClockBell.SC_ClockBell" _returnvalue (struct) 1.0 1.0 0.0 null null null))))))

(fn `UserConstructionScript`)