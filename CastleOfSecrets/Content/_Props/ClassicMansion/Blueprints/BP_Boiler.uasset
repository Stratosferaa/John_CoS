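; Boiler prop for the Classic Mansion set, with an optional active state that adds particles, sound and an animated light.
; When IsActive is set, the construction script adds particle, audio and point light components at a shared offset and stores the light in Light.
; BeginPlay starts two timelines, without checking IsActive, that drive the light's intensity and its relative X/Z position.
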(event `self.ReceiveBeginPlay`
  (bind _light (`self.Light`))
  (`|ExecutionSequence`
    (:`then_0`
      (bind (_direction _newtrack_0) (`Timeline|Timeline_0`)
        (:`Update`
          (`LightComponent.SetIntensity` _light _newtrack_0))))
    (:`then_1`
      (bind (_direction_2 _newtrack_1) (`Timeline|Timeline_1`)
        (:`Update`
          (`SceneComponent.K2_SetRelativeLocation` _light (`KismetMathLibrary.MakeVector` _newtrack_1 0.0 _newtrack_1) false false))))))

(fn `UserConstructionScript`
  (bind _returnvalue (`KismetMathLibrary.MakeTransform` (12.0 0.0 20.0)))
  (if (`self.IsActive`)
    (`AddComponent|NODE_AddParticleSystemComponent-0` :`RelativeTransform` _returnvalue)
    (`AddComponent|NODE_AddAudioComponent-0` :`RelativeTransform` _returnvalue)
    (bind _returnvalue_2 (`AddComponent|NODE_AddPointLightComponent-0` :`RelativeTransform` (`KismetMathLibrary.MakeTransform` (12.0 0.0 20.0))))
    (set `self.Light` _returnvalue_2)))