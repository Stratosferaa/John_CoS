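; Trigger volume actor that switches a Character's animation state while it stands inside its Box.
; On begin overlap it casts the overlapping actor to Character and writes the Begin values for CustomAnimW, CustomAnimI and IsJump.
; On end overlap it writes the matching End values, so each placed instance can define its own pair of animation overrides.
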(event `self.Box.OnComponentBeginOverlap`
  (params (OverlappedComponent :type "PrimitiveComponent Object Reference") (OtherActor :type "Actor Object Reference") (OtherComp :type "PrimitiveComponent Object Reference") (OtherBodyIndex :type Integer) (bFromSweep :type Boolean) (SweepResult :type "HitResult Structure (by ref)"))
  (bind _ascharacter (cast `/Game/Main/Character` OtherActor))
  (set `/Game/Main/Character.custom animW` (`self.Begin Custom AnimW`) _ascharacter)
  (set `/Game/Main/Character.custom animI` (`self.Begin Custom AnimI`) _ascharacter)
  (set `/Game/Main/Character.IsJump` (`self.BeginJamp`) _ascharacter))

(event `self.Box.OnComponentEndOverlap`
  (params (OverlappedComponent :type "PrimitiveComponent Object Reference") (OtherActor :type "Actor Object Reference") (OtherComp :type "PrimitiveComponent Object Reference") (OtherBodyIndex :type Integer))
  (bind _ascharacter (cast `/Game/Main/Character` OtherActor))
  (set `/Game/Main/Character.custom animW` (`self.End Custom AnimW`) _ascharacter)
  (set `/Game/Main/Character.custom animI` (`self.End Custom AnimI`) _ascharacter)
  (set `/Game/Main/Character.IsJump` (`self.EndJamp`) _ascharacter))

(fn `UserConstructionScript`)