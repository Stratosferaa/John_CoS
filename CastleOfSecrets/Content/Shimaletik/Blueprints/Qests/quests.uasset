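; Quest manager that tracks completion of configured quests (НастройкаКвестов), each with a type and target items, and shows them in a W_Quest widget.
; On BeginPlay it creates the widget, sizes each quest's per-item completion array and hands every valid item a back-reference to itself.
; Qestupdatestat finds the first quest containing the reported item and, if the type matches, marks progress or full completion and refreshes the widget.
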(event `self.ReceiveBeginPlay`
  (bind `_настройка_квестов` (`self.Настройка квестов`))
  (bind _returnvalue (`|CreateWidget` "/Game/Shimaletik/Blueprints/Qests/W_Quest.W_Quest_C" (`GameplayStatics.GetPlayerController` 0)))
  (set `self.W_Quest` _returnvalue)
  (`/Game/Shimaletik/Blueprints/Qests/W_Quest.Update stat qests` _returnvalue `_настройка_квестов`)
  (`UserWidget.AddToViewport` _returnvalue 1)
  (for (_array_element _array_index) `_настройка_квестов`
    (`KismetArrayLibrary.Array_Clear` (`self.Complited`))
    (bind (`_описаниеквеста` `_типквеста` `_итемы`) (break `/Game/Shimaletik/Blueprints/Qests/str_qest` _array_element))
    (`KismetArrayLibrary.Array_Set` (`self.Complited`) (`KismetArrayLibrary.Array_LastIndex` `_итемы`) false true)
    (`KismetArrayLibrary.Array_Set` `_настройка_квестов` _array_index (make `/Game/Shimaletik/Blueprints/Qests/str_qest` `_описаниеквеста` `_типквеста` `_итемы` (`self.Complited`)))
    (for _array_element_2 `_итемы`
      (`/Engine/EditorBlueprintResources/StandardMacros.IsValid` _array_element_2
        (:`Is Valid`
          (set `/Game/_Props_2/Core/Blueprints/Items/BP_BaseItem.Qests` self _array_element_2)
          (`/Game/_Props_2/Core/Blueprints/Items/BP_BaseItem.Update qest stat item` _array_element_2))))))

(event `Qest update stat`
  (params (Item :type "/Game/_Props_2/Core/Blueprints/Items/BP_BaseItem Object Reference") (Enum_QestTupe :type "/Game/Shimaletik/Blueprints/Qests/Enum_QestTupe Enum" :default "NewEnumerator0"))
  (bind `_настройка_квестов` (`self.Настройка квестов`))
  (bind _output (`|GetArrayItem` `_настройка_квестов` (`self.Array Index`)))
  (bind (`_описаниеквеста` `_типквеста` `_итемы` _complited) (break `/Game/Shimaletik/Blueprints/Qests/str_qest` _output))
  (bind (`_описаниеквеста_2` `_типквеста_2` `_итемы_2` _complited_2) (break `/Game/Shimaletik/Blueprints/Qests/str_qest` _output))
  (set `self.Array Index` -1)
  (for (_array_element _array_index) `_настройка_квестов`
    (if (not (== (`KismetArrayLibrary.Array_Find` (`.Итемы_12_6B99A178461389FD068863AEBFF0E20F` (break `/Game/Shimaletik/Blueprints/Qests/str_qest` _array_element)) Item) -1))
      (set `self.Array Index` _array_index)
      (break)))
  (if (== (`self.Array Index`) -1)
    _
    (elif (`|EnumEquality` `_типквеста_2` Enum_QestTupe)
      (if (== (`KismetArrayLibrary.Array_Length` `_итемы_2`) 1)
        (`|VariableSetRef` _output (make `/Game/Shimaletik/Blueprints/Qests/str_qest` `_описаниеквеста_2` `_типквеста_2` `_итемы_2` _complited_2 true))
        (`/Game/Shimaletik/Blueprints/Qests/W_Quest.Update stat qests` (`self.W_Quest`) (`self.Настройка квестов`))
        (else
          (bind _output_get (set `self.Complited` _complited))
          (`KismetArrayLibrary.Array_Set` _output_get (`KismetArrayLibrary.Array_Find` `_итемы` Item) true)
          (`|VariableSetRef` _output (make `/Game/Shimaletik/Blueprints/Qests/str_qest` `_описаниеквеста` `_типквеста` `_итемы` (`self.Complited`) (== (`KismetArrayLibrary.Array_Find` (`self.Complited`)) -1)))
          (`/Game/Shimaletik/Blueprints/Qests/W_Quest.Update stat qests` (`self.W_Quest`) (`self.Настройка квестов`)))))))

(fn `UserConstructionScript`)