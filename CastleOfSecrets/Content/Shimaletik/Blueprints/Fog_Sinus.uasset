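; Fog_Sinus oscillates a referenced actor, presumably fog, between Min and Max marker actors until the player enters a trigger box.
; Each tick it moves the actor at constant speed with VInterpToConstant, flipping the target within a tolerance of either marker, so the motion is linear despite the name.
; When Main_Character overlaps the box, a Gate stops the movement for good and the actor snaps to Min.
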(event `self.ReceiveTick`
  (params (DeltaSeconds :type "Float (single-precision)"))
  (bind _actor (`self.Actor`))
  (bind _returnvalue (`self.K2_GetActorLocation` (`self.Min`)))
  (bind _returnvalue_2 (`self.K2_GetActorLocation` (`self.Max`)))
  (bind _returnvalue_3 (`KismetMathLibrary.VInterpTo_Constant` (`self.K2_GetActorLocation` _actor) (`KismetMathLibrary.SelectVector` _returnvalue_2 _returnvalue (`self.Pick A`)) DeltaSeconds (`self.Interp Speed`)))
  (`/Engine/EditorBlueprintResources/StandardMacros.Gate` false :!label _label
    (:`Exit`
      (`self.K2_SetActorLocation` _actor _returnvalue_3 false false)
      (`|ExecutionSequence`
        (:`then_0`
          (if (== _returnvalue_3 _returnvalue_2 :`ErrorTolerance` 110.0)
            (set `self.Pick A` (not (`self.Pick A`)) :!label _label_2)))
        (:`then_1`
          (if (== _returnvalue_3 _returnvalue :`ErrorTolerance` 110.0)
            (goto _label_2)))))))

(event `self.Box.OnComponentBeginOverlap`
  (params (OverlappedComponent :type "PrimitiveComponent Object Reference") (OtherActor :type "Actor Object Reference") (OtherComp :type "PrimitiveComponent Object Reference") (OtherBodyIndex :type Integer) (bFromSweep :type Boolean) (SweepResult :type "HitResult Structure (by ref)"))
  (cast `/Game/Core/Character/Main_Character` OtherActor)
  (`|ExecutionSequence`
    (:`then_0`
      (goto _label :!via `Close`))
    (:`then_1`
      (`self.K2_SetActorLocation` (`self.Actor`) (`self.K2_GetActorLocation` (`self.Min`)) false false))))

(fn `UserConstructionScript`)